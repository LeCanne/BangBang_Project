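; BP_TriggerChangeMusic is a box trigger that stops the level music when the third-person character walks into it.
; It finds the SoundManager actor on BeginPlay.
; When the character's capsule overlaps the box, it stops the level theme intro and loop and clears the manager's IsLevel flag.
; Nodes for starting the boss theme and setting IsBoss are present but disconnected, so they never run.
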(event `self.ReceiveBeginPlay`
  (bind _returnvalue (`GameplayStatics.GetActorOfClass` "/Game/BluePrints/System/SoundManager.SoundManager_C"))
  (set `self.SoundManager` _returnvalue))

(event `self.Box.OnComponentBeginOverlap`
  (params (OverlappedComponent :type "PrimitiveComponent Object Reference") (OtherActor :type "Actor Object Reference") (OtherComp :type "PrimitiveComponent Object Reference") (OtherBodyIndex :type Integer) (bFromSweep :type Boolean) (SweepResult :type "HitResult Structure (by ref)"))
  (bind _soundmanager (`self.SoundManager`))
  (bind _asbp_third_person_character (cast `/Game/BluePrints/Control/BP_ThirdPersonCharacter` OtherActor))
  (if (== (`Character.CapsuleComponent` _asbp_third_person_character) OtherComp)
    (`AudioComponent.Stop` (`/Game/BluePrints/System/SoundManager.Level_ThemeLoop` _soundmanager))
    (`AudioComponent.Stop` (`/Game/BluePrints/System/SoundManager.Level_ThemeIntro` _soundmanager))
    (set `/Game/BluePrints/System/SoundManager.IsLevel` false _soundmanager)))

(fn `UserConstructionScript`)