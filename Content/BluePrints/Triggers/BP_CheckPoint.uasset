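; Breakable checkpoint trigger that becomes the player's respawn point when the character first overlaps it.
; Activation hides every checkpoint's Okay marker, shows its own, and saves the checkpoint name and chrono time to BP_LevelData.
; Explosion enemy overlaps drain HP unless it is Unbreakable.
; At zero HP it turns its sign translucent and recursively walks PreviousCheckpoint links to hand the player back to an unbroken checkpoint.
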(event `self.Box.OnComponentBeginOverlap`
  (params (OverlappedComponent :type "PrimitiveComponent Object Reference") (OtherActor :type "Actor Object Reference") (OtherComp :type "PrimitiveComponent Object Reference") (OtherBodyIndex :type Integer) (bFromSweep :type Boolean) (SweepResult :type "HitResult Structure (by ref)"))
  (bind _sign (`self.sign`))
  (bind _sign_2 (`self.sign`))
  (`|ExecutionSequence`
    (:`then_0`
      (cast `/Game/BluePrints/Interactable/BP_Explosion_Enemy` OtherActor)
      (if (not (`self.Unbreakable`))
        (`/Engine/EditorBlueprintResources/StandardMacros.DecrementInt` (`self.HP`))))
    (:`then_1`
      (if (<= (`self.HP`) 0)
        (`self.SetStartPosition`)
        (`PrimitiveComponent.SetMaterial` _sign_2 (`MeshComponent.GetMaterialIndex` _sign_2 "04") "/Game/Art_Graphics/z_Material/MM_WindowsTranslucent.MM_WindowsTranslucent")
        (`SceneComponent.SetVisibility` (`self.okay`) false false)
        (elif (not (`self.CheckPointTaken`))
          (bind _asbp_third_person_character (cast `/Game/BluePrints/Control/BP_ThirdPersonCharacter` OtherActor))
          (set `self.Player` _asbp_third_person_character)
          (set `/Game/BluePrints/Control/BP_ThirdPersonCharacter.Checkpoint` self _asbp_third_person_character)
          ;[0 0.1634 1] Replace Checkpoint
          (bind _returnvalue (`GameplayStatics.GetActorOfClass` "/Game/BluePrints/System/BP_LevelData.BP_LevelData_C"))
          (`|ExecutionSequence`
            (:`then_0`
              (bind _outactors (`GameplayStatics.GetAllActorsOfClass` "BP_CheckPoint_C"))
              (for _array_element _outactors
                (`SceneComponent.SetVisibility` (`/Game/BluePrints/Triggers/BP_CheckPoint.okay` _array_element) false false)
                (`PrimitiveComponent.SetMaterial` _sign (`MeshComponent.GetMaterialIndex` _sign "04") "/Engine/VREditor/LaserPointer/LaserPointerMaterialInst.LaserPointerMaterialInst")))
            (:`then_1`
              (set `/Game/BluePrints/System/BP_LevelData.CurrentCheckpoint` (`KismetSystemLibrary.GetObjectName` self) _returnvalue)
              (`SceneComponent.SetVisibility` (`self.okay`) true false)
              (set `self.CheckPointTaken` true)
              (bind _returnvalue_2 (`GameplayStatics.GetActorOfClass` "/Game/BluePrints/System/BP_LevelData.BP_LevelData_C"))
              (set `/Game/BluePrints/System/BP_LevelData.SavedChrono` (`/Game/Widget/WB_HUD.Realtime` (`/Game/BluePrints/System/BP_LevelData.Current WB` _returnvalue_2)) _returnvalue_2))))))))

(fn `SetStartPosition`
  (bind _previouscheckpoint (`self.PreviousCheckpoint`))
  (bind _previouscheckpoint_2 (`self.PreviousCheckpoint`))
  (`KismetSystemLibrary.PrintString` "BROKEN!")
  (`/Engine/EditorBlueprintResources/StandardMacros.IsValid` _previouscheckpoint
    (:`Is Valid`
      (if (<= (`/Game/BluePrints/Triggers/BP_CheckPoint.HP` _previouscheckpoint) 0)
        (`self.SetStartPosition` _previouscheckpoint_2)
        (`KismetSystemLibrary.PrintString` "Jump")
        (else
          (set `/Game/BluePrints/Control/BP_ThirdPersonCharacter.Checkpoint` _previouscheckpoint_2 (`self.Player`))
          (bind _returnvalue (`GameplayStatics.GetActorOfClass` "/Game/BluePrints/System/BP_LevelData.BP_LevelData_C"))
          (`|ExecutionSequence`
            (:`then_0`
              (bind _outactors (`GameplayStatics.GetAllActorsOfClass` "BP_CheckPoint_C"))
              (for _array_element _outactors
                (`SceneComponent.SetVisibility` (`/Game/BluePrints/Triggers/BP_CheckPoint.okay` _array_element) false false)))
            (:`then_1`
              (set `/Game/BluePrints/System/BP_LevelData.CurrentCheckpoint` (`KismetSystemLibrary.GetObjectName` (`self.PreviousCheckpoint`)) _returnvalue)
              (`SceneComponent.SetVisibility` (`self.okay`) true false)
              (`KismetSystemLibrary.PrintString` "PreviousCheckPointSet"))))))))

(fn `UserConstructionScript`)