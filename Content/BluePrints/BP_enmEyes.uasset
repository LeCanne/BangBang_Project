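; BP_enmEyes is an actor that animates a pair of eyes through material parameters on PlaneEye, with idle, hit and roll states.
; Tick manually scrubs the current state's timeline with SetNewTime, looping over its length.
; Timeline updates drive eye size and offsets, using sine and cosine for mirrored circular rolling.
; An overlap switches to hit, then to roll after a short delay, restarting the time on each change.
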(event `self.ReceiveBeginPlay`)

(event `self.ReceiveTick`
  (params (DeltaSeconds :type "Float (single-precision)"))
  ;[1 1 1] Set time to timeline
  (bind _output_get (set `self.timelineTime` (mod (+ DeltaSeconds (`self.timelineTime`)) (`TimelineComponent.GetTimelineLength` (`self.GetEyesTimeline`)))))
  (`TimelineComponent.SetNewTime` (`self.GetEyesTimeline`) _output_get))

(event `self.ReceiveActorBeginOverlap`
  (params (OtherActor :type "Actor Object Reference"))
  ;[1 1 1] Change state when Overlap
  (`self.ChangeEyesState` "NewEnumerator1")
  (`KismetSystemLibrary.Delay` 0.5)
  (`self.ChangeEyesState` "NewEnumerator0"))

(fn `ChangeEyesState`
  (params (newState :type "/Game/0_Dossiers_perso/Joseph/E_EyesState Enum" :default "NewEnumerator0"))
  (set `self.eyesState` newState)
  (set `self.timelineTime` 0.0))

(fn `GetEyesTimeline`
  (returns (NewParam :type "TimelineComponent Object Reference"))
  (switch `/Game/0_Dossiers_perso/Joseph/E_EyesState` (`self.eyesState`)
    (:`NewEnumerator0`
      (return (`self.Timeline_Roll`)))
    (:`NewEnumerator1`
      (return (`self.Timeline_Hit`)))
    (:`NewEnumerator2`
      (return (`self.Timeline_Idle`)))))

(fn `UserConstructionScript`)