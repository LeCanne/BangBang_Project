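; Camera zone actor that switches the BP_Camera to its configured state and framing when its transition event is called.
; The event toggles the player's camera icon from LockCamera and passes a spline or fixed point for those states.
; A timeline blends offset, distance and, off-spline, rotation toward HoldSpringArm, used as a framing template.
; The first transition snaps instantly and clears that flag on every trigger camera.
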(event `DoCameraTransition_Event`
  (bind _current_camera (`self.Current Camera`))
  (bind _asbp_third_person_character (cast `/Game/BluePrints/Control/BP_ThirdPersonCharacter` (`self.ThirdPersonRef`)))
  (if (`self.LockCamera`)
    (bind _cameraicon (`/Game/Widget/WB_HUD.CameraIcon` (`/Game/BluePrints/Control/BP_ThirdPersonCharacter.current WB` _asbp_third_person_character)))
    (`Widget.SetVisibility` _cameraicon "Hidden")
    (else
      (`Widget.SetVisibility` _cameraicon "Visible")))
  (bind _returnvalue (`GameplayStatics.GetActorOfClass` "/Game/BluePrints/Camera/BP_Camera.BP_Camera_C"))
  (set `self.Current Camera` _returnvalue)
  (`|ExecutionSequence`
    (:`then_0`
      (`/Game/BluePrints/Camera/BP_Camera.ResetCameraAngle_Event` (`self.Current Camera`)))
    (:`then_1`
      (switch `/Game/BluePrints/Camera/CameraStates` (`self.Camera States`)
        (:`NewEnumerator0`
          _)
        (:`NewEnumerator1`
          ;[0 0.9359 1] Set le state de la Caméra
          (set `/Game/BluePrints/Camera/BP_Camera.SplineReference` (`self.SplineReference`) (`self.Current Camera`)))
        (:`NewEnumerator2`
          (set `/Game/BluePrints/Camera/BP_Camera.PointToJoin` (`SceneComponent.K2_GetComponentLocation` (`self.CameraPoint`)) (`self.Current Camera`))))
      (set `/Game/BluePrints/Camera/BP_Camera.CameraState` (`self.Camera States`) (`self.Current Camera`))
      (`TimelineComponent.SetPlayRate` (`self.NecessaryTime`) (`self.LerpSpeed`))
      (if (`self.FirstTransition`)
        (bind _outactors (`GameplayStatics.GetAllActorsOfClass` "BP_TriggerCamera_C"))
        (for _array_element _outactors
          (set `/Game/BluePrints/Camera/BP_TriggerCamera.FirstTransition` false _array_element))
        (set `self.AlphaTime` 1.0)
        (`/Engine/EditorBlueprintResources/StandardMacros.IsValid` (`self.Current Camera`) :!label _label
          (:`Is Valid`
            ;[1 0 0] Hauteur de la Caméra par rapport à l'origine
            (`|ExecutionSequence`
              (:`then_0`
                (set `/Game/BluePrints/Camera/BP_Camera.AdditionalOffset` (`KismetMathLibrary.VLerp` (`/Game/BluePrints/Camera/BP_Camera.AdditionalOffset` _current_camera) (`SpringArmComponent.SocketOffset` (`self.HoldSpringArm`)) (`self.AlphaTime`)) _current_camera))
              (:`then_1`
                (if (not (`self.OnSpline`))
                  ;[0 0.0615 1] Rotation de la Caméra
                  (set `/Game/BluePrints/Camera/BP_Camera.FinalZoneCamera` (`KismetMathLibrary.RLerp` (`/Game/BluePrints/Camera/BP_Camera.NewCameraAngle` (`self.Current Camera`)) (`SceneComponent.K2_GetComponentRotation` (`self.HoldSpringArm`)) (`self.AlphaTime`) true) (`self.Current Camera`))))
              (:`then_2`
                ;[0 1 0.08937] Distance de la Caméra par rapport à l'origine
                (set `/Game/BluePrints/Camera/BP_Camera.Distance` (`KismetMathLibrary.Lerp` (`/Game/BluePrints/Camera/BP_Camera.Distance` (`self.Current Camera`)) (`SpringArmComponent.TargetArmLength` (`self.HoldSpringArm`)) (`self.AlphaTime`)) (`self.Current Camera`))))))
        (else
          (set `self.AlphaTime` 0.0)
          (bind (_direction _newtrack_0) (`Timeline|NecessaryTime` :!via `PlayFromStart` :!label _label_2)
            (:`Update`
              (set `self.AlphaTime` _newtrack_0)
              (goto _label))))))))

(event `StopTransition_Event`
  (goto _label_2 :!via `Stop`))

(event `self.ReceiveBeginPlay`
  (`SceneComponent.SetVisibility` (`self.SkeletalMesh`) false false)
  (`SceneComponent.K2_SetWorldLocation` (`self.CameraPoint`) (`SceneComponent.K2_GetComponentLocation` (`self.HoldSpringArm`)) false false))

(fn `UserConstructionScript`
  (`TextRenderComponent.K2_SetText` (`self.State`) (`KismetTextLibrary.Conv_StringToText` (`|GetEnumeratorNameAsString` (`self.Camera States`)))))