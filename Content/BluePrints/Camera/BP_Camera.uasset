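; Player camera actor that takes over the view on BeginPlay and follows BP_ThirdPersonCharacter with a spring arm.
; Tick switches between centering on the player and interpolating to the nearest spline point while looking at the player, with a timeline blend back from the spline.
; Arm length eases out while the player is airborne.
; Horizontal input steps through three clamped yaw angles, timeline-blended and combined with a zone rotation.
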(event `self.ReceiveBeginPlay`
  (`SceneComponent.K2_SetWorldRotation` (`self.SpringArm`) (`KismetMathLibrary.ComposeRotators` (`self.FinalZoneCamera`) (`self.FinalCameraAngle`)) false false)
  (`|ExecutionSequence`
    (:`then_0`
      (set `self.bFindCameraComponentWhenViewTarget` true)
      (`PlayerController.SetViewTargetWithBlend` (`GameplayStatics.GetPlayerController` 0) (`ActorComponent.GetOwner` (`self.Camera`)) 0.0 "VTBlend_Linear" 0.0 true))
    (:`then_1`
      (bind _returnvalue (`GameplayStatics.GetActorOfClass` "/Game/BluePrints/Control/BP_ThirdPersonCharacter.BP_ThirdPersonCharacter_C"))
      (set `self.PlayerActor` _returnvalue))))

(event `self.ReceiveTick`
  (params (DeltaSeconds :type "Float (single-precision)"))
  (bind _springarm (`self.SpringArm`))
  (`|ExecutionSequence`
    (:`then_0`
      ;[0 1 0.2777] Get initial position values (Player)
      (set `/Game/BluePrints/Control/BP_ThirdPersonCharacter.DefaultCam` (`self.Camera`) (`self.PlayerActor`))
      (set `self.PlayerPosition` (`self.K2_GetActorLocation` (`self.PlayerActor`)))
      (switch `|SwitchEnum` (`self.CameraState`)
        (:`NewEnumerator0`
          ;[0 1 0.8235] Set Center as Player
          (if (`self.TransitionFromSpline`)
            (`/Engine/EditorBlueprintResources/StandardMacros.DoOnce` false :!label _label
              (:`Completed`
                (bind (_direction _lerptime) (`Timeline|LerpCameraToPos` :!via `PlayFromStart`)
                  (:`Update`
                    (set `self.LerpTimeCameraToPos` _lerptime)
                    (set `self.DesiredPosition` (`KismetMathLibrary.VLerp` (`SceneComponent.K2_GetComponentLocation` (`self.SpringArm`)) (`self.PlayerPosition`) (`self.LerpTimeCameraToPos`))))
                  (:`Finished`
                    (set `self.TransitionFromSpline` false)
                    (goto _label :!via `Reset`)))))
            (else
              (set `self.DesiredPosition` (`self.PlayerPosition`)))))
        (:`NewEnumerator1`
          ;[0 0.1339 1] Lerp on Spline to closest position to player
          (set `self.TransitionFromSpline` true)
          (set `self.DesiredPosition` (`KismetMathLibrary.VInterpTo` (`SceneComponent.K2_GetComponentLocation` (`self.SpringArm`)) (`SplineComponent.FindLocationClosestToWorldLocation` (`/Game/BluePrints/Camera/BP_CameraSpline.Spline` (`self.SplineReference`)) (`self.PlayerPosition`) "World") (`GameplayStatics.GetWorldDeltaSeconds`) 2.0)))))
    (:`then_1`
      (if (`NavMovementComponent.IsMovingOnGround` (`Character.CharacterMovement` (`self.PlayerActor`)))
        (set `self.Desired Distance` (`self.Distance`))
        (else
          (set `self.Desired Distance` (+ (`self.Distance`) 300.0))))
      (set `SpringArmComponent.TargetArmLength` (`KismetMathLibrary.Lerp` (`SpringArmComponent.TargetArmLength` (`self.SpringArm`)) (`self.Desired Distance`) (* (`GameplayStatics.GetWorldDeltaSeconds`) 3.0)) (`self.SpringArm`))
      (switch `|SwitchEnum` (`self.CameraState`)
        (:`NewEnumerator0`
          (`self.SetDesiredCameraRotation_Event`)
          (if (`self.TransitionFromSpline`)
            (`SceneComponent.K2_SetWorldRotation` (`self.SpringArm`) (`self.NewCameraAngle`) false false)
            (else
              (`SceneComponent.K2_SetWorldRotation` (`self.SpringArm`) (`KismetMathLibrary.ComposeRotators` (`self.FinalZoneCamera`) (`self.FinalCameraAngle`)) false false))))
        (:`NewEnumerator1`
          (`SceneComponent.K2_SetWorldRotation` (`self.SpringArm`) (`KismetMathLibrary.RInterpTo` (`SceneComponent.K2_GetComponentRotation` _springarm) (`KismetMathLibrary.FindLookAtRotation` (`SceneComponent.K2_GetComponentLocation` _springarm) (`self.PlayerPosition`)) (`GameplayStatics.GetWorldDeltaSeconds`) 4.0) false false)))
      (set `SpringArmComponent.SocketOffset` (`KismetMathLibrary.MakeVector` 0.0 0.0 (`self.CameraHeight`)) (`self.SpringArm`))
      (`SceneComponent.K2_SetWorldLocation` (`self.SpringArm`) (`self.DesiredPosition`) false false))))

(event `SetDesiredCameraRotation_Event`
  ;[0 0.1339 1] LerpRotation to Look at Player
  (set `self.NewCameraAngle` (`KismetMathLibrary.RLerp` (`SceneComponent.K2_GetComponentRotation` (`self.SpringArm`)) (`self.FinalCameraAngle`) (`self.LerpTimeCameraToPos`) true)))

(event `SetNewCameraView_Event`
  (params (`La Valeur X` :type "Float (double-precision)"))
  (bind _playeranglevalue (`self.PlayerAngleValue`))
  ;[0.3392 1 0.2282] Get the Move Value of Camera Angle
  (if (and (<= `La Valeur X` -0.5) (== (`self.PlayerAngleValue`) 2))
    _
    (elif (not (and (>= `La Valeur X` 0.5) (== (`self.PlayerAngleValue`) 0)))
      (`|ExecutionSequence`
        (:`then_0`
          (if (>= `La Valeur X` 0.5)
            (bind _result (`/Engine/EditorBlueprintResources/StandardMacros.DecrementInt` _playeranglevalue)
              (:`  `
                (set `self.PlayerAngleValue` (`KismetMathLibrary.Clamp` _result 0 2))))))
        (:`then_1`
          (if (<= `La Valeur X` -0.5)
            (bind _result_2 (`/Engine/EditorBlueprintResources/StandardMacros.IncrementInt` _playeranglevalue)
              (:`  `
                (set `self.PlayerAngleValue` (`KismetMathLibrary.Clamp` _result_2 0 2))))))
        (:`then_2`
          (switch `int` (`self.PlayerAngleValue`)
            (:`0`
              (set `self.CameraPlayerAngle` (struct :`Yaw` 45.0)))
            (:`1`
              (set `self.CameraPlayerAngle` (struct)))
            (:`2`
              (set `self.CameraPlayerAngle` (struct :`Yaw` -45.0)))))
        (:`then_3`
          (`KismetSystemLibrary.PrintString` (`KismetStringLibrary.Conv_IntToString` (`self.PlayerAngleValue`)))
          (bind (_direction _newtrack_0) (`Timeline|ChangeAngle` :!via `PlayFromStart` :!label _label_2)
            (:`Update`
              (set `self.FinalCameraAngle` (`KismetMathLibrary.RLerp` (`self.FinalCameraAngle`) (`self.CameraPlayerAngle`) _newtrack_0 true)))))))))

(event `Stop Anim_Event`
  ;[0.3392 1 0.2282] Get the Move Value of Camera Angle
  (goto _label_2 :!via `Stop`))

(fn `UserConstructionScript`)