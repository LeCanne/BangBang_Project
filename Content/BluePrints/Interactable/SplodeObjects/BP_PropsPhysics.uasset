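; BP_PropsPhysics is a configurable physics prop whose mesh, tint and physical behavior are set through variables.
; Its construction script assigns the chosen mesh, puts a dynamic instance of the source material in the first slot and sets its Tint parameter.
; It then enables physics simulation on the static mesh and applies the mass override and linear and angular damping.
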(fn `UserConstructionScript`
  (bind _staticmeshcomponent (`self.StaticMeshComponent`))
  (bind _staticmeshcomponent_2 (`self.StaticMeshComponent`))
  (`StaticMeshComponent.SetStaticMesh` _staticmeshcomponent_2 (`self.Set Mesh`))
  (bind _returnvalue (`KismetMaterialLibrary.CreateDynamicMaterialInstance` (`self.Source Material`)))
  (`PrimitiveComponent.SetMaterial` _staticmeshcomponent_2 0 _returnvalue)
  (`MeshComponent.SetVectorParameterValueOnMaterials` (`self.StaticMeshComponent`) "Tint" (`KismetMathLibrary.Conv_LinearColorToVector` (`KismetMathLibrary.Conv_ColorToLinearColor` (`self.Tint`))))
  (`PrimitiveComponent.SetSimulatePhysics` _staticmeshcomponent true)
  (`PrimitiveComponent.SetMassOverrideInKg` _staticmeshcomponent "None" (`self.Mass (kg)`) true)
  (`PrimitiveComponent.SetLinearDamping` _staticmeshcomponent (`self.LinDamping`))
  (`PrimitiveComponent.SetAngularDamping` _staticmeshcomponent (`self.AngDamping`)))