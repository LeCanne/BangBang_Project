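; Destructible object with two glass windows that shatter when the player character touches them and award score.
; On overlap with BP_ThirdPersonCharacter, each window disables its collision, hides itself, activates its own Niagara shatter effect and plays a glass-break sound.
; Both paths then add a fixed bonus to CurrentScore on BP_LevelData, found via GetActorOfClass.
; The construction script creates dynamic material instances, then applies the Material variable to both windows.
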(event `self.ReceiveBeginPlay`)

(event `self.window1.OnComponentBeginOverlap`
  (params (OverlappedComponent :type "PrimitiveComponent Object Reference") (OtherActor :type "Actor Object Reference") (OtherComp :type "PrimitiveComponent Object Reference") (OtherBodyIndex :type Integer) (bFromSweep :type Boolean) (SweepResult :type "HitResult Structure (by ref)"))
  (bind _window1 (`self.window1`))
  (cast `/Game/BluePrints/Control/BP_ThirdPersonCharacter` OtherActor)
  (`PrimitiveComponent.SetCollisionEnabled` _window1 "NoCollision")
  (`SceneComponent.SetVisibility` _window1 false false)
  (`ActorComponent.Activate` (`self.NS_shatterGlass`) false)
  (`GameplayStatics.PlaySound2D` "/Game/0_Dossiers_perso/Charles/Audio/Sound_Cue/SFX/Enviro/A_GlassBreak_Cue.A_GlassBreak_Cue" 1.0 1.0 0.0 null null)
  (bind _returnvalue (`GameplayStatics.GetActorOfClass` "/Game/BluePrints/System/BP_LevelData.BP_LevelData_C" :!label _label))
  (set `/Game/BluePrints/System/BP_LevelData.CurrentScore` (`KismetMathLibrary.Conv_IntToDouble` (+ (`/Game/BluePrints/System/BP_LevelData.CurrentScore` _returnvalue) 500)) _returnvalue))

(event `self.window2.OnComponentBeginOverlap`
  (params (OverlappedComponent :type "PrimitiveComponent Object Reference") (OtherActor :type "Actor Object Reference") (OtherComp :type "PrimitiveComponent Object Reference") (OtherBodyIndex :type Integer) (bFromSweep :type Boolean) (SweepResult :type "HitResult Structure (by ref)"))
  (bind _window2 (`self.window2`))
  (cast `/Game/BluePrints/Control/BP_ThirdPersonCharacter` OtherActor)
  (`PrimitiveComponent.SetCollisionEnabled` _window2 "NoCollision")
  (`SceneComponent.SetVisibility` _window2 false false)
  (`ActorComponent.Activate` (`self.NS_shatterGlass1`) false)
  (`GameplayStatics.PlaySound2D` "/Game/0_Dossiers_perso/Charles/Audio/Sound_Cue/SFX/Enviro/A_GlassBreak_Cue.A_GlassBreak_Cue" 1.0 1.0 0.0 null null)
  (goto _label))

(event `self.ReceiveTick`
  (params (DeltaSeconds :type "Float (single-precision)")))

(fn `UserConstructionScript`
  (bind _window2 (`self.window2`))
  (bind _window1 (`self.window1`))
  (`PrimitiveComponent.CreateDynamicMaterialInstance` _window1 0 null "None")
  (`PrimitiveComponent.CreateDynamicMaterialInstance` _window2 0 null "None")
  (`PrimitiveComponent.SetMaterial` (`|MakeArray` _window1 _window2 :!type "PrimitiveComponent Object Reference") 0 (`self.Material`)))