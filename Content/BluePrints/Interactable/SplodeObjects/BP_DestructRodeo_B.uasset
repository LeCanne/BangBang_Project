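; Destructible glass prop (top and glass meshes) that shatters when the third-person character overlaps its box while SetupRodeo is false.
; The construction script groups meshes and shatter Niagara effects into arrays for batched calls.
; Breaking activates the effects, disables mesh collision and visibility, removes the trigger, and plays glass-break and pitch-parameterised comic explosion sounds.
; After a delay, it destroys the meshes and adds score to BP_LevelData.
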(event `self.BoxCollider.OnComponentBeginOverlap`
  (params (OverlappedComponent :type "PrimitiveComponent Object Reference") (OtherActor :type "Actor Object Reference") (OtherComp :type "PrimitiveComponent Object Reference") (OtherBodyIndex :type Integer) (bFromSweep :type Boolean) (SweepResult :type "HitResult Structure (by ref)"))
  (bind _arraysm (`self.ArraySM`))
  (`|ExecutionSequence`
    (:`then_0`
      (bind _asbp_third_person_character (cast `/Game/BluePrints/Control/BP_ThirdPersonCharacter` OtherActor))
      (if (not (`/Game/BluePrints/Control/BP_ThirdPersonCharacter.SetupRodeo` _asbp_third_person_character))
        (`PrimitiveComponent.IgnoreActorWhenMoving` (`self.ArraySM`) _asbp_third_person_character false)
        (`ActorComponent.Activate` (`self.ArrayNS`) false)
        (`PrimitiveComponent.SetCollisionEnabled` _arraysm "NoCollision")
        (`SceneComponent.SetVisibility` _arraysm false false)
        (`ActorComponent.K2_DestroyComponent` (`self.BoxCollider`))
        (`GameplayStatics.PlaySound2D` "/Game/0_Dossiers_perso/Charles/Audio/Sound_Cue/SFX/Enviro/A_GlassBreak_Cue.A_GlassBreak_Cue" 1.0 1.0 0.0 null null)
        (`self.ComicSound`)
        (`KismetSystemLibrary.Delay` 4.0)
        (`ActorComponent.K2_DestroyComponent` _arraysm)
        (bind _returnvalue (`GameplayStatics.GetActorOfClass` "/Game/BluePrints/System/BP_LevelData.BP_LevelData_C"))
        (set `/Game/BluePrints/System/BP_LevelData.CurrentScore` (`KismetMathLibrary.Conv_IntToDouble` (+ (`/Game/BluePrints/System/BP_LevelData.CurrentScore` _returnvalue) 200)) _returnvalue)))))

(event `ComicSound`
  (bind _pitchfloat (`self.PitchFloat`))
  ;[1 1 1] Change pitch/volume sound
  (bind _returnvalue (`GameplayStatics.CreateSound2D` "/Game/0_Dossiers_perso/Charles/Audio/Sound_Cue/SFX/A_Explosion_Comic_Cue.A_Explosion_Comic_Cue" 1.0 1.0 0.0 null))
  (`AudioComponent.SetFloatParameter` _returnvalue "ComicPitch" _pitchfloat)
  (`AudioComponent.Play` _returnvalue 0.0)
  (set `self.PitchFloat` (+ _pitchfloat 0.1)))

(event `ResetComic`
  ;[1 1 1] Change pitch/volume sound
  (set `self.PitchFloat` 0.0))

(fn `UserConstructionScript`
  (set `self.ArraySM` (`|MakeArray` (`self.top`) (`self.glass`)))
  (set `self.ArrayNS` (`|MakeArray` (`self.NS_shatterVerriere`) (`self.NS_shatterGlass`))))