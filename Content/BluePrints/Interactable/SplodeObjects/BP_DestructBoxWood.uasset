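; Destructible wooden box that breaks when overlapped by the player (unless SetupRodeo is set), an enemy explosion or an EXPLOSION-tagged component.
; Breaking hides the mesh, disables collision, awards score through the ScoreSpawn child actor, spawns BP_ExplosionItem above it and plays a wood-break sound.
; Only explosion hits activate the Niagara shatter effect.
; The construction script exposes mesh, tint, collider transform and shatter parameters per instance.
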(event `self.BoxCollider.OnComponentBeginOverlap`
  (params (OverlappedComponent :type "PrimitiveComponent Object Reference") (OtherActor :type "Actor Object Reference") (OtherComp :type "PrimitiveComponent Object Reference") (OtherBodyIndex :type Integer) (bFromSweep :type Boolean) (SweepResult :type "HitResult Structure (by ref)"))
  (bind _returnvalue (`self.GetTransform`))
  (`|ExecutionSequence`
    (:`then_0`
      (bind _asbp_third_person_character (cast `/Game/BluePrints/Control/BP_ThirdPersonCharacter` OtherActor))
      (if (not (`/Game/BluePrints/Control/BP_ThirdPersonCharacter.SetupRodeo` _asbp_third_person_character))
        (`PrimitiveComponent.IgnoreActorWhenMoving` (`self.Mesh`) _asbp_third_person_character false)
        (`PrimitiveComponent.SetCollisionEnabled` (`self.Mesh`) "NoCollision" :!label _label)
        (`SceneComponent.SetVisibility` (`self.Mesh`) false false)
        (`PrimitiveComponent.SetCollisionEnabled` (`self.BoxCollider`) "NoCollision")
        (bind _asbp_give_score (cast `/Game/BluePrints/System/BP_GiveScore` (`ChildActorComponent.ChildActor` (`self.ScoreSpawn`))))
        (`GameplayStatics.GetActorOfClass` "/Game/BluePrints/System/BP_LevelData.BP_LevelData_C")
        (`/Game/BluePrints/System/BP_GiveScore.Give Score` _asbp_give_score 50.0 false)
        (`|SpawnActorFromClass` "/Game/BluePrints/Interactable/BP_ExplosionItem.BP_ExplosionItem_C" (`KismetMathLibrary.MakeTransform` (`KismetMathLibrary.MakeVector` (.x (.location _returnvalue)) (.y (.location _returnvalue)) (+ (.z (.location _returnvalue)) 200.0))) "Undefined" "MultiplyWithRoot" null null)
        (`GameplayStatics.PlaySound2D` "/Game/0_Dossiers_perso/Charles/Audio/Sound_Cue/SFX/Enviro/A_WoodBreak_Cue.A_WoodBreak_Cue" 1.0 1.0 0.0 null null)))
    (:`then_1`
      (cast `/Game/BluePrints/Interactable/BP_Explosion_Enemy` OtherActor)
      (`ActorComponent.Activate` (`self.NS_shatter`) false :!label _label_2)
      (goto _label))
    (:`then_2`
      (if (`ActorComponent.ComponentHasTag` OtherComp "EXPLOSION")
        (goto _label_2)))))

(fn `UserConstructionScript`
  (bind _mesh (`self.Mesh`))
  ;[1 0.9411 0] Vector2
  (`NiagaraComponent.SetVariableVec2` (`self.NS_shatter`) "SpriteMax" (`self.Size Max`))
  (`NiagaraComponent.SetVariableVec2` (`self.NS_shatter`) "SpriteMin" (`self.Size Min`))
  ;[0 0.08976 1] Color
  (`NiagaraComponent.SetVariableLinearColor` (`self.NS_shatter`) "ColorMax" (`self.Color Max`))
  (`NiagaraComponent.SetVariableLinearColor` (`self.NS_shatter`) "ColorMin" (`self.Color Min`))
  ;[0.08409 1 0] Float
  (`NiagaraComponent.SetVariableFloat` (`self.NS_shatter`) "Scale" (`self.Scale`))
  (`NiagaraComponent.SetVariableFloat` (`self.NS_shatter`) "VelocityMax" (`self.Velocity Max`))
  (`NiagaraComponent.SetVariableFloat` (`self.NS_shatter`) "VelocityMin" (`self.VelocityMin`))
  (`NiagaraComponent.SetVariableFloat` (`self.NS_shatter`) "ScaleSmoke" (`self.Scale Smoke`))
  ;[0.1029 1 0.8094] Int
  (`NiagaraComponent.SetVariableInt` (`self.NS_shatter`) "SpawnCount" (`self.Spawn Count`))
  (`StaticMeshComponent.SetStaticMesh` (`self.Mesh`) (`self.New Mesh`))
  (`SceneComponent.K2_SetRelativeTransform` (`self.BoxCollider`) (`self.ColliderTransform`) false false)
  ;[1 1 1] Mesh Tint
  (bind _returnvalue (`PrimitiveComponent.CreateDynamicMaterialInstance` _mesh 0 null "None"))
  (`PrimitiveComponent.SetMaterial` _mesh 0 _returnvalue)
  (`MeshComponent.SetVectorParameterValueOnMaterials` _mesh "Tint" (`KismetMathLibrary.Conv_LinearColorToVector` (`KismetMathLibrary.Conv_ColorToLinearColor` (`self.Tint`))))
  ;[1 1 1] NiagaraMat
  (`NiagaraComponent.SetVariableMaterial` (`self.NS_shatter`) "Mat" (`self.Material`)))