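; Destructible steel box that breaks on overlap with an enemy explosion or with a player character whose SetupRodeo flag is off.
; Both triggers share a teardown that disables collision, hides the mesh, removes the trigger box and destroys the mesh after a delay.
; Only the explosion path activates the NSShatter effect.
; The construction script feeds exposed size, color, velocity, scale and count settings into NSShatter and tints the mesh via a dynamic material.
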(event `self.BoxCollider.OnComponentBeginOverlap`
  (params (OverlappedComponent :type "PrimitiveComponent Object Reference") (OtherActor :type "Actor Object Reference") (OtherComp :type "PrimitiveComponent Object Reference") (OtherBodyIndex :type Integer) (bFromSweep :type Boolean) (SweepResult :type "HitResult Structure (by ref)"))
  (`|ExecutionSequence`
    (:`then_0`
      (bind _asbp_third_person_character (cast `/Game/BluePrints/Control/BP_ThirdPersonCharacter` OtherActor))
      (if (not (`/Game/BluePrints/Control/BP_ThirdPersonCharacter.SetupRodeo` _asbp_third_person_character))
        (`PrimitiveComponent.IgnoreActorWhenMoving` (`self.base`) _asbp_third_person_character false)
        (`PrimitiveComponent.SetCollisionEnabled` (`self.base`) "NoCollision" :!label _label)
        (`SceneComponent.SetVisibility` (`self.base`) false false)
        (`ActorComponent.K2_DestroyComponent` (`self.BoxCollider`))
        (`KismetSystemLibrary.Delay` 4.0)
        (`ActorComponent.K2_DestroyComponent` (`self.base`))))
    (:`then_1`
      (cast `/Game/BluePrints/Interactable/BP_Explosion_Enemy` OtherActor)
      (`ActorComponent.Activate` (`self.NS_shatter`) false)
      (goto _label))))

(fn `UserConstructionScript`
  (bind _base (`self.base`))
  ;[1 0.9411 0] Vector2
  (`NiagaraComponent.SetVariableVec2` (`self.NS_shatter`) "SpriteMax" (`self.Size Max`))
  (`NiagaraComponent.SetVariableVec2` (`self.NS_shatter`) "SpriteMin" (`self.Size Min`))
  ;[0 0.08976 1] Color
  (`NiagaraComponent.SetVariableLinearColor` (`self.NS_shatter`) "ColorMax" (`self.Color Max`))
  (`NiagaraComponent.SetVariableLinearColor` (`self.NS_shatter`) "ColorMin" (`self.Color Min`))
  ;[0.08409 1 0] Float
  (`NiagaraComponent.SetVariableFloat` (`self.NS_shatter`) "Scale" (`self.Scale`))
  (`NiagaraComponent.SetVariableFloat` (`self.NS_shatter`) "VelocityMax" (`self.Velocity Max`))
  (`NiagaraComponent.SetVariableFloat` (`self.NS_shatter`) "VelocityMin" (`self.VelocityMin`))
  (`NiagaraComponent.SetVariableFloat` (`self.NS_shatter`) "ScaleSmoke" (`self.Scale Smoke`))
  ;[0.1029 1 0.8094] Int
  (`NiagaraComponent.SetVariableInt` (`self.NS_shatter`) "SpawnCount" (`self.Spawn Count`))
  ;[1 1 1] Mesh Tint
  (bind _returnvalue (`PrimitiveComponent.CreateDynamicMaterialInstance` _base 0 null "None"))
  (`PrimitiveComponent.SetMaterial` _base 0 _returnvalue)
  (`MeshComponent.SetVectorParameterValueOnMaterials` _base "Tint" (`KismetMathLibrary.Conv_LinearColorToVector` (`KismetMathLibrary.Conv_ColorToLinearColor` (`self.Tint`)))))