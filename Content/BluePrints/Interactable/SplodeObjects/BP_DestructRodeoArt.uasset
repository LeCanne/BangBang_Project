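; BP_DestructRodeoArt is a destructible glass roof prop (verrière) that shatters when the third-person character overlaps it while that character's SetupRodeo flag is false.
; On overlap it turns off step-up on the two meshes, SMVerriereSecond and SMVerriereWindows, then destroys both components.
; It then activates the NSVerriereBurst effect to play the burst.
; All logic lives in the overlap event, with no Tick or construction script work.
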(event `self.ReceiveActorBeginOverlap`
  (params (OtherActor :type "Actor Object Reference"))
  (bind _sm_verriere_second (`self.SM_verriere_second`))
  (bind _sm_verriere_windows (`self.SM_verriere_windows`))
  (bind _asbp_third_person_character (cast `/Game/BluePrints/Control/BP_ThirdPersonCharacter` OtherActor))
  (if (not (`/Game/BluePrints/Control/BP_ThirdPersonCharacter.SetupRodeo` _asbp_third_person_character))
    (set `PrimitiveComponent.CanCharacterStepUpOn` "ECB_No" _sm_verriere_second)
    (`PrimitiveComponent.IgnoreActorWhenMoving` _sm_verriere_second _asbp_third_person_character false)
    (set `PrimitiveComponent.CanCharacterStepUpOn` "ECB_No" _sm_verriere_windows)
    (`PrimitiveComponent.IgnoreActorWhenMoving` _sm_verriere_windows null false)
    (`ActorComponent.K2_DestroyComponent` _sm_verriere_second)
    (`ActorComponent.K2_DestroyComponent` _sm_verriere_windows)
    (`ActorComponent.Activate` (`self.NS_verriereBurst`) false)))

(fn `UserConstructionScript`)