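; BP_DestructRodeo_C is a destructible glass canopy ("verrière") that shatters when the third-person character overlaps its box while SetupRodeo is false.
; The construction script groups the breakable meshes and Niagara effects into arrays and sets the glass spawn count.
; Breaking hides those meshes, disables their collision, triggers effects and sound, then after four seconds destroys them and adds score to BP_LevelData.
; An explosion-enemy trigger is present but unconnected.
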(event `self.ReceiveBeginPlay`)

(event `self.BoxCollider.OnComponentBeginOverlap`
  (params (OverlappedComponent :type "PrimitiveComponent Object Reference") (OtherActor :type "Actor Object Reference") (OtherComp :type "PrimitiveComponent Object Reference") (OtherBodyIndex :type Integer) (bFromSweep :type Boolean) (SweepResult :type "HitResult Structure (by ref)"))
  (bind _arraysm (`self.ArraySM`))
  (bind _sm_verriere_main (`self.SM_verriere_main`))
  (`|ExecutionSequence`
    (:`then_0`
      (bind _asbp_third_person_character (cast `/Game/BluePrints/Control/BP_ThirdPersonCharacter` OtherActor))
      (if (not (`/Game/BluePrints/Control/BP_ThirdPersonCharacter.SetupRodeo` _asbp_third_person_character))
        (set `PrimitiveComponent.CanCharacterStepUpOn` "ECB_No" _sm_verriere_main)
        (`PrimitiveComponent.IgnoreActorWhenMoving` _sm_verriere_main _asbp_third_person_character false)
        (`PrimitiveComponent.SetCollisionEnabled` _arraysm "NoCollision")
        (`SceneComponent.SetVisibility` _arraysm false false)
        (`ActorComponent.K2_DestroyComponent` (`self.BoxCollider`))
        (`ActorComponent.Activate` (`self.ArrayNS`) false)
        (`GameplayStatics.PlaySound2D` "/Game/0_Dossiers_perso/Charles/Audio/Sound_Cue/SFX/Enviro/A_GlassBreak_Cue.A_GlassBreak_Cue" 1.0 1.0 0.0 null null)
        (`KismetSystemLibrary.Delay` 4.0)
        (`ActorComponent.K2_DestroyComponent` _arraysm)
        (bind _returnvalue (`GameplayStatics.GetActorOfClass` "/Game/BluePrints/System/BP_LevelData.BP_LevelData_C"))
        (set `/Game/BluePrints/System/BP_LevelData.CurrentScore` (`KismetMathLibrary.Conv_IntToDouble` (+ (`/Game/BluePrints/System/BP_LevelData.CurrentScore` _returnvalue) 200)) _returnvalue)))))

(event `self.ReceiveTick`
  (params (DeltaSeconds :type "Float (single-precision)")))

(fn `UserConstructionScript`
  (set `self.ArraySM` (`|MakeArray` (`self.SM_verriere_second`) (`self.SM_verriere_windows`)))
  (set `self.ArrayNS` (`|MakeArray` (`self.NS_shatterVerriere`) (`self.NS_shatterGlass`)))
  (`NiagaraComponent.SetVariableInt` (`self.NS_shatterGlass`) "SpawnCount" (`self.ShatteredGlass_SpawnCount`)))