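; BP_DestructRodeo_A is a destructible glass canopy (verrière) that shatters when the third-person character overlaps it while SetupRodeo is false.
; The overlap hides and disables the secondary and window meshes, removes the box collider, fires two Niagara shatter effects, then destroys those meshes after a delay.
; A repeatedly restarted GlassSlide timeline animates the window material's U_slide parameter, and Tick prints its value.
; The construction script groups the breakable parts and sets the glass shard count.
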(event `self.ReceiveBeginPlay`
  (bind (_direction _glassslide) (`Timeline|GlassSlide` :!label _label)
    (:`Update`
      (`MeshComponent.SetScalarParameterValueOnMaterials` (`self.SM_verriere_windows`) "U_slide" (* _glassslide 2.0))
      (`KismetSystemLibrary.Delay` 2.0)
      (goto _label :!via `PlayFromStart`))))

(event `self.ReceiveActorBeginOverlap`
  (params (OtherActor :type "Actor Object Reference"))
  (bind _sm_verriere_main (`self.SM_verriere_main`))
  (bind _arraysm (`self.ArraySM`))
  (bind _asbp_third_person_character (cast `/Game/BluePrints/Control/BP_ThirdPersonCharacter` OtherActor))
  (if (not (`/Game/BluePrints/Control/BP_ThirdPersonCharacter.SetupRodeo` _asbp_third_person_character))
    (set `PrimitiveComponent.CanCharacterStepUpOn` "ECB_No" _sm_verriere_main)
    (`PrimitiveComponent.IgnoreActorWhenMoving` _sm_verriere_main _asbp_third_person_character false)
    (`PrimitiveComponent.SetCollisionEnabled` _arraysm "NoCollision")
    (`SceneComponent.SetVisibility` _arraysm false false)
    (`ActorComponent.K2_DestroyComponent` (`self.BoxCollider`))
    (`ActorComponent.Activate` (`self.ArrayNS`) false)
    (`KismetSystemLibrary.Delay` 4.0)
    (`ActorComponent.K2_DestroyComponent` _arraysm)))

(event `self.ReceiveTick`
  (params (DeltaSeconds :type "Float (single-precision)"))
  (`KismetSystemLibrary.PrintString` (`KismetStringLibrary.Conv_DoubleToString` (stale `self.ReceiveBeginPlay` _glassslide))))

(fn `UserConstructionScript`
  (set `self.ArraySM` (`|MakeArray` (`self.SM_verriere_second`) (`self.SM_verriere_windows`)))
  (set `self.ArrayNS` (`|MakeArray` (`self.NS_shatterVerriere`) (`self.NS_shatterGlass`)))
  (`NiagaraComponent.SetVariableInt` (`self.NS_shatterGlass`) "SpawnCount" (`self.ShatteredGlass_SpawnCount`)))