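; BP_DestructBush is a destructible bush that shatters when a BP_Explosion_Enemy actor overlaps its BoxCollider.
; The construction script groups three bush meshes and three leaf-shatter effects into arrays.
; On that overlap it activates the effects, hides the meshes and destroys the collider.
; It then awards a fixed score through the BP_GiveScore child actor in ScoreSpawn, with score display turned off.
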(event `self.BoxCollider.OnComponentBeginOverlap`
  (params (OverlappedComponent :type "PrimitiveComponent Object Reference") (OtherActor :type "Actor Object Reference") (OtherComp :type "PrimitiveComponent Object Reference") (OtherBodyIndex :type Integer) (bFromSweep :type Boolean) (SweepResult :type "HitResult Structure (by ref)"))
  (cast `/Game/BluePrints/Interactable/BP_Explosion_Enemy` OtherActor)
  (`ActorComponent.Activate` (`self.ArrayNS`) false)
  (`SceneComponent.SetVisibility` (`self.ArraySM`) false false)
  (`ActorComponent.K2_DestroyComponent` (`self.BoxCollider`))
  (bind _asbp_give_score (cast `/Game/BluePrints/System/BP_GiveScore` (`ChildActorComponent.ChildActor` (`self.ScoreSpawn`))))
  (`GameplayStatics.GetActorOfClass` "/Game/BluePrints/System/BP_LevelData.BP_LevelData_C")
  (`/Game/BluePrints/System/BP_GiveScore.Give Score` _asbp_give_score 30.0 false))

(fn `UserConstructionScript`
  (set `self.ArraySM` (`|MakeArray` (`self.bush1`) (`self.bush`) (`self.bush2`)))
  (set `self.ArrayNS` (`|MakeArray` (`self.NS_shatterLeave`) (`self.NS_shatterLeave2`) (`self.NS_shatterLeave1`))))