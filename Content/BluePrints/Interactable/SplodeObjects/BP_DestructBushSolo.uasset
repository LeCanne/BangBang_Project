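; BP_DestructBushSolo is a destructible bush that awards score when an enemy explosion overlaps it.
; Its BoxCollider overlap event casts the other actor to BP_Explosion_Enemy, then activates the NSShatterLeave effect, hides the Bush component and destroys the collider so it cannot retrigger.
; It then finds BP_LevelData with GetActorOfClass and adds points to its CurrentScore.
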(event `self.BoxCollider.OnComponentBeginOverlap`
  (params (OverlappedComponent :type "PrimitiveComponent Object Reference") (OtherActor :type "Actor Object Reference") (OtherComp :type "PrimitiveComponent Object Reference") (OtherBodyIndex :type Integer) (bFromSweep :type Boolean) (SweepResult :type "HitResult Structure (by ref)"))
  (cast `/Game/BluePrints/Interactable/BP_Explosion_Enemy` OtherActor)
  (`ActorComponent.Activate` (`self.NS_shatterLeave`) false)
  (`SceneComponent.SetVisibility` (`self.bush`) false false)
  (`ActorComponent.K2_DestroyComponent` (`self.BoxCollider`))
  (bind _returnvalue (`GameplayStatics.GetActorOfClass` "/Game/BluePrints/System/BP_LevelData.BP_LevelData_C"))
  (set `/Game/BluePrints/System/BP_LevelData.CurrentScore` (`KismetMathLibrary.Conv_IntToDouble` (+ (`/Game/BluePrints/System/BP_LevelData.CurrentScore` _returnvalue) 10)) _returnvalue))

(fn `UserConstructionScript`)