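; BP_Explosion_Enemy is a short-lived explosion effect that launches tagged props as it expands.
; On BeginPlay it plays a sound at world origin and runs a Timeline that scales the visual sphere and collision sphere together, then destroys itself.
; Static mesh actors tagged "ObjectExplode" that overlap the collision sphere switch to simulated physics and receive upward, radial and random angular impulses.
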(event `self.ReceiveBeginPlay`
  ;[1 1 1] Explosion avec une Timeline + Son
  (`TimelineComponent.SetPlayRate` (`self.Timeline`) (`self.AnimationSpeed`))
  (`GameplayStatics.PlaySoundAtLocation` "/Game/0_Dossiers_perso/Charles/Audio/Sound_Cue/SFX/A_explosion_Cue.A_explosion_Cue" (0.0 0.0 0.0) (struct) 1.0 1.0 0.0 null null null null)
  (bind (_direction _scale) (`Timeline|Timeline`)
    (:`Update`
      (`|ExecutionSequence`
        (:`then_0`
          (`SceneComponent.SetWorldScale3D` (`self.Sphere`) (`KismetMathLibrary.Conv_DoubleToVector` _scale)))
        (:`then_1`
          (`SceneComponent.SetWorldScale3D` (`self.SphereCollision_Explosion`) (`KismetMathLibrary.Conv_DoubleToVector` _scale)))))
    (:`Finished`
      (`self.K2_DestroyActor`))))

(event `self.SphereCollision_Explosion.OnComponentBeginOverlap`
  (params (OverlappedComponent :type "PrimitiveComponent Object Reference") (OtherActor :type "Actor Object Reference") (OtherComp :type "PrimitiveComponent Object Reference") (OtherBodyIndex :type Integer) (bFromSweep :type Boolean) (SweepResult :type "HitResult Structure (by ref)"))
  (bind _asstatic_mesh_actor (cast `StaticMeshActor` OtherActor))
  (if (`self.ActorHasTag` OtherActor "ObjectExplode")
    (bind _staticmeshcomponent (`StaticMeshActor.StaticMeshComponent` _asstatic_mesh_actor))
    (`PrimitiveComponent.SetCollisionObjectType` _staticmeshcomponent "ECC_WorldDynamic")
    (`PrimitiveComponent.SetSimulatePhysics` _staticmeshcomponent true)
    (`PrimitiveComponent.AddImpulse` _staticmeshcomponent (0.0 0.0 300.0) "None" true)
    (`PrimitiveComponent.AddRadialImpulse` _staticmeshcomponent (`SceneComponent.K2_GetComponentLocation` (`self.SphereCollision_Explosion`)) 20000.0 500.0 "RIF_Constant" false)
    (bind _output_get (set `self.Strengh` (`KismetMathLibrary.RandomUnitVector`)))
    (`PrimitiveComponent.AddAngularImpulseInDegrees` _staticmeshcomponent (* _output_get 100.0) "None" false)))

(fn `UserConstructionScript`)