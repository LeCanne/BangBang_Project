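; BP_PropsPhysics_sign is a physics prop sign with a configurable tint and an arrow.
; The construction script creates dynamic materials for the tint and the arrow, rotated in 90-degree steps, and applies mass and damping overrides to the mesh.
; When a BP_Explosion_Enemy overlaps the sign, its mesh briefly ignores the Pawn collision channel, then blocks it again.
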(event `self.ReceiveActorBeginOverlap`
  (params (OtherActor :type "Actor Object Reference"))
  (cast `/Game/BluePrints/Interactable/BP_Explosion_Enemy` OtherActor)
  (`PrimitiveComponent.SetCollisionResponseToChannel` (`self.StaticMeshComponent`) "ECC_Pawn" "ECR_Ignore")
  (`KismetSystemLibrary.Delay` 1.0)
  (`PrimitiveComponent.SetCollisionResponseToChannel` (`self.StaticMeshComponent`) "ECC_Pawn" "ECR_Block"))

(fn `UserConstructionScript`
  (bind _staticmeshcomponent (`self.StaticMeshComponent`))
  (bind _returnvalue (`KismetMaterialLibrary.CreateDynamicMaterialInstance` (`self.Source Material`)))
  (`PrimitiveComponent.SetMaterial` _staticmeshcomponent 0 _returnvalue)
  (`MeshComponent.SetVectorParameterValueOnMaterials` _staticmeshcomponent "Tint" (`KismetMathLibrary.Conv_LinearColorToVector` (`KismetMathLibrary.Conv_ColorToLinearColor` (`self.Tint`))))
  (`PrimitiveComponent.SetMassOverrideInKg` _staticmeshcomponent "None" (`self.Mass (kg)`) true)
  (`PrimitiveComponent.SetLinearDamping` _staticmeshcomponent (`self.LinDamping`))
  (`PrimitiveComponent.SetAngularDamping` _staticmeshcomponent (`self.AngDamping`))
  (bind _returnvalue_2 (`PrimitiveComponent.CreateDynamicMaterialInstance` (`self.Arrow`) 0 "/Game/Art_Graphics/z_Material/MM_arrowOnly.MM_arrowOnly" "None"))
  (`MaterialInstanceDynamic.SetScalarParameterValue` _returnvalue_2 "Rotation" (`KismetMathLibrary.Conv_IntToDouble` (* (`self.Rotation`) 90))))