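; BP_PropsPhysics_poteauD is an interactable physics prop Blueprint, named as a post variant, with configurable look and physical behavior.
; Its construction script creates a dynamic material instance from SourceMaterial on the static mesh and sets the Tint parameter.
; It then applies a mass override plus linear and angular damping from variables.
; The event graph holds only an empty ActorBeginOverlap event.
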(event `self.ReceiveActorBeginOverlap`
  (params (OtherActor :type "Actor Object Reference")))

(fn `UserConstructionScript`
  (bind _staticmeshcomponent (`self.StaticMeshComponent`))
  (bind _returnvalue (`KismetMaterialLibrary.CreateDynamicMaterialInstance` (`self.Source Material`)))
  (`PrimitiveComponent.SetMaterial` _staticmeshcomponent 0 _returnvalue)
  (`MeshComponent.SetVectorParameterValueOnMaterials` _staticmeshcomponent "Tint" (`KismetMathLibrary.Conv_LinearColorToVector` (`KismetMathLibrary.Conv_ColorToLinearColor` (`self.Tint`))))
  (`PrimitiveComponent.SetMassOverrideInKg` _staticmeshcomponent "None" (`self.Mass (kg)`) true)
  (`PrimitiveComponent.SetLinearDamping` _staticmeshcomponent (`self.LinDamping`))
  (`PrimitiveComponent.SetAngularDamping` _staticmeshcomponent (`self.AngDamping`)))