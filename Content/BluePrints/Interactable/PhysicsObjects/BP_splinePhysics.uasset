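; BP_splinePhysics is a placement actor that fills a spline with evenly spaced child actors of a configurable class.
; Its construction script divides the spline length by a spacing distance and adds a child actor component at each step, including the start point.
; Each child takes its local position from the spline but uses a shared rotation and scale rather than following the curve direction.
; The event graph has no runtime logic.
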(event `self.ReceiveActorBeginOverlap`
  (params (OtherActor :type "Actor Object Reference")))

(fn `UserConstructionScript`
  (for _index (range (+ (`.ReturnValue` (`KismetMathLibrary.FMod` (`SplineComponent.GetSplineLength` (`self.Spline`)) (`self.Distance`))) 1))
    (bind _returnvalue (`AddComponent|NODE_AddChildActorComponent-0` :`RelativeTransform` (`KismetMathLibrary.MakeTransform` (`SplineComponent.GetLocationAtDistanceAlongSpline` (`self.Spline`) (* _index (`self.Distance`)) "Local") (`self.Rotation`) (`self.Scale`))))
    (`ChildActorComponent.SetChildActorClass` _returnvalue (`self.In Class`))))