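; Barrel cannon interactable (DK) that captures the overlapping player character, rotates toward its spline, then fires them out.
; Entry zeroes gravity and velocity and plays a scale-up; Tick drives rotation, then fires automatically or awaits Control_Barrel, depending on Enum.
; After a scale-down, IsNewMethode selects moving the player along the spline or the older LaunchCharacter impulse, with explosion VFX and sound.
; One Enum mode disables the barrel after exit.
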(event `self.ReceiveTick`
  (params (DeltaSeconds :type "Float (single-precision)"))
  (bind _as_bp_third_person_character (`self.As BP Third Person Character`))
  (bind _enum (`self.Enum`))
  (bind _forcepulse (`self.ForcePulse`))
  (`|ExecutionSequence`
    (:`then_0`
      (if (`self.IsStartRotation`)
        ;[1 1 1] Rotation du canon
        (`self.OpenCanon` DeltaSeconds)
        (elif (`self.IsStartSpline`)
          ;[0.9565 1 0.2656] Nouvelle méthode
          (bind _output_get (set `self.Distance` (+ (`self.Distance`) (* DeltaSeconds (* (`self.Speed`) 100.0)))))
          (bind (_sweephitresult _returnvalue) (`self.K2_SetActorLocation` _as_bp_third_person_character (`SplineComponent.GetLocationAtDistanceAlongSpline` (`self.Spline`) _output_get "World") (`self.IsEndOverlap`) false))
          (if _returnvalue
            (if (>= (`self.Distance`) (`SplineComponent.GetSplineLength` (`self.Spline`)))
              (set `self.IsFinish` true :!label _label)
              (set `self.IsStartSpline` false)
              (set `self.IsDK` false)
              (`/Game/BluePrints/Control/BP_ThirdPersonCharacter.ChangeMapping` _as_bp_third_person_character))
            (else
              (goto _label))))))
    (:`then_1`
      (if (and (`self.IsDone`) (not (`self.IsFinish`)))
        (if (not (`|EnumEquality` _enum "NewEnumerator0"))
          (`/Engine/EditorBlueprintResources/StandardMacros.DoOnce` false :!label _label_2
            (:`Completed`
              (set `self.IsDone` false)
              (bind (_direction _scaledown) (`Timeline|ScalingDown` :!via `PlayFromStart`)
                (:`Update`
                  (`SceneComponent.SetWorldScale3D` (`self.Cylinder`) (`KismetMathLibrary.Conv_DoubleToVector` _scaledown)))
                (:`Finished`
                  (if (`self.IsNewMethode`)
                    (`ActorComponent.Activate` (`self.NS_explosionCanon`) true)
                    (`GameplayStatics.SpawnSound2D` "/Game/0_Dossiers_perso/Charles/Audio/Sound_Cue/SFX/A_explosion_Cue.A_explosion_Cue" 1.0 1.0 0.0 null)
                    (if (not (`self.IsFinish`))
                      (set `self.Distance` 0.0)
                      (set `self.IsStartSpline` true)
                      (`self.Reset Do Once`))
                    (else
                      ;[0.3927 0.3927 0.3927] Ancienne Méthode
                      (`self.Project_Barrel` (* (`KismetMathLibrary.Normal` (- (`SceneComponent.K2_GetComponentLocation` (`self.Scene`)) (`SceneComponent.K2_GetComponentLocation` (`self.Cylinder`)))) (`KismetMathLibrary.MakeVector` _forcepulse _forcepulse _forcepulse)))
                      (if (`|EnumEquality` _enum "NewEnumerator2")
                        (`self.SetActorHiddenInGame` false))
                      (`self.Reset Do Once`))))))))))))

(event `Control_Barrel`
  (if (not (`self.IsFinish`))
    (goto _label_2)))

(event `self.ReceiveActorBeginOverlap`
  (params (OtherActor :type "Actor Object Reference"))
  (bind _asbp_third_person_character (cast `/Game/BluePrints/Control/BP_ThirdPersonCharacter` OtherActor))
  (if (and (not (`self.IsDK`)) (not (`self.IsDesable`)))
    (`GameplayStatics.PlaySound2D` "/Game/0_Dossiers_perso/Charles/Audio/SFX/Blocking/Canon/SFX_EnterCanonV2.SFX_EnterCanonV2" 1.0 1.0 0.0 null null)
    (set `self.IsDK` true)
    (set `self.IsEndOverlap` false)
    (bind _output_get (set `self.As BP Third Person Character` _asbp_third_person_character))
    (`self.K2_SetActorLocation` _output_get (`self.K2_GetActorLocation`) false false)
    (bind _charactermovement (`Character.CharacterMovement` _asbp_third_person_character))
    (set `CharacterMovementComponent.GravityScale` 0.0 _charactermovement)
    (set `MovementComponent.Velocity` (0.0 0.0 0.0) _charactermovement)
    (set `self.IsStartRotation` true)
    (set `self.RotateFloat` 0.0)
    ;[1 1 1] Feedback quand on rentre
    (bind (_direction _scalexy _rotationlength _scalez) (`Timeline|ScalingUp` :!via `PlayFromStart`)
      (:`Update`
        (`SceneComponent.SetWorldScale3D` (`self.Cylinder`) (`KismetMathLibrary.MakeVector` _scalexy _scalexy _scalez)))
      (:`Finished`
        (set `self.IsFinish` false)))))

(event `Reset Do Once`
  (goto _label_2 :!via `Reset`))

(event `self.ReceiveActorEndOverlap`
  (params (OtherActor :type "Actor Object Reference"))
  (cast `/Game/BluePrints/Control/BP_ThirdPersonCharacter` OtherActor)
  (set `self.IsEndOverlap` true)
  (if (`|EnumEquality` (`self.Enum`) "NewEnumerator2")
    (`SceneComponent.SetHiddenInGame` (`self.Cylinder`) true false)
    (set `self.IsDesable` true)))

(event `StopTimeline`
  ;[0.9565 1 0.2656] Nouvelle méthode
  (set `self.IsFinish` true)
  (set `self.IsStartSpline` false)
  (set `self.IsDK` false))

(fn `OpenCanon`
  (params (A :type "Float (double-precision)"))
  (bind _scene1 (`self.Scene1`))
  (bind _returnvalue (`SceneComponent.K2_GetComponentRotation` _scene1))
  (bind _returnvalue_2 (`SceneComponent.K2_GetComponentRotation` (`self.Spline`)))
  (bind _output_get (set `self.RotateFloat` (+ (`self.RotateFloat`) (* A (* (`self.Speed_Rotation`) 1.0)))))
  (`SceneComponent.K2_SetWorldRotation` _scene1 (`KismetMathLibrary.RLerp` _returnvalue _returnvalue_2 _output_get true) false false)
  (if (== _returnvalue _returnvalue_2 :`ErrorTolerance` 1.0)
    (set `self.IsStartRotation` false)
    (set `self.IsDone` true)))

(fn `Project_Barrel`
  (params (Impulse :type "Vector Structure"))
  (`Character.LaunchCharacter` (`self.As BP Third Person Character`) Impulse false false)
  (`ActorComponent.Activate` (`self.NS_explosionCanon`) true)
  (`GameplayStatics.SpawnSound2D` "/Game/0_Dossiers_perso/Charles/Audio/Sound_Cue/SFX/A_explosion_Cue.A_explosion_Cue" 1.0 1.0 0.0 null))

(fn `UserConstructionScript`)