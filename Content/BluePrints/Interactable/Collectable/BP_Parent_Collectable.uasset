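; Parent Blueprint for collectables, providing a base with mostly stubbed behavior.
; The Hit event only casts the other actor to BP_ThirdPersonCharacter, with nothing following.
; CollectableRare sets the Cylinder to a transparent rare material when IsCollect is true, otherwise reapplies its current one.
; CollectableRotate is disconnected because the material handles spinning, and CollectablePoint is empty.
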(event `self.ReceiveBeginPlay`)

(event `self.ReceiveHit`
  (params (MyComp :type "PrimitiveComponent Object Reference") (Other :type "Actor Object Reference") (OtherComp :type "PrimitiveComponent Object Reference") (bSelfMoved :type Boolean) (HitLocation :type "Vector Structure") (HitNormal :type "Vector Structure") (NormalImpulse :type "Vector Structure") (Hit :type "HitResult Structure (by ref)"))
  (`|ExecutionSequence`
    (:`then_0`
      (cast `/Game/BluePrints/Control/BP_ThirdPersonCharacter` Other))))

(fn `Collectable Point`)

(fn `Collectable Rare`
  (bind _cylinder (`self.Cylinder`))
  (if (`self.IsCollect`)
    (`PrimitiveComponent.SetMaterial` (`self.Cylinder`) 0 "/Game/0_Dossiers_perso/Charles/Materials/Transparent_CollectableRare.Transparent_CollectableRare")
    (else
      (`PrimitiveComponent.SetMaterial` _cylinder 0 (`PrimitiveComponent.GetMaterial` _cylinder 0)))))

(fn `Collectable Rotate`
  (params (A :type "Float (double-precision)"))
  ;[1 1 1] Rotate le collectable (Désactivé car le matériau s'occupe de faire tourner déjà)
)

(fn `UserConstructionScript`)