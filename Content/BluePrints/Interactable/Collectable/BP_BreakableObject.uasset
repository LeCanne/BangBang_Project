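; BP_BreakableObject is a breakable world object that scatters collectables when an enemy explosion hits it.
; Overlap with a BP_Explosion_Enemy actor trips a one-shot Broken flag, then spawns BP_Child_CollectableClassic pickups in a loop driven by CollectSpawns.
; Each pickup is moved to a random horizontal offset around the object, which is then hidden in game rather than destroyed.
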(event `self.ReceiveActorBeginOverlap`
  (params (OtherActor :type "Actor Object Reference"))
  (cast `/Game/BluePrints/Interactable/BP_Explosion_Enemy` OtherActor)
  (if (not (`self.Broken`))
    (set `self.Broken` true)
    (for _ (range (+ (`self.CollectSpawns`) 1))
      (bind _returnvalue (`|SpawnActorFromClass` "/Game/BluePrints/Interactable/Collectable/BP_Child_CollectableClassic.BP_Child_CollectableClassic_C" (`self.GetTransform`) "Undefined" "MultiplyWithRoot" null null))
      (`self.K2_SetActorLocation` _returnvalue (+ (`self.K2_GetActorLocation`) (`KismetMathLibrary.MakeVector` (`KismetMathLibrary.RandomFloatInRange` -200.0 200.0) (`KismetMathLibrary.RandomFloatInRange` -200.0 200.0))) false false))
    (`self.SetActorHiddenInGame` true)))

(fn `UserConstructionScript`)