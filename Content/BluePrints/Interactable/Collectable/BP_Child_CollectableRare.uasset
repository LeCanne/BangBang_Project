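; Rare variant of a collectable pickup that rotates in the world and disappears when the player character touches it.
; It calls parent functions to set its rare state on BeginPlay and to rotate every Tick.
; Overlap with BP_ThirdPersonCharacter destroys the actor on both branches of an IsCollect check, setting that flag only where it is already true.
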(event `self.ReceiveBeginPlay`
  ;[1 1 1 1 15] Fonction parent pour donner un état
  (`self.Collectable Rare`))

(event `self.ReceiveTick`
  (params (DeltaSeconds :type "Float (single-precision)"))
  ;[1 1 1 1 15] Fonction Parent pour rotate l'objet
  (`self.Collectable Rotate` DeltaSeconds))

(event `self.ReceiveActorBeginOverlap`
  (params (OtherActor :type "Actor Object Reference"))
  (cast `/Game/BluePrints/Control/BP_ThirdPersonCharacter` OtherActor)
  (if (`self.IsCollect`)
    (set `self.IsCollect` true)
    (`self.K2_DestroyActor`)
    (else
      (`self.K2_DestroyActor`))))

(fn `UserConstructionScript`
  (`parent.UserConstructionScript`))