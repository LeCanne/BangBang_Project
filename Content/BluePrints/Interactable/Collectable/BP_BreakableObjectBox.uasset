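; Breakable box that bursts into physics collectables, breaking once when overlapped by an enemy explosion, a static mesh actor or a component tagged EXPLOSION.
; On break it traces down for each spawn position, then launches the collectables upward and outward in an evenly spaced ring scaled by Radius.
; The block is then hidden with collision off, and shatter and pouf Niagara effects play, scaled by ShatterScale in the construction script.
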(event `self.ReceiveActorBeginOverlap`
  (params (OtherActor :type "Actor Object Reference"))
  (bind _blocktobreak (`self.BlockToBreak`))
  (bind _collectspawns (`self.CollectSpawns`))
  (cast `/Game/BluePrints/Interactable/BP_Explosion_Enemy` OtherActor
    (:`then`
      _)
    (:`CastFailed`
      (cast `StaticMeshActor` OtherActor)))
  (if (not (`self.Broken`)) :!label _label
    (set `self.Broken` true)
    (for _index (range (+ _collectspawns 1))
      (bind _outhit (`KismetSystemLibrary.LineTraceSingle` (`SceneComponent.K2_GetComponentLocation` (`self.Scene`)) (+ (`self.K2_GetActorLocation`) (0.0 0.0 -400.0)) "TraceTypeQuery1"))
      (bind (_bblockinghit _binitialoverlap _time _distance _location) (`GameplayStatics.BreakHitResult` _outhit))
      (bind _returnvalue (`|SpawnActorFromClass` "/Game/BluePrints/Interactable/Collectable/BP_Child_CollectablePhysics.BP_Child_CollectablePhysics_C" (`KismetMathLibrary.MakeTransform` (`KismetMathLibrary.MakeVector` (.x _location) (.y _location) (+ (.z _location) 100.0))) "AdjustIfPossibleButAlwaysSpawn" "MultiplyWithRoot" self null))
      (`/Game/BluePrints/Interactable/Collectable/BP_Child_CollectablePhysics.ImpulseUp_Event` _returnvalue 2000.0 (* (`KismetMathLibrary.GetForwardVector` (`KismetMathLibrary.MakeRotator` 0.0 0.0 (`KismetMathLibrary.Conv_IntToDouble` (* _index (/ 360 _collectspawns))))) (`self.Radius`))))
    (`SceneComponent.SetHiddenInGame` _blocktobreak true false)
    (`PrimitiveComponent.SetCollisionEnabled` _blocktobreak "NoCollision")
    (`ActorComponent.Activate` (`|MakeArray` (`self.NS_shatter`) (`self.NS_pouf`) :!type "ActorComponent Object Reference") false)))

(event `self.BlockToBreak.OnComponentBeginOverlap`
  (params (OverlappedComponent :type "PrimitiveComponent Object Reference") (OtherActor :type "Actor Object Reference") (OtherComp :type "PrimitiveComponent Object Reference") (OtherBodyIndex :type Integer) (bFromSweep :type Boolean) (SweepResult :type "HitResult Structure (by ref)"))
  (if (`ActorComponent.ComponentHasTag` OtherComp "EXPLOSION")
    (goto _label)))

(fn `UserConstructionScript`
  (`NiagaraComponent.SetVariableFloat` (`|MakeArray` (`self.NS_shatter`) (`self.NS_pouf`)) "scale" (`self.ShatterScale`)))