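; Child collectable Blueprint that adds projectile physics, so a spawned pickup can be launched and then picked up.
; BeginPlay moves the ProjectileMovement's updated component to the Cylinder and, after a short delay, sets a Collectable flag.
; Overlaps reach the parent's pickup logic only once that flag is set.
; ImpulseUp_Event sets launch velocity from ImpulseForceXY and the passed upward force.
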(event `self.ReceiveBeginPlay`
  (`MovementComponent.SetUpdatedComponent` (`self.ProjectileMovement`) (`self.Cylinder`))
  (`|ExecutionSequence`
    (:`then_0`
      (`parent.ReceiveBeginPlay`))
    (:`then_1`
      (`KismetSystemLibrary.Delay` 0.2)
      (set `self.Collectable` true))))

(event `self.ReceiveActorBeginOverlap`
  (params (OtherActor :type "Actor Object Reference"))
  (if (`self.Collectable`)
    (`parent.ReceiveActorBeginOverlap` OtherActor)))

(event `self.ReceiveTick`
  (params (DeltaSeconds :type "Float (single-precision)"))
  (`parent.ReceiveTick` DeltaSeconds))

(event `ImpulseUp_Event`
  (params (`Impulse Force UpWard` :type "Float (double-precision)") (ImpulseForceXY :type "Vector Structure"))
  (set `MovementComponent.Velocity` (`KismetMathLibrary.MakeVector` ImpulseForceXY_X ImpulseForceXY_Y `Impulse Force UpWard`) (`self.ProjectileMovement`)))

(fn `UserConstructionScript`
  (`parent.UserConstructionScript`))