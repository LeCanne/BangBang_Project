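; Classic score collectable Blueprint, a child of a parent collectable, that awards points when the player character touches it.
; Tick calls the inherited rotate function to spin it.
; On overlap with BP_ThirdPersonCharacter, it adds a fixed amount to the character's ScorePoint, hides the cylinder, plays a pickup sound and activates a Niagara effect.
; It destroys itself after a short delay, with no guard against repeat overlaps during that window.
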(event `self.ReceiveTick`
  (params (DeltaSeconds :type "Float (single-precision)"))
  ;[1 1 1] Appelle la fonction parent
  (`self.Collectable Rotate` DeltaSeconds))

(event `self.ReceiveActorBeginOverlap`
  (params (OtherActor :type "Actor Object Reference"))
  (bind _asbp_third_person_character (cast `/Game/BluePrints/Control/BP_ThirdPersonCharacter` OtherActor))
  (bind _output_get (set `self.As BP Third Person Character` _asbp_third_person_character))
  (set `/Game/BluePrints/Control/BP_ThirdPersonCharacter.ScorePoint` (`KismetMathLibrary.Conv_IntToDouble` (+ (`/Game/BluePrints/Control/BP_ThirdPersonCharacter.ScorePoint` _output_get) 10)) _output_get)
  (`SceneComponent.SetVisibility` (`self.Cylinder`) false false)
  (`GameplayStatics.SpawnSound2D` "/Game/0_Dossiers_perso/Charles/Audio/SFX/Blocking/PickUp/SFX_PickUpV1.SFX_PickUpV1" 1.0 1.0 0.0 null)
  (`ActorComponent.Activate` (`self.NS_collectable`) false)
  (`KismetSystemLibrary.Delay` 1.0)
  (`self.K2_DestroyActor`))

(fn `UserConstructionScript`
  (`parent.UserConstructionScript`))