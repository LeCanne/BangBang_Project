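; Collectable ring actor that arranges classic collectable coins in a circle and spins them as a group.
; The construction script adds BP_Child_CollectableClassic child actors in a loop, placing them at Radius around the actor's origin using angle steps of 360 divided by MakeCoins.
; Tick yaws the whole actor in world space by Speed scaled with delta time, so the coins orbit the center.
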(event `self.ReceiveTick`
  (params (DeltaSeconds :type "Float (single-precision)"))
  (`self.K2_AddActorWorldRotation` (`KismetMathLibrary.MakeRotator` 0.0 0.0 (* DeltaSeconds (`self.Speed`)))))

(fn `UserConstructionScript`
  (bind _makecoins (`self.MakeCoins`))
  (for _index (range (+ _makecoins 1))
    (bind _returnvalue (`AddComponent|NODE_AddChildActorComponent-0` :`RelativeTransform` (`KismetMathLibrary.MakeTransform` (+ (`KismetMathLibrary.InverseTransformLocation` (`self.GetTransform`) (`self.K2_GetActorLocation`)) (* (`KismetMathLibrary.GetForwardVector` (`KismetMathLibrary.MakeRotator` 0.0 0.0 (`KismetMathLibrary.Conv_IntToDouble` (* (/ 360 _makecoins) _index)))) (`self.Radius`))))))
    (`ChildActorComponent.SetChildActorClass` _returnvalue "/Game/BluePrints/Interactable/Collectable/BP_Child_CollectableClassic.BP_Child_CollectableClassic_C")))