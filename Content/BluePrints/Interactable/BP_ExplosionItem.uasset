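; BP_ExplosionItem is an explosion actor that expands as soon as it spawns and then removes itself.
; On BeginPlay it plays a Timeline at AnimationSpeed, whose Scale output times ScaleEnemy drives the world scale of both Sphere and SphereCollisionExplosion.
; The Timeline update also starts a Delay of ExplosionLifetime, counted from the first update, after which the actor is destroyed.
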(event `self.ReceiveBeginPlay`
  ;[1 1 1] Explosion avec une Timeline + Son
  (`TimelineComponent.SetPlayRate` (`self.Timeline`) (`self.AnimationSpeed`))
  (bind (_direction _scale) (`Timeline|Timeline`)
    (:`Update`
      (`|ExecutionSequence`
        (:`then_0`
          (bind _returnvalue (`KismetMathLibrary.Conv_DoubleToVector` (* _scale (`self.ScaleEnemy`))))
          (`SceneComponent.SetWorldScale3D` (`self.Sphere`) _returnvalue))
        (:`then_1`
          (`SceneComponent.SetWorldScale3D` (`self.SphereCollision_Explosion`) _returnvalue))
        (:`then_2`
          (`KismetSystemLibrary.Delay` (`self.ExplosionLifetime`))
          (`self.K2_DestroyActor`))))))

(fn `UserConstructionScript`)