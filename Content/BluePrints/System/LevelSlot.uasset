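; Level-select slot actor in the menu world that BP_MichaelMenu walks into to choose and launch a level.
; Overlapping LevelEntry selects the slot and replaces all on-screen widgets with a selection widget showing its name, score and colon-separated time.
; Leaving clears the selection but keeps the widget.
; Pressing IA_Jump on a selected, enabled slot disables the menu character's input and opens the level after a short delay.
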(event `self.ReceiveBeginPlay`
  (`self.EnableInput` (`GameplayStatics.GetPlayerController` 0)))

(event `EnhancedInput|/Game/BluePrints/Control/Input/Actions/IA_Jump`
  (params (ActionValue :type Boolean) (ElapsedSeconds :type "Float (double-precision)") (TriggeredSeconds :type "Float (double-precision)") (InputAction :type "InputAction Object Reference" :default "/Game/BluePrints/Control/Input/Actions/IA_Jump.IA_Jump"))
  (:`Started`
    (if (`self.LevelEnabled`)
      (if (`self.Selected`)
        (bind _returnvalue (`GameplayStatics.GetActorOfClass` "/Game/BluePrints/Control/BP_MichaelMenu.BP_MichaelMenu_C"))
        (`self.DisableInput` _returnvalue (`GameplayStatics.GetPlayerController` 0))
        (`KismetSystemLibrary.Delay` 3.0)
        (`GameplayStatics.OpenLevelBySoftObjectPtr` (`self.Level`))))))

(event `self.LevelEntry.OnComponentBeginOverlap`
  (params (OverlappedComponent :type "PrimitiveComponent Object Reference") (OtherActor :type "Actor Object Reference") (OtherComp :type "PrimitiveComponent Object Reference") (OtherBodyIndex :type Integer) (bFromSweep :type Boolean) (SweepResult :type "HitResult Structure (by ref)"))
  (bind _time (`self.Time`))
  (bind _returnvalue (`KismetMathLibrary.FTrunc` (`KismetMathLibrary.Conv_IntToDouble` (`KismetMathLibrary.FFloor` _time))))
  (cast `/Game/BluePrints/Control/BP_MichaelMenu` OtherActor)
  (set `self.Selected` true)
  (`WidgetLayoutLibrary.RemoveAllWidgets`)
  (bind _returnvalue_2 (`|CreateWidget` "/Game/Widget/WidgetSelection.WidgetSelection_C" (`GameplayStatics.GetPlayerController` 0)))
  (`UserWidget.AddToViewport` _returnvalue_2 0)
  (set `TextBlock.Text` (`KismetTextLibrary.Conv_StringToText` (`self.Name`)) (`/Game/Widget/WidgetSelection.TITLE` _returnvalue_2))
  (set `TextBlock.Text` (`KismetTextLibrary.Conv_IntToText` (`self.Score`)) (`/Game/Widget/WidgetSelection.ScoreHandler` _returnvalue_2))
  (set `TextBlock.Text` (`KismetTextLibrary.Conv_StringToText` (`KismetStringLibrary.Concat_StrStr` (`KismetStringLibrary.Concat_StrStr` (`KismetStringLibrary.Concat_StrStr` (`KismetStringLibrary.Concat_StrStr` (`KismetTextLibrary.Conv_TextToString` (`KismetTextLibrary.Conv_IntToText` (mod (`KismetMathLibrary.FFloor` (/ _returnvalue (`self.float60`))) 60) false true 2 2)) ":") (`KismetTextLibrary.Conv_TextToString` (`KismetTextLibrary.Conv_IntToText` _returnvalue false true 2 2))) ":") (`KismetTextLibrary.Conv_TextToString` (`KismetTextLibrary.Conv_DoubleToText` (* _time 100.0) "HalfToEven" false true 2 2 0 0)))) (`/Game/Widget/WidgetSelection.TimeHandler` _returnvalue_2)))

(event `self.LevelEntry.OnComponentEndOverlap`
  (params (OverlappedComponent :type "PrimitiveComponent Object Reference") (OtherActor :type "Actor Object Reference") (OtherComp :type "PrimitiveComponent Object Reference") (OtherBodyIndex :type Integer))
  (cast `/Game/BluePrints/Control/BP_MichaelMenu` OtherActor)
  (set `self.Selected` false))

(fn `UserConstructionScript`)