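; BP_TextScore is a short-lived floating score popup actor whose text is set through SetTextScore.
; On BeginPlay, a half-speed Timeline lifts the TextRender toward a point above the actor, lerping from its current location each update for an eased motion.
; Late in the timeline, a delayed visibility toggle makes the text blink, and the actor destroys itself when the timeline finishes.
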(event `self.ReceiveBeginPlay`
  (`TimelineComponent.SetPlayRate` (`self.Timeline`) 0.5)
  (bind (_direction _newtrack_0) (`Timeline|Timeline`)
    (:`Update`
      (`|ExecutionSequence`
        (:`then_0`
          (if (>= _newtrack_0 0.65)
            (`KismetSystemLibrary.Delay` 0.1)
            (`SceneComponent.ToggleVisibility` (`self.TextRender`) false)))
        (:`then_1`
          (`SceneComponent.K2_SetWorldLocation` (`self.TextRender`) (`KismetMathLibrary.VLerp` (`SceneComponent.K2_GetComponentLocation` (`self.TextRender`)) (+ (`self.K2_GetActorLocation`) (0.0 0.0 100.0)) _newtrack_0) false false))))
    (:`Finished`
      (`self.K2_DestroyActor`))))

(fn `SetTextScore`
  (params (InputScore :type "Float (double-precision)"))
  (`TextRenderComponent.K2_SetText` (`self.TextRender`) (`KismetTextLibrary.Conv_DoubleToText` InputScore "HalfToEven")))

(fn `UserConstructionScript`)