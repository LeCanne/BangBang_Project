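; Per-level manager that runs a level session: HUD, timer, checkpoint-style state, restarts and final results.
; Start and restart stream the level in, spawn the player at a stored transform, play a first-time intro and destroy already-collected items by object name.
; SaveData snapshots score, shards, time and pickups, which restart restores after unloading the level.
; Final save ranks a new high score, keeps the best time and writes to the GameInstance's level list.
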(event `SaveFinalData_Event`
  (bind (_leveldatafinal_levelfinished _leveldatafinal_score) (break `/Game/BluePrints/System/SaveSystem/Levels/LevelDataStruct` (`self.LevelDataFinal`)))
  (bind (_leveldatafinal_levelfinished_2 _leveldatafinal_score_2 _leveldatafinal_rank _leveldatafinal_levelname _leveldatafinal_levelid _leveldatafinal_time) (break `/Game/BluePrints/System/SaveSystem/Levels/LevelDataStruct` (`self.LevelDataFinal`)))
  (bind (_leveldatafinal_levelfinished_3 _leveldatafinal_score_3 _leveldatafinal_rank_2 _leveldatafinal_levelname_2 _leveldatafinal_levelid_2 _leveldatafinal_time_2) (break `/Game/BluePrints/System/SaveSystem/Levels/LevelDataStruct` (`self.LevelDataFinal`)))
  (bind (_leveldatafinal_levelfinished_4 _leveldatafinal_score_4 _leveldatafinal_rank_3 _leveldatafinal_levelname_3 _leveldatafinal_levelid_3) (break `/Game/BluePrints/System/SaveSystem/Levels/LevelDataStruct` (`self.LevelDataFinal`)))
  (bind _asbp_game_instance (cast `/Game/BluePrints/System/BP_GameInstance` (`GameplayStatics.GetGameInstance`)))
  (`|ExecutionSequence`
    (:`then_0`
      (bind (_output_levelfinished _output_score _output_rank _output_levelname _output_levelid _output_time) (break `/Game/BluePrints/System/SaveSystem/Levels/LevelDataStruct` (`|GetArrayItem` (`/Game/BluePrints/System/BP_GameInstance.LevelList` _asbp_game_instance) (`self.LevelId`))))
      (set `self.LevelDataFinal` (make `/Game/BluePrints/System/SaveSystem/Levels/LevelDataStruct` true _output_score _output_rank _output_levelname _output_levelid _output_time)))
    (:`then_1`
      (if (> (`self.CurrentScore`) _leveldatafinal_score)
        (`|ExecutionSequence`
          (:`then_0`
            (set `self.CurrentRank` "S")
            (if (not (> (`self.CurrentScore`) (`self.S Score`)))
              (set `self.CurrentRank` "A")
              (if (not (> (`self.CurrentScore`) (`self.A Score`)))
                (set `self.CurrentRank` "B")
                (if (not (> (`self.CurrentScore`) (`self.B Score`)))
                  (set `self.CurrentRank` "C")
                  (if (not (> (`self.CurrentScore`) (`self.C Score`)))
                    (set `self.CurrentRank` "D"))))))
          (:`then_1`
            (set `self.LevelDataFinal` (make `/Game/BluePrints/System/SaveSystem/Levels/LevelDataStruct` _leveldatafinal_levelfinished_3 (`KismetMathLibrary.FTrunc` (`self.CurrentScore`)) (`self.CurrentRank`) _leveldatafinal_levelname_2 _leveldatafinal_levelid_2 _leveldatafinal_time_2))))))
    (:`then_2`
      (if (< (`self.InitialChrono`) _leveldatafinal_time)
        (set `self.LevelDataFinal` (make `/Game/BluePrints/System/SaveSystem/Levels/LevelDataStruct` _leveldatafinal_levelfinished_4 _leveldatafinal_score_4 _leveldatafinal_rank_3 _leveldatafinal_levelname_3 _leveldatafinal_levelid_3 (`self.InitialChrono`)))))
    (:`then_3`
      (`KismetArrayLibrary.Array_Set` (`/Game/BluePrints/System/BP_GameInstance.LevelList` _asbp_game_instance) (`self.LevelId`) (`self.LevelDataFinal`))
      (`/Game/BluePrints/System/BP_GameInstance.SaveLevelData_Event` _asbp_game_instance))))

(event `self.ReceiveTick`
  (params (DeltaSeconds :type "Float (single-precision)"))
  ;[0.6077 0.1557 1] Handle Time
  (`/Engine/EditorBlueprintResources/StandardMacros.IsValid` (`self.Current WB`)
    (:`Is Valid`
      (bind _output_get (set `self.InitialChrono` (+ (`GameplayStatics.GetWorldDeltaSeconds`) (`self.InitialChrono`))))
      (set `/Game/Widget/WB_HUD.Realtime` _output_get (`self.Current WB`)))))

(event `Save Data_Event`
  ;[0.7756 0.9185 1] Save all Data
  (set `self.SavedScore` (`self.CurrentScore`))
  (set `self.SavedShards` (`self.CurrentShards`))
  (set `self.SavedChrono` (`self.InitialChrono`))
  (set `self.SavedCollectables` (`self.CurrentCollectables`))
  (set `self.SavedCrates` (`self.CurrentCrates`)))

(event `StartLevel_Event`
  ;[1 0.2479 0.9896] Level Transition
  (`GameplayStatics.SetGlobalTimeDilation` 0.0)
  (bind _returnvalue (`|CreateWidget` "/Game/Widget/WB_HUD.WB_HUD_C"))
  (set `self.current WB` _returnvalue)
  (`UserWidget.AddToViewport` (`self.Current WB`) 0)
  (`self.HandleInitialization_Event`))

(event `RestartLevel_Event`
  ;[1 0.2479 0.9896] Level Transition
  (`GameplayStatics.SetGlobalTimeDilation` 0.0)
  (set `self.MaxCollectables` 0)
  (set `self.InitialChrono` (`self.SavedChrono`))
  (set `self.CurrentScore` (`self.SavedScore`))
  (set `self.CurrentShards` (`self.SavedShards`))
  (set `self.CurrentCollectables` (`self.SavedCollectables`))
  (set `self.CurrentCrates` (`self.SavedCrates`))
  (bind _returnvalue (`GameplayStatics.GetActorOfClass` "/Game/BluePrints/System/SoundManager.SoundManager_C"))
  (`/Game/BluePrints/System/SoundManager.StopLevelTheme` _returnvalue)
  (`GameplayStatics.UnloadStreamLevelBySoftObjectPtr` (`self.Level`) true)
  (`self.HandleInitialization_Event`))

(event `HandleInitialization_Event`
  ;[0.07239 0.9702 1] Initializer Process
  (`self.LoadLevel_Event`))

(event `PostInitialization_Event`
  ;[0.07239 0.9702 1] Initializer Process
  (`|ExecutionSequence`
    (:`then_0`
      (`self.Initialize Player_Event`))
    (:`then_1`
      (`self.HandleIntroduction_Event`))
    (:`then_2`
      (`self.HandleCollectables_Event`))))

(event `LoadLevel_Event`
  ;[0.4319 0.2885 1] LoadLevel
  (`GameplayStatics.LoadStreamLevelBySoftObjectPtr` (`self.Level`) true true)
  (bind _outactors (`GameplayStatics.GetAllActorsOfClass` "/Game/BluePrints/Camera/BP_TriggerCamera.BP_TriggerCamera_C"))
  (for _array_element _outactors
    (set `/Game/BluePrints/Camera/BP_TriggerCamera.FirstTransition` true _array_element))
  (`GameplayStatics.SetGlobalTimeDilation` 1.0)
  (`self.PostInitialization_Event`))

(event `Initialize Player_Event`
  (bind (_cptransform_location _cptransform_rotation) (`KismetMathLibrary.BreakTransform` (`self.CPtransform`)))
  ;[0.1982 0.6667 0.154] Spawn Player and attach dependencies
  (bind _asbp_third_person_game_mode (cast `/Game/BluePrints/GameModes/BP_ThirdPersonGameMode` (`GameplayStatics.GetGameMode`)))
  (`GameModeBase.RestartPlayerAtTransform` _asbp_third_person_game_mode (`GameplayStatics.GetPlayerController` 0) (`KismetMathLibrary.MakeTransform` _cptransform_location _cptransform_rotation))
  (bind _returnvalue (`GameplayStatics.GetActorOfClass` "/Game/BluePrints/Control/BP_ThirdPersonCharacter.BP_ThirdPersonCharacter_C"))
  (set `self.CurrentPlayer` _returnvalue)
  (`/Game/Widget/WB_HUD.SetAsPlayer_Event` (`self.Current WB`))
  (`/Game/BluePrints/Control/BP_ThirdPersonCharacter.SetView_Event` (`self.CurrentPlayer`))
  (`/Game/BluePrints/Control/BP_ThirdPersonCharacter.CheckOverlappingActors` (`self.CurrentPlayer`))
  (set `/Game/BluePrints/Control/BP_ThirdPersonCharacter.PlayerSpawned` true (`self.CurrentPlayer`))
  (`/Game/BluePrints/Camera/BP_Camera.SetCameraAtStart` (`/Game/BluePrints/Control/BP_ThirdPersonCharacter.CameraBPRef` (`self.CurrentPlayer`)))
  (bind _returnvalue_2 (`GameplayStatics.GetActorOfClass` "/Game/BluePrints/Camera/BP_Camera.BP_Camera_C"))
  (`/Game/BluePrints/Camera/BP_Camera.SetStartPos_Event` _returnvalue_2))

(event `HandleIntroduction_Event`
  (bind _currentplayer (`self.CurrentPlayer`))
  ;[0.6406 0.04338 0.04338] Handle Introduction, Play it if first time.
  (bind _returnvalue (`GameplayStatics.GetActorOfClass` "/Game/BluePrints/System/SoundManager.SoundManager_C"))
  (`/Game/BluePrints/System/SoundManager.PlayLevelTheme` _returnvalue)
  (if (`self.IntroPlayedForLevel`)
    (`/Game/BluePrints/Control/BP_ThirdPersonCharacter.GiveControl_Event` _currentplayer)
    (else
      (`/Game/BluePrints/Control/BP_ThirdPersonCharacter.DoIntro_Event` _currentplayer)
      (bind _returnvalue_2 (`|CreateWidget` "/Game/Widget/WB_Transition.WB_Transition_C"))
      (`UserWidget.AddToViewport` _returnvalue_2 0)
      (set `self.IntroPlayedForLevel` true))))

(event `HandleCollectables_Event`
  ;[1 0.8796 0.2708] Handle Collected Collectables
  (`|ExecutionSequence`
    (:`then_0`
      (bind _outactors (`GameplayStatics.GetAllActorsOfClass` "/Game/BluePrints/Interactable/Collectable/BP_Child_CollectableRare.BP_Child_CollectableRare_C"))
      (for _array_element _outactors
        (if (`KismetArrayLibrary.Array_Contains` (`self.CollectablesLevel`) (`KismetSystemLibrary.GetObjectName` _array_element))
          (`self.K2_DestroyActor` _array_element))))
    (:`then_1`
      (bind _outactors_2 (`GameplayStatics.GetAllActorsOfClass` "/Game/BluePrints/Interactable/Collectable/BP_Child_CollectableClassic.BP_Child_CollectableClassic_C"))
      (for _array_element_2 _outactors_2
        (`/Engine/EditorBlueprintResources/StandardMacros.IncrementInt` (`self.MaxCollectables`)
          (:`  `
            (if (`KismetArrayLibrary.Array_Contains` (`self.SavedCollectables`) (`KismetSystemLibrary.GetObjectName` _array_element_2))
              (`self.K2_DestroyActor` _array_element_2))))))
    (:`then_2`
      (bind _outactors_3 (`GameplayStatics.GetAllActorsOfClass` "/Game/BluePrints/Interactable/Collectable/BP_BreakableObject.BP_BreakableObject_C"))
      (for _array_element_3 _outactors_3
        (set `self.MaxCollectables` (+ (`/Game/BluePrints/Interactable/Collectable/BP_BreakableObject.CollectSpawns` _array_element_3) (`self.MaxCollectables`)))
        (if (`KismetArrayLibrary.Array_Contains` (`self.SavedCrates`) (`KismetSystemLibrary.GetObjectName` _array_element_3))
          (`self.K2_DestroyActor` _array_element_3))))
    (:`then_3`
      (bind _outactors_4 (`GameplayStatics.GetAllActorsOfClass` "/Game/BluePrints/Interactable/Collectable/BP_BreakableObjectBox.BP_BreakableObjectBox_C"))
      (for _array_element_4 _outactors_4
        (set `self.MaxCollectables` (+ (`/Game/BluePrints/Interactable/Collectable/BP_BreakableObjectBox.CollectSpawns` _array_element_4) (`self.MaxCollectables`)))
        (if (`KismetArrayLibrary.Array_Contains` (`self.SavedCrates`) (`KismetSystemLibrary.GetObjectName` _array_element_4))
          (`self.K2_DestroyActor` _array_element_4))))))

(fn `UserConstructionScript`)