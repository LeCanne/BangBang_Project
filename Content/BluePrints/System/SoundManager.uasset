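; Central sound manager that plays menu, level, boss and win music, plus UI, wall-slide and water-state sound effects.
; Events start, stop or pause themes and effects, using audio components or one-shot 2D sounds.
; Tick times the level and boss intros while their flags are set, then starts each loop once at a fixed offset.
; Stopping the level theme resets both timers and DoOnce gates.
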(event `self.ReceiveTick`
  (params (DeltaSeconds :type "Float (single-precision)"))
  ;[1 1 1] Event_Tick
  (`|ExecutionSequence`
    (:`then_0`
      (bind _returnvalue (>= (stale _output_get) 8.14))
      (if (and (`self.IsLevel`) (not _returnvalue))
        (bind _output_get (set `self.TimerLevel` (+ DeltaSeconds (`self.TimerLevel`))))
        (`KismetSystemLibrary.PrintString` (`KismetStringLibrary.Conv_DoubleToString` _output_get))
        (if _returnvalue
          (`/Engine/EditorBlueprintResources/StandardMacros.DoOnce` false :!label _label
            (:`Completed`
              (`AudioComponent.Play` (`self.Level_ThemeLoop`) 0.0))))))
    (:`then_1`
      (bind _returnvalue_2 (>= (stale _output_get_2) 10.28))
      (if (and (`self.IsBoss`) (not _returnvalue_2))
        (bind _output_get_2 (set `self.TimerBoss` (+ DeltaSeconds (`self.TimerBoss`))))
        (if _returnvalue_2
          (`/Engine/EditorBlueprintResources/StandardMacros.DoOnce` false :!label _label_2
            (:`Completed`
              (`AudioComponent.Play` (`self.Boss_ThemeLoop`) 0.0))))))))

(event `ResetMusic`
  ;[1 1 1] Event_Tick
  (set `self.TimerLevel` 0.0)
  (set `self.TimerBoss` 0.0)
  (`|ExecutionSequence`
    (:`then_0`
      (goto _label :!via `Reset`))
    (:`then_1`
      (goto _label_2 :!via `Reset`))))

(event `self.ReceiveBeginPlay`
  ;[1 1 1] BeginPlay
  (bind _returnvalue (`GameplayStatics.GetActorOfClass` "/Game/BluePrints/Control/BP_ThirdPersonCharacter.BP_ThirdPersonCharacter_C"))
  (set `self.Player` _returnvalue))

(event `StopLevelTheme`
  ;[0.2179 0.09202 1] Event_Music
  ;;[1 1 1] Level/Win
  (`self.ResetMusic`)
  (`AudioComponent.Stop` (`self.Level_ThemeIntro`))
  (`AudioComponent.Stop` (`self.Level_ThemeLoop`)))

(event `PlayMenuTheme`
  ;[0.2179 0.09202 1] Event_Music
  ;;[1 1 1] MainMenu
  (`AudioComponent.Play` (`self.Menu_Theme`) 0.0))

(event `PlayLevelTheme`
  ;[0.2179 0.09202 1] Event_Music
  ;;[1 1 1] Level/Win
  (if (or (`AudioComponent.IsPlaying` (`self.Boss_ThemeIntro`)) (`AudioComponent.IsPlaying` (`self.Boss_ThemeLoop`)))
    (set `self.IsLevel` false)
    (else
      (`AudioComponent.Play` (`self.Level_ThemeIntro`) 0.0))))

(event `StopMenuTheme`
  ;[0.2179 0.09202 1] Event_Music
  ;;[1 1 1] MainMenu
  (`AudioComponent.Stop` (`self.Menu_Theme`)))

(event `PlayWinTheme`
  ;[0.2179 0.09202 1] Event_Music
  ;;[1 1 1] Level/Win
  (`AudioComponent.Stop` (`self.Level_ThemeIntro`))
  (`AudioComponent.Stop` (`self.Level_ThemeLoop`))
  (`AudioComponent.Stop` (`self.Boss_ThemeIntro`))
  (`AudioComponent.Stop` (`self.Boss_ThemeLoop`))
  (`GameplayStatics.PlaySound2D` (`self.WinTheme`) 1.0 1.0 0.0 null null))

(event `PlayBossTheme`
  ;[0.2179 0.09202 1] Event_Music
  ;;[1 1 1] Boss
  (`AudioComponent.Play` (`self.Boss_ThemeIntro`) 0.0))

(event `StopBossTheme`
  ;[0.2179 0.09202 1] Event_Music
  ;;[1 1 1] Boss
  (`AudioComponent.Stop` (`self.Boss_ThemeIntro`))
  (`AudioComponent.Stop` (`self.Boss_ThemeLoop`)))

(event `PauseUnpauseMusic_Event`
  ;[0.2179 0.09202 1] Event_Music
  ;;[1 1 1] Level/Win
  (bind _isa (`/Engine/EditorBlueprintResources/StandardMacros.FlipFlop`)
    (:`A`
      _)
    (:`B`
      _))
  (`AudioComponent.SetPaused` (`self.Level_ThemeIntro`) _isa)
  (`AudioComponent.SetPaused` (`self.Level_ThemeLoop`) _isa))

(event `PlayWallSlide`
  ;[0.1344 1 0.6052] Event_SFX_WallSlide
  (`AudioComponent.Play` (`self.SFX_WallSlide`) 0.0))

(event `PlaySelectButton`
  (params (InInt :type Integer))
  ;[1 0.1448 0.1448] Event_Interface
  (bind _returnvalue (`GameplayStatics.CreateSound2D` (`self.SFX_SelectButton`) 1.0 1.0 0.0 null))
  (`AudioComponent.SetIntParameter` _returnvalue "NbSelectButton" InInt)
  (`AudioComponent.Play` _returnvalue 0.0))

(event `PlayChangeButton`
  (params (InFloat :type "Float (single-precision)"))
  ;[1 0.1448 0.1448] Event_Interface
  (`GameplayStatics.PlaySound2D` (`self.SFX_ChangeButton`) 1.0 1.0 0.0 null null))

(event `StopWallSlide`
  ;[0.1344 1 0.6052] Event_SFX_WallSlide
  (`AudioComponent.Stop` (`self.SFX_WallSlide`)))

(event `PlaySelectLevel`
  ;[1 0.1448 0.1448] Event_Interface
  (`GameplayStatics.PlaySound2D` (`self.SFX_SelectLevel`) 1.0 1.0 0.0 null null)
  (`self.StopMenuTheme`))

(fn `EtatEau`
  (`GameplayStatics.PlaySound2D` (`self.SFX_Eteint`) 1.0 1.0 0.0 null null))

(fn `UserConstructionScript`)