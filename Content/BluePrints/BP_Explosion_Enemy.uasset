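; BP_Explosion_Enemy is a short-lived explosion actor, named for enemies, that plays a growing blast effect with sound.
; On BeginPlay it plays the explosion sound at world origin and starts a Timeline at AnimationSpeed rate.
; Each Timeline update sets the visible sphere and collision sphere to the same curve-driven scale and calls Activate on the Niagara effect.
; The actor destroys itself after a short delay once the Timeline finishes.
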(event `self.ReceiveBeginPlay`
  ;[1 1 1] Explosion avec une Timeline + Son
  (`TimelineComponent.SetPlayRate` (`self.Timeline`) (`self.AnimationSpeed`))
  (`GameplayStatics.PlaySoundAtLocation` "/Game/0_Dossiers_perso/Charles/Audio/SFX/Sound_Cue/SC_explosion.SC_explosion" (0.0 0.0 0.0) (struct) 1.0 1.0 0.0 null null null null)
  (bind (_direction _scale) (`Timeline|Timeline`)
    (:`Update`
      (`|ExecutionSequence`
        (:`then_0`
          (`SceneComponent.SetWorldScale3D` (`self.Sphere`) (`KismetMathLibrary.Conv_DoubleToVector` _scale))
          (`ActorComponent.Activate` (`self.NS_Explosion`) false))
        (:`then_1`
          (`SceneComponent.SetWorldScale3D` (`self.SphereCollision_Explosion`) (`KismetMathLibrary.Conv_DoubleToVector` _scale)))))
    (:`Finished`
      (`KismetSystemLibrary.Delay` 3.0)
      (`self.K2_DestroyActor`))))

(fn `UserConstructionScript`)