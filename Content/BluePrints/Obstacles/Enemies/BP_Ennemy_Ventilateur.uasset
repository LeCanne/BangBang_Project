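; Fan enemy that chases the player character on sight and blows physics objects with wind.
; Pawn sensing triggers an AI move to the player; the move's immediate output sets walking mode and plays a timeline that animates a scene component's Z scale.
; Every tick, physics-simulating components overlapping the cylinder receive a randomly varied force along the actor's forward vector.
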(event `self.ReceiveBeginPlay`
  (bind _returnvalue (`GameplayStatics.GetActorOfClass` "/Game/BluePrints/System/SoundManager.SoundManager_C"))
  (set `self.SoundManager` _returnvalue))

(event `self.ReceiveActorBeginOverlap`
  (params (OtherActor :type "Actor Object Reference")))

(event `self.PawnSensing.OnSeePawn`
  (params (Pawn :type "Pawn Object Reference"))
  (bind _asbp_third_person_character (cast `/Game/BluePrints/Control/BP_ThirdPersonCharacter` Pawn))
  (`|AIMoveTo` self (0.0 0.0 0.0) _asbp_third_person_character 10.0
    (:`then`
      (`CharacterMovementComponent.SetMovementMode` (`self.CharacterMovement`) "MOVE_Walking" 0)
      (bind (_direction _wind) (`Timeline|Timeline`)
        (:`Update`
          (`SceneComponent.SetWorldScale3D` (`self.Scene`) (`KismetMathLibrary.MakeVector` 0.5 0.5 _wind)))))))

(event `self.ReceiveTick`
  (params (DeltaSeconds :type "Float (single-precision)"))
  (for _array_element (`PrimitiveComponent.GetOverlappingComponents` (`self.Cylinder`))
    (if (`SceneComponent.IsSimulatingPhysics` _array_element "None")
      (`PrimitiveComponent.AddForceAtLocation` _array_element (* (`KismetMathLibrary.GetForwardVector` (`self.K2_GetActorRotation`)) (* (* (`self.WindStrength`) (`KismetMathLibrary.RandomFloatInRange` 0.8 1.4)) 1.0)) (`SceneComponent.K2_GetComponentLocation` _array_element) "None"))))

(fn `UserConstructionScript`)