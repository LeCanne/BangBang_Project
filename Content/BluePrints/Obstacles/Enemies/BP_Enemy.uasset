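; BP_Enemy is an enemy that chases the player and explodes on contact.
; PawnSensing sets a seeing flag and starts AIMoveTo toward the player, also setting movement mode to None and recoloring its text.
; Any overlap end retargets movement to itself and clears the flag.
; Player or explosion overlap triggers Death, spawning BP_Explosion_Enemy, so explosions can chain between enemies.
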(event `self.PawnSensing.OnSeePawn`
  (params (Pawn :type "Pawn Object Reference"))
  ;[1 0.399 0.399] Détecter le joueur
  (set `self.IsSeeingPlayer` true)
  (`self.Follow Player`))

(event `Follow Player`
  ;[1 0.399 0.399] Détecter le joueur
  (if (`self.IsSeeingPlayer`)
    ;;[1 1 1] Phase Agro sur le joueur
    (`|AIMoveTo` self (0.0 0.0 0.0) (`GameplayStatics.GetPlayerCharacter` 0)
      (:`then`
        (`CharacterMovementComponent.SetMovementMode` (`self.CharacterMovement`) "MOVE_None" 0)
        (`TextRenderComponent.SetTextRenderColor` (`self.TextRender`) (make `Color` 0 0 0 100))))))

(event `Death`
  ;[0 1 0.5204] Mort (en teste)
  (`self.K2_DestroyActor`)
  (`|SpawnActorFromClass` "/Game/BluePrints/BP_Explosion_Enemy.BP_Explosion_Enemy_C" (`self.GetTransform`) "Undefined" "MultiplyWithRoot" null null))

(event `self.ReceiveActorEndOverlap`
  (params (OtherActor :type "Actor Object Reference"))
  ;[0 0.6955 1] Détection via la collision
  ;;[1 1 1] Sortie de la collision
  (`GameplayStatics.GetActorOfClass` "/Game/BluePrints/Control/BP_ThirdPersonCharacter.BP_ThirdPersonCharacter_C")
  (`|AIMoveTo` self (0.0 0.0 0.0) self
    (:`then`
      (set `self.IsSeeingPlayer` false))))

(event `self.ReceiveActorBeginOverlap`
  (params (OtherActor :type "Actor Object Reference"))
  ;[0 0.6955 1] Détection via la collision
  ;;[1 1 1] Entre de la collision
  (cast `/Game/BluePrints/Control/BP_ThirdPersonCharacter` OtherActor)
  (`self.Death` :!label _label))

(event `self.CapsuleComponent.OnComponentBeginOverlap`
  (params (OverlappedComponent :type "PrimitiveComponent Object Reference") (OtherActor :type "Actor Object Reference") (OtherComp :type "PrimitiveComponent Object Reference") (OtherBodyIndex :type Integer) (bFromSweep :type Boolean) (SweepResult :type "HitResult Structure (by ref)"))
  ;[0 0.6955 1] Détection via la collision
  ;;[1 1 1] Entre de la collision
  (cast `/Game/BluePrints/BP_Explosion_Enemy` (stale `self.ReceiveActorBeginOverlap` OtherActor))
  (goto _label))

(fn `UserConstructionScript`)