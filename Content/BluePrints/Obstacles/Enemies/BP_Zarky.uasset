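; BP_Zarky is an enemy character that chases the player and knocks them away on contact with its attack radius.
; Hearing-radius overlap starts smooth yaw turning, while PawnSensing sight triggers a one-time hop and tick-driven forward movement with text and sound cues.
; Leaving the ignore radius clears both states and re-arms the hop.
; Overlapping an EXPLOSION-tagged component spawns an enemy explosion and destroys it.
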(event `self.ReceiveBeginPlay`
  ;[1 1 1] Get Sound Manager
  (bind _returnvalue (`GameplayStatics.GetActorOfClass` "/Game/BluePrints/System/SoundManager.SoundManager_C"))
  (set `self.Sound Manager` _returnvalue))

(event `self.ReceiveTick`
  (params (DeltaSeconds :type "Float (single-precision)"))
  ;[1 1 1] MainBehavior
  (`|ExecutionSequence`
    (:`then_0`
      (`self.TurnTowardsPlayer_Event`))
    (:`then_2`
      (`self.Follow Player`))))

(event `self.AcceptanceRadius.OnComponentBeginOverlap`
  (params (OverlappedComponent :type "PrimitiveComponent Object Reference") (OtherActor :type "Actor Object Reference") (OtherComp :type "PrimitiveComponent Object Reference") (OtherBodyIndex :type Integer) (bFromSweep :type Boolean) (SweepResult :type "HitResult Structure (by ref)"))
  ;[1 1 1] AIBehavior
  ;;[0 1 0.317] Player Heard
  (bind _asbp_third_person_character (cast `/Game/BluePrints/Control/BP_ThirdPersonCharacter` OtherActor))
  (set `self.CurrentTarget` _asbp_third_person_character)
  (set `self.TurnToPlayer` true))

(event `self.PawnSensing.OnSeePawn`
  (params (Pawn :type "Pawn Object Reference"))
  ;[1 1 1] AIBehavior
  ;;[1 0 0.7105] See Player
  (bind _asbp_third_person_character (cast `/Game/BluePrints/Control/BP_ThirdPersonCharacter` Pawn))
  (set `self.CurrentTarget` _asbp_third_person_character)
  (set `self.IsSeeingPlayer` true))

(event `TurnTowardsPlayer_Event`
  (bind (_returnvalue_roll _returnvalue_pitch _returnvalue_yaw) (`KismetMathLibrary.BreakRotator` (`KismetMathLibrary.RInterpTo` (`SceneComponent.K2_GetComponentRotation` (`self.CapsuleComponent`)) (`KismetMathLibrary.FindLookAtRotation` (`SceneComponent.K2_GetComponentLocation` (`self.CapsuleComponent`)) (`SceneComponent.K2_GetComponentLocation` (`Actor.RootComponent` (`self.CurrentTarget`)))) (`GameplayStatics.GetWorldDeltaSeconds`) 2.0)))
  ;[1 1 1] AIBehavior
  ;;[1 0.3281 0.3281] Turn Towards Player
  (if (`self.TurnToPlayer`)
    (`SceneComponent.K2_SetWorldRotation` (`self.CapsuleComponent`) (`KismetMathLibrary.MakeRotator` 0.0 0.0 _returnvalue_yaw) false false)))

(event `Follow Player`
  ;[1 1 1] AIBehavior
  ;;[1 0.1629 0.1354] Move To Player
  (if (`self.IsSeeingPlayer`)
    (`|ExecutionSequence`
      (:`then_0`
        (`/Engine/EditorBlueprintResources/StandardMacros.DoOnce` false :!label _label
          (:`Completed`
            (`CharacterMovementComponent.AddImpulse` (`self.CharacterMovement`) (0.0 0.0 200.0) true))))
      (:`then_1`
        (if (`NavMovementComponent.IsMovingOnGround` (`self.CharacterMovement`))
          (`PawnMovementComponent.AddInputVector` (`self.CharacterMovement`) (* (`SceneComponent.GetForwardVector` (`self.CapsuleComponent`)) (* (`self.Speed`) (`GameplayStatics.GetWorldDeltaSeconds`))) true)
          (`SceneComponent.SetVisibility` (`self.TextRender`) true false)
          (`GameplayStatics.SpawnSoundAtLocation` null (`self.K2_GetActorLocation` self) (struct) 1.0 1.0 0.0 null null))))))

(event `ResetPlayerPos_Event`
  ;[1 1 1] AIBehavior
  ;;[1 0.1629 0.1354] Move To Player
  (goto _label :!via `Reset`))

(event `self.AttackRadius.OnComponentBeginOverlap`
  (params (OverlappedComponent :type "PrimitiveComponent Object Reference") (OtherActor :type "Actor Object Reference") (OtherComp :type "PrimitiveComponent Object Reference") (OtherBodyIndex :type Integer) (bFromSweep :type Boolean) (SweepResult :type "HitResult Structure (by ref)"))
  (bind _capsulecomponent (`self.CapsuleComponent`))
  ;[1 1 1] AIBehavior
  ;;[1 0.01949 0] Attaque
  (bind _asbp_third_person_character (cast `/Game/BluePrints/Control/BP_ThirdPersonCharacter` OtherActor))
  (`CharacterMovementComponent.AddImpulse` (`Character.CharacterMovement` _asbp_third_person_character) (+ (* (`SceneComponent.GetForwardVector` _capsulecomponent) (`self.StrenghtForward`)) (* (`SceneComponent.GetUpVector` _capsulecomponent) (`self.StrenghtUp`))) true))

(event `self.IgnoreRadius.OnComponentEndOverlap`
  (params (OverlappedComponent :type "PrimitiveComponent Object Reference") (OtherActor :type "Actor Object Reference") (OtherComp :type "PrimitiveComponent Object Reference") (OtherBodyIndex :type Integer))
  ;[1 1 1] AIBehavior
  ;;[0 0.3946 1] Ignore Player if far
  (cast `/Game/BluePrints/Control/BP_ThirdPersonCharacter` OtherActor)
  (set `self.TurnToPlayer` false)
  (set `self.IsSeeingPlayer` false)
  (`self.ResetPlayerPos_Event`))

(event `self.CapsuleComponent.OnComponentBeginOverlap`
  (params (OverlappedComponent :type "PrimitiveComponent Object Reference") (OtherActor :type "Actor Object Reference") (OtherComp :type "PrimitiveComponent Object Reference") (OtherBodyIndex :type Integer) (bFromSweep :type Boolean) (SweepResult :type "HitResult Structure (by ref)"))
  ;[1 1 1] AIBehavior
  ;;[1 0.08333 0.08333] DamageProcess
  (if (`ActorComponent.ComponentHasTag` OtherComp "EXPLOSION")
    (`self.Death`)))

(event `Death`
  ;[1 1 1] AIBehavior
  ;;[0 1 0.5204] Mort
  (`/Engine/EditorBlueprintResources/StandardMacros.DoOnce` false
    (:`Completed`
      (`|SpawnActorFromClass` "/Game/BluePrints/Interactable/BP_Explosion_Enemy.BP_Explosion_Enemy_C" (`self.GetTransform`) "Undefined" "MultiplyWithRoot" null null)
      (`self.K2_DestroyActor`))))

(fn `UserConstructionScript`)