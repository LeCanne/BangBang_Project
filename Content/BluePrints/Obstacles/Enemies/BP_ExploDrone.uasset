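; Exploding drone enemy that patrols a spline each tick, looping on closed paths and ping-ponging on open ones.
; Hitting its body stuns and knocks back the player, gated by a grace period.
; Explosions overlapping its HurtBox kill it; player explosions also call GiveExplosionEvent on the player and launch them upward.
; Death spawns an enemy explosion that can chain to other drones, hides it, then respawns it after a delay, resetting DoOnce gates.
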(event `self.ReceiveBeginPlay`)

(event `self.ReceiveTick`
  (params (DeltaSeconds :type "Float (single-precision)"))
  (`self.MoveOnSpline_Event`))

(event `self.HurtBox.OnComponentBeginOverlap`
  (params (OverlappedComponent :type "PrimitiveComponent Object Reference") (OtherActor :type "Actor Object Reference") (OtherComp :type "PrimitiveComponent Object Reference") (OtherBodyIndex :type Integer) (bFromSweep :type Boolean) (SweepResult :type "HitResult Structure (by ref)"))
  ;[1 1 1] Enemy Exploded
  (`KismetSystemLibrary.DelayUntilNextTick`)
  (`|ExecutionSequence`
    (:`then_0`
      (bind _asbp_explosion_enemy (cast `/Game/BluePrints/Interactable/BP_Explosion_Enemy` OtherActor))
      (switch `/Game/BluePrints/Interactable/Enum_Explosion` (`/Game/BluePrints/Interactable/BP_Explosion_Enemy.ExplosionType` _asbp_explosion_enemy)
        (:`NewEnumerator0`
          _)
        (:`NewEnumerator1`
          (`/Engine/EditorBlueprintResources/StandardMacros.DoOnce` false :!label _label
            (:`Completed`
              (bind _returnvalue (`GameplayStatics.GetActorOfClass` "/Game/BluePrints/Control/BP_ThirdPersonCharacter.BP_ThirdPersonCharacter_C"))
              (`/Game/BluePrints/Control/BP_ThirdPersonCharacter.GiveExplosion_Event` _returnvalue)
              (`/Game/BluePrints/Control/BP_ThirdPersonCharacter.ThrowPlayer_Event` _returnvalue (0.0 0.0 500.0) false false)))))
      (`self.Death_Event` :!label _label_2))
    (:`then_1`
      (if (`ActorComponent.ComponentHasTag` OtherComp "EXPLOSIONJOUEUR")
        (goto _label)))
    (:`then_2`
      (if (`ActorComponent.ComponentHasTag` OtherComp "EXPLOSION")
        (goto _label_2)))))

(event `ResetStates_Event`
  ;[1 1 1] Enemy Exploded
  (goto _label :!via `Reset`))

(event `Death_Event`
  (bind _returnvalue (`SceneComponent.K2_GetComponentLocation` (`self.Enemy`)))
  ;[1 0 0] Death Event
  (`/Engine/EditorBlueprintResources/StandardMacros.DoOnce` false :!label _label_3
    (:`Completed`
      (`AudioComponent.Stop` (`self.SFX_Flame`))
      (`GameplayStatics.PlaySound2D` "/Game/0_Dossiers_perso/Charles/Audio/Sound_Cue/SFX/Ennemy/A_Robot_Death_Cue.A_Robot_Death_Cue" 1.0 1.0 0.0 null null)
      (`|SpawnActorFromClass` "/Game/BluePrints/Interactable/BP_Explosion_Enemy.BP_Explosion_Enemy_C" (`KismetMathLibrary.MakeTransform` (`SceneComponent.K2_GetComponentLocation` (`self.Enemy`))) "Undefined" "MultiplyWithRoot" null null)
      (`NiagaraFunctionLibrary.SpawnSystemAtLocation` "/Game/0_Dossiers_perso/Valentin/Niagara/NS_Explo_Enemy.NS_Explo_Enemy" _returnvalue)
      (`NiagaraFunctionLibrary.SpawnSystemAtLocation` "/Game/0_Dossiers_perso/Valentin/Niagara/NS_blastFlyzark.NS_blastFlyzark" _returnvalue)
      (`SceneComponent.SetVisibility` (`self.Enemy`) false true)
      (`self.SetActorEnableCollision` false)
      (`KismetSystemLibrary.Delay` 2.0)
      (`self.Respawn`))))

(event `ResetDeath_Event`
  ;[1 0 0] Death Event
  (goto _label_3 :!via `Reset`))

(event `Respawn`
  ;[0.8293 0 1] Respawn
  (`ActorComponent.Activate` (`self.NS_pouf`) true)
  (`SceneComponent.SetVisibility` (`self.Enemy`) true true)
  (`self.SetActorEnableCollision` true)
  (`self.ResetStates_Event`)
  (`self.ResetDeath_Event`)
  (`AudioComponent.Play` (`self.SFX_Flame`) 0.0))

(event `self.Enemy.OnComponentHit`
  (params (HitComponent :type "PrimitiveComponent Object Reference") (OtherActor :type "Actor Object Reference") (OtherComp :type "PrimitiveComponent Object Reference") (NormalImpulse :type "Vector Structure") (Hit :type "HitResult Structure (by ref)"))
  (bind _enemy (`self.Enemy`))
  ;[1 0.2504 0.0498] Attack Player
  (bind _asbp_third_person_character (cast `/Game/BluePrints/Control/BP_ThirdPersonCharacter` OtherActor))
  (`/Engine/EditorBlueprintResources/StandardMacros.DoOnce` false :!label _label_4
    (:`Completed`
      (`/Game/BluePrints/Control/BP_ThirdPersonCharacter.StunPlayerFor_Event` _asbp_third_person_character 0.5)
      (bind (_returnvalue_x _returnvalue_y) (`KismetMathLibrary.BreakVector` (`KismetMathLibrary.Normal` (- (`SceneComponent.K2_GetComponentLocation` (`Character.CapsuleComponent` _asbp_third_person_character)) (`SceneComponent.K2_GetComponentLocation` _enemy)))))
      (`/Game/BluePrints/Control/BP_ThirdPersonCharacter.ThrowPlayer_Event` _asbp_third_person_character (+ (* (`KismetMathLibrary.MakeVector` _returnvalue_x _returnvalue_y) (`self.StrenghtForward`)) (* (`SceneComponent.GetUpVector` _enemy) (`self.StrenghtUp`))) true false)
      (`KismetSystemLibrary.Delay` (`self.GracePeriod`))
      (`self.ResetHit_Event`))))

(event `ResetHit_Event`
  ;[1 0.2504 0.0498] Attack Player
  (goto _label_4 :!via `Reset`))

(event `MoveOnSpline_Event`
  (bind _returnvalue (* (`GameplayStatics.GetWorldDeltaSeconds`) (* (`self.Speed`) 100.0)))
  ;[1 1 1] Move On Spline
  (if (`SplineComponent.IsClosedLoop` (`self.SplinePath`))
    (bind _output_get (set `self.Distance` (+ (`self.Distance`) _returnvalue) :!label _label_5))
    (`SceneComponent.K2_SetWorldLocation` (`self.Enemy`) (`SplineComponent.GetLocationAtDistanceAlongSpline` (`self.SplinePath`) _output_get "World") false false)
    (if (>= (`self.Distance`) (`SplineComponent.GetSplineLength` (`self.SplinePath`)))
      (if (`SplineComponent.IsClosedLoop` (`self.SplinePath`))
        (set `self.Distance` 0.0)
        (else
          (set `self.Backtrack` false))))
    (elif (`self.Backtrack`)
      (goto _label_5)
      (else
        (bind _output_get_2 (set `self.Distance` (+ (* _returnvalue -1.0) (`self.Distance`))))
        (`SceneComponent.K2_SetWorldLocation` (`self.Enemy`) (`SplineComponent.GetLocationAtDistanceAlongSpline` (`self.SplinePath`) _output_get_2 "World") false false)
        (if (<= (`self.Distance`) 0.0)
          (set `self.Backtrack` true))))))

(fn `UserConstructionScript`)