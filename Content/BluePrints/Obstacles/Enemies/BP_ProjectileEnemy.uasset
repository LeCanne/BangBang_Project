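; Robot enemy that turns toward the player, optionally chases them, and fires physics projectiles.
; Overlap radii toggle turning, while Tick drives rotation, a one-shot detect sound, AI movement once PawnSensing sees the player, and shooting throttled by DoOnce plus Delay.
; Entering AcceptanceRadius enables shooting, which is never switched off.
; Contact with an EXPLOSION-tagged component destroys it with effects and can decrement the player's JumpCount.
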(event `self.PawnSensing.OnSeePawn`
  (params (Pawn :type "Pawn Object Reference"))
  ;[1 0.399 0.399] Détecter le joueur
  (cast `/Game/BluePrints/Control/BP_ThirdPersonCharacter` Pawn)
  (set `self.IsSeeingPlayer` true))

(event `Follow Player`
  ;[1 0.399 0.399] Détecter le joueur
  (if (`self.IsSeeingPlayer`)
    ;;[1 1 1] Phase Agro sur le joueur
    (`|AIMoveTo` null (0.0 0.0 0.0) null 10.0
      (:`then`
        (`CharacterMovementComponent.SetMovementMode` (`self.CharacterMovement`) "MOVE_Walking" 0)
        (`SceneComponent.SetVisibility` (`self.TextRender`) true false)))))

(event `self.ReceiveTick`
  (params (DeltaSeconds :type "Float (single-precision)"))
  (bind _turntoplayer (`self.TurnToPlayer`))
  (bind _capsulecomponent (`self.CapsuleComponent`))
  (bind (_returnvalue_roll _returnvalue_pitch _returnvalue_yaw) (`KismetMathLibrary.BreakRotator` (`KismetMathLibrary.RInterpTo` (`SceneComponent.K2_GetComponentRotation` _capsulecomponent) (`KismetMathLibrary.FindLookAtRotation` (`SceneComponent.K2_GetComponentLocation` _capsulecomponent) (`SceneComponent.K2_GetComponentLocation` (`Actor.RootComponent` (`self.BP_ThirdPersonCharacter`)))) DeltaSeconds 2.0)))
  ;[1 0.399 0.399] Détecter le joueur
  (`|ExecutionSequence`
    (:`then_0`
      (if (and _turntoplayer (`self.IsMove`))
        (`self.Follow Player`)
        (`SceneComponent.K2_SetWorldRotation` (`self.CapsuleComponent`) (`KismetMathLibrary.MakeRotator` 0.0 0.0 _returnvalue_yaw) false false :!label _label)
        (`self.Play Sound`)
        (elif _turntoplayer
          (goto _label))))
    (:`then_1`
      (if (`self.ShootPlayer`)
        (`/Engine/EditorBlueprintResources/StandardMacros.DoOnce` false :!label _label_2
          (:`Completed`
            (`self.Shoot`)
            (`KismetSystemLibrary.Delay` 5.0)
            (goto _label_2 :!via `Reset`)))))))

(event `Death`
  ;[0 1 0.5204] Mort (en teste)
  (`self.K2_DestroyActor`)
  (`|SpawnActorFromClass` "/Game/BluePrints/Interactable/BP_Explosion_Enemy.BP_Explosion_Enemy_C" (`self.GetTransform`) "Undefined" "MultiplyWithRoot" null null)
  (`GameplayStatics.PlaySound2D` "/Game/0_Dossiers_perso/Charles/Audio/Sound_Cue/SFX/Ennemy/A_Robot_Death_Cue.A_Robot_Death_Cue" 1.0 1.0 0.0 null null))

(event `Play Sound`
  ;[1 1 1] Discovers player
  (`/Engine/EditorBlueprintResources/StandardMacros.DoOnce` false :!label _label_3
    (:`Completed`
      (`GameplayStatics.SpawnSoundAtLocation` "/Game/0_Dossiers_perso/Charles/Audio/Sound_Cue/SFX/Ennemy/A_Robot_Detect_Cue.A_Robot_Detect_Cue" (`self.K2_GetActorLocation` self) (struct) 1.0 1.0 0.0 null null))))

(event `self.ReceiveActorEndOverlap`
  (params (OtherActor :type "Actor Object Reference"))
  ;[0 0.6955 1] Détection via la collision
  ;;[1 1 1] Sortie de la collision
  (cast `/Game/BluePrints/Control/BP_ThirdPersonCharacter` OtherActor)
  (`|AIMoveTo` self (0.0 0.0 0.0) self
    (:`then`
      (set `self.IsSeeingPlayer` false)
      (`SceneComponent.SetVisibility` (`self.TextRender`) false false)
      ;[1 0.399 0.399] Détecter le joueur
      ;;[1 1 1] Phase Agro sur le joueur
      (`self.Reset Sound`))))

(event `Reset Sound`
  ;[1 1 1] Discovers player
  (goto _label_3 :!via `Reset`))

(event `Shoot`
  (bind _force_pulse (`self.Force Pulse`))
  (bind _returnvalue (* (`KismetMathLibrary.Normal` (- (`self.K2_GetActorLocation` (`self.BP_ThirdPersonCharacter`)) (`SceneComponent.K2_GetComponentLocation` (`self.Arrow1`)))) (`KismetMathLibrary.MakeVector` _force_pulse _force_pulse _force_pulse)))
  ;[0 1 0.5204] Attaque
  (bind _returnvalue_2 (`|SpawnActorFromClass` "/Game/BluePrints/Obstacles/Enemies/BP_Projectile.BP_Projectile_C" (`SceneComponent.K2_GetComponentToWorld` (`self.Arrow1`)) "Undefined" "OverrideRootScale" null null))
  (set `self.Impulse` _returnvalue)
  (`PrimitiveComponent.AddImpulse` (`/Game/BluePrints/Obstacles/Enemies/BP_Projectile.Sphere` _returnvalue_2) _returnvalue "None" false))

(event `self.IgnoreRadius.OnComponentEndOverlap`
  (params (OverlappedComponent :type "PrimitiveComponent Object Reference") (OtherActor :type "Actor Object Reference") (OtherComp :type "PrimitiveComponent Object Reference") (OtherBodyIndex :type Integer))
  ;[0 0.6955 1] Détection via la collision
  ;;[1 1 1] Entre de la collision
  (cast `/Game/BluePrints/Control/BP_ThirdPersonCharacter` OtherActor)
  (set `self.TurnToPlayer` false))

(event `self.CapsuleComponent.OnComponentBeginOverlap`
  (params (OverlappedComponent :type "PrimitiveComponent Object Reference") (OtherActor :type "Actor Object Reference") (OtherComp :type "PrimitiveComponent Object Reference") (OtherBodyIndex :type Integer) (bFromSweep :type Boolean) (SweepResult :type "HitResult Structure (by ref)"))
  (bind _bp_thirdpersoncharacter (`self.BP_ThirdPersonCharacter`))
  ;[0 0.6955 1] Détection via la collision
  ;;[1 1 1] Entre de la collision
  (if (`ActorComponent.ComponentHasTag` OtherComp "EXPLOSION")
    (`|ExecutionSequence`
      (:`then_0`
        (`self.Death`))
      (:`then_1`
        ;[1 1 1] Donne 1 d'explosion
        (if (`/Game/BluePrints/Control/BP_ThirdPersonCharacter.IsExplode` _bp_thirdpersoncharacter)
          (set `/Game/BluePrints/Control/BP_ThirdPersonCharacter.IsExplode` false _bp_thirdpersoncharacter)
          (bind _result (`/Engine/EditorBlueprintResources/StandardMacros.DecrementInt` (`/Game/BluePrints/Control/BP_ThirdPersonCharacter.JumpCount` _bp_thirdpersoncharacter))
            (:`  `
              (set `/Game/BluePrints/Control/BP_ThirdPersonCharacter.JumpCount` _result _bp_thirdpersoncharacter))))))))

(event `self.AcceptanceRadius.OnComponentBeginOverlap`
  (params (OverlappedComponent :type "PrimitiveComponent Object Reference") (OtherActor :type "Actor Object Reference") (OtherComp :type "PrimitiveComponent Object Reference") (OtherBodyIndex :type Integer) (bFromSweep :type Boolean) (SweepResult :type "HitResult Structure (by ref)"))
  ;[0 0.6955 1] Détection via la collision
  ;;[1 1 1] Entre de la collision
  (bind _asbp_third_person_character (cast `/Game/BluePrints/Control/BP_ThirdPersonCharacter` OtherActor))
  (set `self.BP_ThirdPersonCharacter` _asbp_third_person_character)
  (set `self.TurnToPlayer` true)
  (set `self.ShootPlayer` true))

(fn `UserConstructionScript`)