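; Yzark boss enemy that activates when the player enters its detection zone and fights through a Tick-driven moving, punch, wind-shoot and hurt state machine.
; It follows the player along a spline, then picks punches or, at lower HP, cannon volleys that lead into punches.
; DoOnce gates and delays pace the attacks, and punches stun and launch the player.
; Player explosions on its hurtbox cost HP, throw the player back and eventually destroy it.
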(event `self.PlayerDetection.OnComponentBeginOverlap`
  (params (OverlappedComponent :type "PrimitiveComponent Object Reference") (OtherActor :type "Actor Object Reference") (OtherComp :type "PrimitiveComponent Object Reference") (OtherBodyIndex :type Integer) (bFromSweep :type Boolean) (SweepResult :type "HitResult Structure (by ref)"))
  ;[1 1 1] PlayerDetection
  (cast `/Game/BluePrints/Control/BP_ThirdPersonCharacter` OtherActor)
  (set `self.isActive` true))

(event `self.ReceiveBeginPlay`
  ;[1 1 1] Get Sound Manager & Original World Rotation
  (bind _returnvalue (`GameplayStatics.GetActorOfClass` "/Game/BluePrints/System/SoundManager.SoundManager_C"))
  (set `self.Sound Manager` _returnvalue)
  (set `self.OriginRotation` (`SceneComponent.K2_GetComponentRotation` (`self.CapsuleComponent`)))
  (set `self.ArrayMeshes` (`|MakeArray` (`self.BossYzark_Shoulder_R`) (`self.BossYzark_Hand_R`) (`self.BossYzark_Arm_R`) (`self.BossYzark_Shoulder_L`) (`self.BossYzark_Hand_L`) (`self.BossYzark_Arm_L`) (`self.Cannon`) (`self.BossYzark_Base`))))

(event `ResetRotation_Event`
  ;[1 1 1] MainBehavior
)

(event `self.ReceiveTick`
  (params (DeltaSeconds :type "Float (single-precision)"))
  ;[1 1 1] MainBehavior
  ;;[0.2961 0.2961 0.016] Switch Boss States
  (if (`self.isActive`)
    (`|ExecutionSequence`
      (:`then_0`
        (switch `/Game/BluePrints/Obstacles/Enemies/BossStates` (`self.StateBoss`)
          (:`NewEnumerator0`
            (`self.FollowPlayer_Event`))
          (:`NewEnumerator1`
            (`self.PunchPlayer_Event`))
          (:`NewEnumerator3`
            (`self.ShootPlayer_Event`))
          (:`NewEnumerator4`
            (`self.HurtBoss_Event`)))))))

(event `ChangeState_Event`
  (params (NewParam :type "/Game/BluePrints/Obstacles/Enemies/BossStates Enum" :default "NewEnumerator0"))
  ;[1 1 1] MainBehavior
  ;;[0.1195 0.1195 0.006512] Change State Event
  (set `self.StateBoss` NewParam)
  (bind (_direction _ultrafloattrack) (`Timeline|Timeline` :!via `PlayFromStart`)
    (:`Update`
      (`SceneComponent.K2_SetWorldRotation` (`self.CapsuleComponent`) (`KismetMathLibrary.RLerp` (`SceneComponent.K2_GetComponentRotation` (`self.CapsuleComponent`)) (`self.OriginRotation`) _ultrafloattrack true) false false))))

(event `FollowPlayer_Event`
  ;[1 1 1] AIBehavior
  ;;[0.6123 0.9601 1] Follow Player
  (bind _returnvalue (`GameplayStatics.GetActorOfClass` "/Game/BluePrints/Control/BP_ThirdPersonCharacter.BP_ThirdPersonCharacter_C"))
  (`SceneComponent.K2_SetWorldLocation` (`self.CapsuleComponent`) (`KismetMathLibrary.VInterpTo` (`SceneComponent.K2_GetComponentLocation` (`self.CapsuleComponent`)) (`SplineComponent.FindLocationClosestToWorldLocation` (`/Game/BluePrints/Camera/BP_CameraSpline.Spline` (`self.SplineRef`)) (`SceneComponent.K2_GetComponentLocation` (`Character.CapsuleComponent` _returnvalue)) "World") (`GameplayStatics.GetWorldDeltaSeconds`) (`self.Speed`)) false false)
  (`KismetSystemLibrary.Delay` (`self.MoveDuration`))
  (switch `int` (`self.HPBoss`)
    (:`1`
      (`self.ChangeState_Event` "NewEnumerator3" :!label _label))
    (:`2`
      (goto _label))
    (:`3`
      (`self.ChangeState_Event` "NewEnumerator1"))))

(event `ResetState_Event`
  ;[1 1 1] AIBehavior
  ;;[1 1 1] Reset State
  (set `self.isPunchingL` false)
  (set `self.isPunchingR` false)
  (set `self.isPunchingDouble` false)
  (set `self.Initated Punch` false)
  (`self.ResetPunch_Event`))

(event `PunchPlayer_Event`
  ;[1 1 1] AIBehavior
  ;;[0.7872 0.4547 1] Punch Player
  (set `self.Initated Punch` true)
  (`/Engine/EditorBlueprintResources/StandardMacros.DoOnce` false :!label _label_2
    (:`Completed`
      (set `self.isPunchingL` true)
      (`KismetSystemLibrary.Delay` (`self.GracePeriod`))
      (if (`self.Initated Punch`)
        (set `self.isPunchingL` false)
        (set `self.isPunchingR` true)
        (`KismetSystemLibrary.Delay` (`self.GracePeriod`))
        (if (`self.Initated Punch`)
          (set `self.isPunchingR` false)
          (set `self.isPunchingDouble` true)
          (`KismetSystemLibrary.Delay` (`self.VulnerablePeriod`))
          (if (`self.Initated Punch`)
            (set `self.isPunchingDouble` false)
            (`self.ChangeState_Event` "NewEnumerator0")
            (goto _label_2 :!via `Reset`)))))))

(event `ResetPunch_Event`
  ;[1 1 1] AIBehavior
  ;;[0.7872 0.4547 1] Punch Player
  (goto _label_2 :!via `Reset`))

(event `ShootPlayer_Event`
  (bind _int_shoot (`self.Int Shoot`))
  (bind _returnvalue_location (`KismetMathLibrary.BreakTransform` (`SceneComponent.K2_GetComponentToWorld` (`self.Cannon`))))
  (bind (_returnvalue_roll _returnvalue_pitch _returnvalue_yaw) (`KismetMathLibrary.BreakRotator` (`SceneComponent.K2_GetComponentRotation` (`self.CapsuleComponent`))))
  ;[1 1 1] AIBehavior
  ;;[0.5493 1 0.577] Shoot Wind
  (`SceneComponent.K2_SetWorldLocation` (`self.Cannon`) (`KismetMathLibrary.VInterpTo` (`SceneComponent.K2_GetComponentLocation` (`self.Cannon`)) (`SceneComponent.K2_GetComponentLocation` (`self.FinalCannonPos`)) (`GameplayStatics.GetWorldDeltaSeconds`) 5.0) false false)
  (bind _returnvalue (`GameplayStatics.GetActorOfClass` "/Game/BluePrints/Control/BP_ThirdPersonCharacter.BP_ThirdPersonCharacter_C"))
  (bind (_returnvalue_roll_2 _returnvalue_pitch_2 _returnvalue_yaw_2) (`KismetMathLibrary.BreakRotator` (`KismetMathLibrary.FindLookAtRotation` (`SceneComponent.K2_GetComponentLocation` (`self.CapsuleComponent`)) (`SceneComponent.K2_GetComponentLocation` (`Character.CapsuleComponent` _returnvalue)))))
  (bind (_returnvalue_roll_3 _returnvalue_pitch_3 _returnvalue_yaw_3) (`KismetMathLibrary.BreakRotator` (`KismetMathLibrary.RInterpTo` (`SceneComponent.K2_GetComponentRotation` (`self.CapsuleComponent`)) (`KismetMathLibrary.MakeRotator` 0.0 0.0 (`KismetMathLibrary.ClampAngle` _returnvalue_yaw_2 90.0 270.0)) (`GameplayStatics.GetWorldDeltaSeconds`) 3.0)))
  (`SceneComponent.K2_SetWorldRotation` (`self.CapsuleComponent`) (`KismetMathLibrary.MakeRotator` 0.0 0.0 _returnvalue_yaw_3) false false)
  (`KismetSystemLibrary.Delay` 1.0)
  (`/Engine/EditorBlueprintResources/StandardMacros.DoOnce` false :!label _label_3
    (:`Completed`
      (set `self.isWindShooting` true :!label _label_4)
      (bind _returnvalue_2 (`|SpawnActorFromClass` "/Game/BluePrints/Obstacles/Enemies/BP_WhispyProjectile.BP_WhispyProjectile_C" (`KismetMathLibrary.MakeTransform` _returnvalue_location (`KismetMathLibrary.MakeRotator` 0.0 0.0 _returnvalue_yaw)) "Undefined" "MultiplyWithRoot" null null))
      (`/Game/BluePrints/Obstacles/Enemies/BP_WhispyProjectile.PlaySound` _returnvalue_2)
      (`AudioComponent.Play` (`self.Audio_WindCanon`) 0.0)
      (`/Engine/EditorBlueprintResources/StandardMacros.IncrementInt` _int_shoot
        (:`  `
          (if (>= _int_shoot 5)
            (`KismetSystemLibrary.Delay` (`self.EndShoot`))
            (`SceneComponent.K2_SetWorldLocation` (`self.Cannon`) (`KismetMathLibrary.VInterpTo` (`SceneComponent.K2_GetComponentLocation` (`self.Cannon`)) (`SceneComponent.K2_GetComponentLocation` (`self.Centre`)) (`GameplayStatics.GetWorldDeltaSeconds`) 5.0) false false)
            (`KismetSystemLibrary.Delay` 1.0)
            (`self.ChangeState_Event` "NewEnumerator1")
            (set `self.Int Shoot` 0)
            (set `self.isWindShooting` false)
            (`|ExecutionSequence`
              (:`then_0`
                (goto _label_3 :!via `Reset`)))
            (else
              (`KismetSystemLibrary.Delay` (`self.ShootPeriod`))
              (goto _label_4))))))))

(event `self.HurtBox.OnComponentBeginOverlap`
  (params (OverlappedComponent :type "PrimitiveComponent Object Reference") (OtherActor :type "Actor Object Reference") (OtherComp :type "PrimitiveComponent Object Reference") (OtherBodyIndex :type Integer) (bFromSweep :type Boolean) (SweepResult :type "HitResult Structure (by ref)"))
  ;[1 1 1] AIBehavior
  ;;[1 0.4671 0.5069] OnBossHit
  (`KismetSystemLibrary.DelayUntilNextTick`)
  (bind _asbp_explosion_enemy (cast `/Game/BluePrints/Interactable/BP_Explosion_Enemy` OtherActor))
  (switch `/Game/BluePrints/Interactable/Enum_Explosion` (`/Game/BluePrints/Interactable/BP_Explosion_Enemy.ExplosionType` _asbp_explosion_enemy)
    (:`NewEnumerator1`
      (`KismetSystemLibrary.PrintString` "BOSS EXPLOSIONNNNNNNNNN" true true (struct :`R` 1.0 :`B` 0.069411 :`A` 1.0) 10.0)
      (`self.ResetState_Event`)
      (`self.ChangeState_Event` "NewEnumerator4"))))

(event `HurtBoss_Event`
  ;[1 1 1] AIBehavior
  ;;[1 0.4671 0.5069] Hurt Event
  (`/Engine/EditorBlueprintResources/StandardMacros.DoOnce` false :!label _label_5
    (:`Completed`
      (`/Engine/EditorBlueprintResources/StandardMacros.DecrementInt` (`self.HPBoss`)
        (:`  `
          (bind _returnvalue (`GameplayStatics.GetActorOfClass` "/Game/BluePrints/Control/BP_ThirdPersonCharacter.BP_ThirdPersonCharacter_C"))
          (set `self.isHit` true)
          (`/Game/BluePrints/Control/BP_ThirdPersonCharacter.ThrowPlayer_Event` _returnvalue (* (`SceneComponent.GetForwardVector` (`self.CapsuleComponent`)) (1500.0 0.0 500.0)) false true)
          (`self.HitFeedback_Event`)
          (`KismetSystemLibrary.Delay` 2.0)
          (if (<= (`self.HPBoss`) 0)
            ;;[1 0.2081 0.9292] Create Death Explosion (not polished)
            (for _array_element (`self.ArrayMeshes`)
              (`NiagaraFunctionLibrary.SpawnSystemAtLocation` (`self.NS_death`) (`SceneComponent.K2_GetComponentLocation` _array_element))
              (`KismetSystemLibrary.Delay` 1.0)
              (`self.K2_DestroyActor`))
            (else
              (set `self.isHit` false)
              (`self.ChangeState_Event` "NewEnumerator0")
              (goto _label_5 :!via `Reset`))))))))

(event `self.BossYzark_Hand_R.OnComponentBeginOverlap`
  (params (OverlappedComponent :type "PrimitiveComponent Object Reference") (OtherActor :type "Actor Object Reference") (OtherComp :type "PrimitiveComponent Object Reference") (OtherBodyIndex :type Integer) (bFromSweep :type Boolean) (SweepResult :type "HitResult Structure (by ref)"))
  (bind _capsulecomponent (`self.CapsuleComponent`))
  ;[1 1 1] AIBehavior
  ;;[1 0 0] Punches hit player
  (bind _asbp_third_person_character (cast `/Game/BluePrints/Control/BP_ThirdPersonCharacter` OtherActor :!label _label_6))
  (`/Engine/EditorBlueprintResources/StandardMacros.DoOnce` false :!label _label_7
    (:`Completed`
      (`/Game/BluePrints/Control/BP_ThirdPersonCharacter.StunPlayerFor_Event` _asbp_third_person_character 0.5)
      (bind (_returnvalue_x _returnvalue_y) (`KismetMathLibrary.BreakVector` (`KismetMathLibrary.Normal` (- (`SceneComponent.K2_GetComponentLocation` (`Character.CapsuleComponent` _asbp_third_person_character)) (`SceneComponent.K2_GetComponentLocation` _capsulecomponent)))))
      (`/Game/BluePrints/Control/BP_ThirdPersonCharacter.ThrowPlayer_Event` _asbp_third_person_character (+ (* (`KismetMathLibrary.MakeVector` _returnvalue_x _returnvalue_y) (`self.StrenghtForward`)) (* (`SceneComponent.GetUpVector` _capsulecomponent) (`self.StrenghtUp`))) true true)
      (`KismetSystemLibrary.Delay` (`self.GracePeriod`))
      (`self.ResetHit_Event`))))

(event `HitFeedback_Event`
  (bind _arraymeshes (`self.ArrayMeshes`))
  ;[1 1 1] AIBehavior
  ;;[1 1 1] HitFeedback
  (`PrimitiveComponent.SetMaterial` _arraymeshes 0 "/Game/Art_Graphics/Characters/ENM_Gold/bossYzark/M_bossYzarkWhite.M_bossYzarkWhite")
  (`KismetSystemLibrary.Delay` 0.1)
  (`PrimitiveComponent.SetMaterial` _arraymeshes 0 "/Game/Art_Graphics/Characters/ENM_Gold/bossYzark/MI_bossYzark.MI_bossYzark")
  (`PrimitiveComponent.SetMaterial` (`self.Cannon`) 0 "/Game/Art_Graphics/Props/canon2/M_canon1.M_canon1")
  (`KismetSystemLibrary.Delay` 0.1)
  (`PrimitiveComponent.SetMaterial` _arraymeshes 0 "/Game/Art_Graphics/Props/baril/MI_baril_white.MI_baril_white")
  (`KismetSystemLibrary.Delay` 0.1)
  (`PrimitiveComponent.SetMaterial` _arraymeshes 0 "/Game/Art_Graphics/Characters/ENM_Gold/bossYzark/MI_bossYzark.MI_bossYzark")
  (`PrimitiveComponent.SetMaterial` (`self.Cannon`) 0 "/Game/Art_Graphics/Props/canon2/M_canon1.M_canon1"))

(event `self.BossYzark_Hand_R.OnComponentHit`
  (params (HitComponent :type "PrimitiveComponent Object Reference") (OtherActor :type "Actor Object Reference") (OtherComp :type "PrimitiveComponent Object Reference") (NormalImpulse :type "Vector Structure") (Hit :type "HitResult Structure (by ref)"))
  ;[1 1 1] AIBehavior
  ;;[1 0 0] Punches hit player
  (goto _label_6))

(event `self.BossYzark_Hand_L.OnComponentHit`
  (params (HitComponent :type "PrimitiveComponent Object Reference") (OtherActor :type "Actor Object Reference") (OtherComp :type "PrimitiveComponent Object Reference") (NormalImpulse :type "Vector Structure") (Hit :type "HitResult Structure (by ref)"))
  ;[1 1 1] AIBehavior
  ;;[1 0 0] Punches hit player
  (goto _label_6))

(event `self.BossYzark_Hand_L.OnComponentBeginOverlap`
  (params (OverlappedComponent :type "PrimitiveComponent Object Reference") (OtherActor :type "Actor Object Reference") (OtherComp :type "PrimitiveComponent Object Reference") (OtherBodyIndex :type Integer) (bFromSweep :type Boolean) (SweepResult :type "HitResult Structure (by ref)"))
  (goto _label_6))

(event `ResetHit_Event`
  ;[1 1 1] AIBehavior
  ;;[1 0 0] Punches hit player
  (goto _label_7 :!via `Reset`))

(fn `UserConstructionScript`)