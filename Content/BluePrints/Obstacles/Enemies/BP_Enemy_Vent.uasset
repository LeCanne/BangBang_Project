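; Fan robot enemy that chases the player and pushes them with wind gusts, awarding score when destroyed by an explosion.
; Pawn sensing and radius overlaps gate AI chase and yaw tracking on Tick; a forward capsule trace hit stops it and starts timeline-scaled gusts.
; While the player is inside the wind cylinder, Tick either damps their velocity or adds randomized impulse, clearing the push when the trace misses.
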(event `PlayerLaunch`
  (bind _returnvalue (`self.K2_GetActorLocation` (`ActorComponent.GetOwner` (`self.Ventilo`))))
  ;[1 1 1] Désactiver le player launch si la capsule ne détecte rien
  (bind _outhit (`KismetSystemLibrary.CapsuleTraceSingleForObjects` _returnvalue (+ _returnvalue (* (`KismetMathLibrary.GetForwardVector` (`self.K2_GetActorRotation` (`ActorComponent.GetOwner` (`self.Ventilo`)))) (`self.Vector_Raycast`))) 70.0 140.0 (`self.Object Types`)))
  (if (not (`GameplayStatics.BreakHitResult` _outhit))
    (set `self.IsPlayerLaunch` false)))

(event `Play Sound`
  ;[1 1 1] Discovers player
  (`/Engine/EditorBlueprintResources/StandardMacros.DoOnce` false :!label _label
    (:`Completed`
      (`GameplayStatics.SpawnSoundAtLocation` "/Game/0_Dossiers_perso/Charles/Audio/SFX/Blocking/Robot/SFX_Robot_Mario1.SFX_Robot_Mario1" (`self.K2_GetActorLocation` self) (struct) 1.0 1.0 0.0 null null))))

(event `Reset Sound`
  ;[1 1 1] Discovers player
  (goto _label :!via `Reset`))

(event `self.ReceiveBeginPlay`
  (bind _returnvalue (`GameplayStatics.GetActorOfClass` "/Game/BluePrints/System/SoundManager.SoundManager_C"))
  (set `self.Sound Manager` _returnvalue)
  (`GameplayStatics.GetAllActorsOfClass` "/Game/BluePrints/Obstacles/Enemies/BP_Enemy.BP_Enemy_C")
  (`GameplayStatics.GetAllActorsOfClass` "/Game/BluePrints/Obstacles/Enemies/BP_Enemy_Arroseur.BP_Enemy_Arroseur_C"))

(event `self.PawnSensing.OnSeePawn`
  (params (Pawn :type "Pawn Object Reference"))
  ;[1 0.399 0.399] Détecter le joueur
  (bind _asbp_third_person_character (cast `/Game/BluePrints/Control/BP_ThirdPersonCharacter` Pawn))
  (set `self.IsSeeingPlayer` true))

(event `Follow Player`
  ;[1 0.399 0.399] Détecter le joueur
  (if (`self.IsSeeingPlayer`)
    ;;[1 1 1] Phase Agro sur le joueur
    (`|AIMoveTo` self (0.0 0.0 0.0) (stale `self.PawnSensing.OnSeePawn` _asbp_third_person_character) 10.0
      (:`then`
        (`CharacterMovementComponent.SetMovementMode` (`self.CharacterMovement`) "MOVE_Walking" 0)
        (`SceneComponent.SetVisibility` (`self.TextRender`) true false)))))

(event `self.ReceiveTick`
  (params (DeltaSeconds :type "Float (single-precision)"))
  (bind _as_bp_third_person_character (`self.As BP Third Person Character`))
  (bind _capsulecomponent (`self.CapsuleComponent`))
  (bind _returnvalue (`KismetMathLibrary.GetForwardVector` (`self.K2_GetActorRotation`)))
  (bind _charactermovement (`Character.CharacterMovement` _as_bp_third_person_character))
  (bind _returnvalue_2 (`self.K2_GetActorLocation` (`ActorComponent.GetOwner` (`self.Ventilo`))))
  (bind (_returnvalue_roll _returnvalue_pitch _returnvalue_yaw) (`KismetMathLibrary.BreakRotator` (`KismetMathLibrary.RInterpTo` (`SceneComponent.K2_GetComponentRotation` _capsulecomponent) (`KismetMathLibrary.FindLookAtRotation` (`SceneComponent.K2_GetComponentLocation` _capsulecomponent) (`SceneComponent.K2_GetComponentLocation` (`Actor.RootComponent` (`self.BP_ThirdPersonCharacter`)))) DeltaSeconds 2.0)))
  ;[1 0.399 0.399] Détecter le joueur
  (`|ExecutionSequence`
    (:`then_0`
      (if (not (`self.IsBlow`))
        (if (and (`self.TurnToPlayer`) (`self.IsMove`))
          (`self.Follow Player`)
          (`SceneComponent.K2_SetWorldRotation` (`self.CapsuleComponent`) (`KismetMathLibrary.MakeRotator` 0.0 0.0 _returnvalue_yaw) false false))
        ;;[1 1 1] Système du souffle
        (`self.Play Sound`)
        (bind _outhit (`KismetSystemLibrary.CapsuleTraceSingleForObjects` :`Start` _returnvalue_2 :`End` (+ _returnvalue_2 (* (`KismetMathLibrary.GetForwardVector` (`self.K2_GetActorRotation` (`ActorComponent.GetOwner` (`self.Ventilo`)))) (`self.Vector_Raycast`))) :`Radius` 70.0 :`HalfHeight` 140.0 :`ObjectTypes` (`self.Object Types`) :`TraceColor` (struct :`R` 0.642435 :`B` 1.0 :`A` 1.0) :`DrawTime` 2.0))
        (if (`GameplayStatics.BreakHitResult` _outhit)
          (set `self.IsBlow` true)
          (set `self.TurnToPlayer` false)
          (`self.Attack`))))
    (:`then_1`
      ;[1 1 1] Wind Push Player
      (if (`self.IsPlayerLaunch`)
        (if (and (!= (`self.GetActorForwardVector` _as_bp_third_person_character) _returnvalue :`ErrorTolerance` 1.0) (`/Game/BluePrints/Control/BP_ThirdPersonCharacter.Moving` _as_bp_third_person_character))
          (set `MovementComponent.Velocity` (/ (`MovementComponent.Velocity` _charactermovement) 1.2) _charactermovement)
          (else
            (`CharacterMovementComponent.AddImpulse` _charactermovement (* _returnvalue (* (* (`self.WindStrength`) (`KismetMathLibrary.RandomFloatInRange` 0.8 1.4)) 1.0)) true)))))
    (:`then_2`
      (`self.PlayerLaunch`))))

(event `Death`
  (bind _bp_thirdpersoncharacter (`self.BP_ThirdPersonCharacter`))
  ;[0 1 0.5204] Mort (en teste)
  (`/Engine/EditorBlueprintResources/StandardMacros.DoOnce` false
    (:`Completed`
      (`|SpawnActorFromClass` "/Game/BluePrints/Interactable/BP_Explosion_Enemy.BP_Explosion_Enemy_C" (`self.GetTransform`) "Undefined" "MultiplyWithRoot" null null)
      (`GameplayStatics.PlaySound2D` "/Game/0_Dossiers_perso/Charles/Audio/Sound_Cue/SFX/A_Robot_Death_Cue.A_Robot_Death_Cue" 1.0 1.0 0.0 null null)
      (set `/Game/BluePrints/Control/BP_ThirdPersonCharacter.ScorePoint` (+ (`/Game/BluePrints/Control/BP_ThirdPersonCharacter.ScorePoint` _bp_thirdpersoncharacter) (`self.ScoreGiven`)) _bp_thirdpersoncharacter)
      (bind _asbp_spawn_text (cast `/Game/BluePrints/System/BP_SpawnText` (`ChildActorComponent.ChildActor` (`self.ScoreSpawn`))))
      (`SceneComponent.K2_SetWorldRotation` :`self` (`/Game/BluePrints/System/BP_SpawnText.DefaultSceneRoot` _asbp_spawn_text))
      (`/Game/BluePrints/System/BP_SpawnText.SpawnText` _asbp_spawn_text (`self.ScoreGiven`))
      (`self.K2_DestroyActor`))))

(event `self.ReceiveActorEndOverlap`
  (params (OtherActor :type "Actor Object Reference"))
  ;[0 0.6955 1] Détection via la collision
  ;;[1 1 1] Sortie de la collision
  (cast `/Game/BluePrints/Control/BP_ThirdPersonCharacter` OtherActor)
  (`|AIMoveTo` self (0.0 0.0 0.0) self
    (:`then`
      (`|ExecutionSequence`
        (:`then_0`
          (set `self.IsSeeingPlayer` false)
          (`SceneComponent.SetVisibility` (`self.TextRender`) false false)
          ;[1 0.399 0.399] Détecter le joueur
          ;;[1 1 1] Phase Agro sur le joueur
          (`self.Reset Sound`))
        (:`then_1`
          (set `self.IsPlayerLaunch` false :!label _label_2))))))

(event `self.Cylinder.OnComponentEndOverlap`
  (params (OverlappedComponent :type "PrimitiveComponent Object Reference") (OtherActor :type "Actor Object Reference") (OtherComp :type "PrimitiveComponent Object Reference") (OtherBodyIndex :type Integer))
  ;[0 0.6955 1] Détection via la collision
  ;;[1 1 1] Sortie de la collision
  (cast `/Game/BluePrints/Control/BP_ThirdPersonCharacter` OtherActor)
  (goto _label_2))

(event `Attack`
  (bind _endpoint (`self.EndPoint`))
  (bind _scene (`self.Scene`))
  ;[0 1 0.5204] Attaque
  (`CharacterMovementComponent.SetMovementMode` (`self.CharacterMovement`) "MOVE_None" 0)
  (bind (_direction _wind) (`Timeline|BlowOn` :!via `PlayFromStart`)
    (:`Update`
      (`SceneComponent.SetRelativeScale3D` _scene (`KismetMathLibrary.MakeVector` 0.5 _wind 0.5)))
    (:`Finished`
      (`KismetSystemLibrary.Delay` 2.0)
      (bind (_direction_2 _wind_2) (`Timeline|BlowOff` :!via `PlayFromStart`)
        (:`Update`
          (`SceneComponent.SetRelativeScale3D` _endpoint (`KismetMathLibrary.MakeVector` 1.0 _wind_2 1.0)))
        (:`Finished`
          (`SceneComponent.SetRelativeScale3D` _endpoint (1.0 1.0 1.0))
          (set `self.IsBlow` false)
          (set `self.TurnToPlayer` true)
          (`SceneComponent.SetRelativeScale3D` _scene (0.0 0.0 0.0)))))))

(event `self.IgnoreRadius.OnComponentEndOverlap`
  (params (OverlappedComponent :type "PrimitiveComponent Object Reference") (OtherActor :type "Actor Object Reference") (OtherComp :type "PrimitiveComponent Object Reference") (OtherBodyIndex :type Integer))
  ;[0 0.6955 1] Détection via la collision
  ;;[1 1 1] Sortie de la collision
  (cast `/Game/BluePrints/Control/BP_ThirdPersonCharacter` OtherActor)
  (set `self.TurnToPlayer` false))

(event `self.CapsuleComponent.OnComponentBeginOverlap`
  (params (OverlappedComponent :type "PrimitiveComponent Object Reference") (OtherActor :type "Actor Object Reference") (OtherComp :type "PrimitiveComponent Object Reference") (OtherBodyIndex :type Integer) (bFromSweep :type Boolean) (SweepResult :type "HitResult Structure (by ref)"))
  (bind _bp_thirdpersoncharacter (`self.BP_ThirdPersonCharacter`))
  ;[0 0.6955 1] Détection via la collision
  ;;[1 1 1] Entre de la collision
  (if (`ActorComponent.ComponentHasTag` OtherComp "EXPLOSION")
    (`|ExecutionSequence`
      (:`then_0`
        (`self.Death`))
      (:`then_1`
        ;[1 1 1] Donne 1 d'explosion
        (if (`/Game/BluePrints/Control/BP_ThirdPersonCharacter.IsExplode` _bp_thirdpersoncharacter)
          (set `/Game/BluePrints/Control/BP_ThirdPersonCharacter.IsExplode` false _bp_thirdpersoncharacter)
          (bind _result (`/Engine/EditorBlueprintResources/StandardMacros.DecrementInt` (`/Game/BluePrints/Control/BP_ThirdPersonCharacter.JumpCount` _bp_thirdpersoncharacter))
            (:`  `
              (set `/Game/BluePrints/Control/BP_ThirdPersonCharacter.JumpCount` _result _bp_thirdpersoncharacter))))))))

(event `self.AcceptanceRadius.OnComponentBeginOverlap`
  (params (OverlappedComponent :type "PrimitiveComponent Object Reference") (OtherActor :type "Actor Object Reference") (OtherComp :type "PrimitiveComponent Object Reference") (OtherBodyIndex :type Integer) (bFromSweep :type Boolean) (SweepResult :type "HitResult Structure (by ref)"))
  ;[0 0.6955 1] Détection via la collision
  ;;[1 1 1] Entre de la collision
  (bind _asbp_third_person_character (cast `/Game/BluePrints/Control/BP_ThirdPersonCharacter` OtherActor))
  (set `self.BP_ThirdPersonCharacter` _asbp_third_person_character)
  (set `self.TurnToPlayer` true)
  (`SceneComponent.ResetRelativeTransform` (`self.Body`)))

(event `self.Cylinder.OnComponentBeginOverlap`
  (params (OverlappedComponent :type "PrimitiveComponent Object Reference") (OtherActor :type "Actor Object Reference") (OtherComp :type "PrimitiveComponent Object Reference") (OtherBodyIndex :type Integer) (bFromSweep :type Boolean) (SweepResult :type "HitResult Structure (by ref)"))
  ;[0 0.6955 1] Détection via la collision
  ;;[1 1 1] Entre de la collision
  (bind _asbp_third_person_character (cast `/Game/BluePrints/Control/BP_ThirdPersonCharacter` OtherActor))
  (set `self.As BP Third Person Character` _asbp_third_person_character)
  (`KismetSystemLibrary.Delay` 0.1)
  (set `self.IsPlayerLaunch` true))

(fn `UserConstructionScript`)