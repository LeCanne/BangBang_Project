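; Shower enemy obstacle that travels along a spline path while periodically releasing falling water projectiles.
; Each tick advances the enemy's distance along the spline by speed and delta time, wrapping on closed loops or ping-ponging on open paths via the Backtrack flag.
; A delta-time accumulator, also updated on tick, spawns BP_WaterProjectileFall at the shoot origin whenever the shoot interval elapses.
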(event `self.ReceiveTick`
  (params (DeltaSeconds :type "Float (single-precision)"))
  (`|ExecutionSequence`
    (:`then_0`
      (`self.MoveEnemyOnSpline_Event`))
    (:`then_1`
      (`self.ShootWater_Event`))))

(event `MoveEnemyOnSpline_Event`
  (bind _returnvalue (* (`GameplayStatics.GetWorldDeltaSeconds`) (* (`self.Speed`) 100.0)))
  ;[0.01589 0.58 0] Move On Spline
  (if (`SplineComponent.IsClosedLoop` (`self.SplinePath`))
    (bind _output_get (set `self.Distance` (+ (`self.Distance`) _returnvalue) :!label _label))
    (`SceneComponent.K2_SetWorldLocation` (`self.Enemy`) (`SplineComponent.GetLocationAtDistanceAlongSpline` (`self.SplinePath`) _output_get "World") false false)
    (if (>= (`self.Distance`) (`SplineComponent.GetSplineLength` (`self.SplinePath`)))
      (if (`SplineComponent.IsClosedLoop` (`self.SplinePath`))
        (set `self.Distance` 0.0)
        (else
          (set `self.Backtrack` false))))
    (elif (`self.Backtrack`)
      (goto _label)
      (else
        (bind _output_get_2 (set `self.Distance` (+ (* _returnvalue -1.0) (`self.Distance`))))
        (`SceneComponent.K2_SetWorldLocation` (`self.Enemy`) (`SplineComponent.GetLocationAtDistanceAlongSpline` (`self.SplinePath`) _output_get_2 "World") false false)
        (if (<= (`self.Distance`) 0.0)
          (set `self.Backtrack` true))))))

(event `ShootWater_Event`
  ;[0.08 0.2816 1] ShootWater
  (set `self.CurrentInterval` (+ (`GameplayStatics.GetWorldDeltaSeconds`) (`self.CurrentInterval`)))
  (if (>= (`self.CurrentInterval`) (`self.ShootIntervals`))
    (`|SpawnActorFromClass` "/Game/BluePrints/Obstacles/Enemies/BP_WaterProjectileFall.BP_WaterProjectileFall_C" (`KismetMathLibrary.MakeTransform` (`SceneComponent.K2_GetComponentLocation` (`self.ShootOrigin`))) "Undefined" "MultiplyWithRoot" null null)
    (set `self.CurrentInterval` 0.0)))

(fn `UserConstructionScript`)