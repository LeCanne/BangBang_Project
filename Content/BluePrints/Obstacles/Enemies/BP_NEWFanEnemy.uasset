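; Fan enemy that rises when the player enters its detection radius, turns toward them and blows wind, turning slower while blowing.
; Timelines scale the wind space on and off; overlapping the wind cylinder applies a distance-scaled push, weaker when airborne and switched by running state.
; The facing-angle check is disconnected, so attacks start once aggroed.
; Explosion-tagged hits kill it, awarding score and spawning an explosion and collectible.
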(event `self.ReceiveBeginPlay`
  ;[0 0.64 0.07452] BehaviorLoop
  (set `self.VectorOriginScale` (`SceneComponent.RelativeScale3D` (`self.WindSpace`))))

(event `self.ReceiveTick`
  (params (DeltaSeconds :type "Float (single-precision)"))
  ;[0 0.64 0.07452] BehaviorLoop
  (if (`self.PlayerDetected`)
    (`|ExecutionSequence`
      (:`then_0`
        (`self.DoAggroAnim_Event` true))
      (:`then_1`
        (if (`self.AggroEnabled`)
          (if (`self.Blowing`)
            (set `self.RotationSpeed` 70.0)
            (else
              (set `self.RotationSpeed` 140.0)))
          (`self.RotateToPlayer_Event`)))
      (:`then_2`
        (if (`self.AggroEnabled`)
          (`self.CompareRotations_Event`)))
      (:`then_3`
        (if (and (`self.AttackPossible`) (`self.AggroEnabled`))
          (`self.AttackPlayer_Event`)))
      (:`then_4`
        (if (`self.PlayerInWind`)
          (`self.PushPlayer_Event`))))
    (else
      (`self.DoAggroAnim_Event` false))))

(event `self.DetectionRadius.OnComponentBeginOverlap`
  (params (OverlappedComponent :type "PrimitiveComponent Object Reference") (OtherActor :type "Actor Object Reference") (OtherComp :type "PrimitiveComponent Object Reference") (OtherBodyIndex :type Integer) (bFromSweep :type Boolean) (SweepResult :type "HitResult Structure (by ref)"))
  ;[1 0.0411 0] Detect Player
  (bind _asbp_third_person_character (cast `/Game/BluePrints/Control/BP_ThirdPersonCharacter` OtherActor))
  (set `self.BP_CharacterReference` _asbp_third_person_character)
  (set `self.PlayerDetected` true))

(event `self.WindCylinder.OnComponentBeginOverlap`
  (params (OverlappedComponent :type "PrimitiveComponent Object Reference") (OtherActor :type "Actor Object Reference") (OtherComp :type "PrimitiveComponent Object Reference") (OtherBodyIndex :type Integer) (bFromSweep :type Boolean) (SweepResult :type "HitResult Structure (by ref)"))
  ;[0.7 0 0] CheckIfPlayerInWind
  (cast `/Game/BluePrints/Control/BP_ThirdPersonCharacter` OtherActor)
  (set `self.PlayerInWind` true))

(event `self.DetectionRadius.OnComponentEndOverlap`
  (params (OverlappedComponent :type "PrimitiveComponent Object Reference") (OtherActor :type "Actor Object Reference") (OtherComp :type "PrimitiveComponent Object Reference") (OtherBodyIndex :type Integer))
  ;[1 0.0411 0] Detect Player
  (cast `/Game/BluePrints/Control/BP_ThirdPersonCharacter` OtherActor)
  (set `self.PlayerDetected` false)
  (set `self.AggroEnabled` false)
  (`self.SoundAggroReset_Event`)
  (if (`self.Blowing`)
    (`self.StopBlowing_Event`)))

(event `self.WindCylinder.OnComponentEndOverlap`
  (params (OverlappedComponent :type "PrimitiveComponent Object Reference") (OtherActor :type "Actor Object Reference") (OtherComp :type "PrimitiveComponent Object Reference") (OtherBodyIndex :type Integer))
  ;[0.7 0 0] CheckIfPlayerInWind
  (cast `/Game/BluePrints/Control/BP_ThirdPersonCharacter` OtherActor)
  (set `self.PlayerInWind` false))

(event `DeathEvent`
  (bind (_returnvalue_x _returnvalue_y _returnvalue_z) (`KismetMathLibrary.BreakVector` (`SceneComponent.K2_GetComponentLocation` (`self.Base`))))
  ;[0 0 0] DestroyEnemy
  (`/Engine/EditorBlueprintResources/StandardMacros.DoOnce` false
    (:`Completed`
      (`GameplayStatics.PlaySound2D` "/Game/0_Dossiers_perso/Charles/Audio/Sound_Cue/SFX/Ennemy/A_Robot_Death_Cue.A_Robot_Death_Cue" 1.0 1.0 0.0 null null)
      (`|SpawnActorFromClass` "/Game/BluePrints/Interactable/BP_Explosion_Enemy.BP_Explosion_Enemy_C" (`self.GetTransform`) "Undefined" "MultiplyWithRoot" null null)
      (bind _asbp_give_score (cast `/Game/BluePrints/System/BP_GiveScore` (`ChildActorComponent.ChildActor` (`self.ScoreSpawn`))))
      (`/Game/BluePrints/System/BP_GiveScore.Give Score` _asbp_give_score 500.0 (`self.BP_CharacterReference`) true)
      (`self.SetActorTickEnabled` false)
      (`SceneComponent.SetHiddenInGame` (`self.Base`) true true)
      (`self.SetActorEnableCollision` false)
      (bind _returnvalue (`|SpawnActorFromClass` "/Game/BluePrints/Interactable/Collectable/BP_Child_CollectablePhysics.BP_Child_CollectablePhysics_C" (`KismetMathLibrary.MakeTransform` (`KismetMathLibrary.MakeVector` _returnvalue_x _returnvalue_y (+ _returnvalue_z 100.0))) "AlwaysSpawn" "MultiplyWithRoot" self null))
      (`/Game/BluePrints/Interactable/Collectable/BP_Child_CollectablePhysics.ImpulseUp_Event` _returnvalue 2000.0 (0.0 0.0 0.0)))))

(event `self.EnemyHitbox.OnComponentBeginOverlap`
  (params (OverlappedComponent :type "PrimitiveComponent Object Reference") (OtherActor :type "Actor Object Reference") (OtherComp :type "PrimitiveComponent Object Reference") (OtherBodyIndex :type Integer) (bFromSweep :type Boolean) (SweepResult :type "HitResult Structure (by ref)"))
  ;[0.87 0 0] CollisionWithExplosion
  (if (`ActorComponent.ComponentHasTag` OtherComp "EXPLOSION")
    (`self.DeathEvent`)))

(event `DoAggroAnim_Event`
  (params (Enable :type Boolean))
  (bind _returnvalue (* (`GameplayStatics.GetWorldDeltaSeconds`) (`self.Speed Transition`)))
  (bind _relativelocation (`SceneComponent.RelativeLocation` (`self.EnemyHitbox`)))
  ;[0.08 0.3951 1] TransitionAggroed
  (if Enable
    (`SceneComponent.K2_SetRelativeLocation` (`self.EnemyHitbox`) (`KismetMathLibrary.VLerp` _relativelocation (0.0 0.0 85.0) _returnvalue) false false)
    (`KismetSystemLibrary.Delay` 0.5)
    (set `self.AggroEnabled` true)
    (`/Engine/EditorBlueprintResources/StandardMacros.DoOnce` false :!label _label
      (:`Completed`
        (`GameplayStatics.SpawnSoundAtLocation` "/Game/0_Dossiers_perso/Charles/Audio/Sound_Cue/SFX/Ennemy/A_Robot_Detect_Cue.A_Robot_Detect_Cue" (`self.K2_GetActorLocation` self) (struct) 1.0 1.0 0.0 null null)))
    (else
      (`SceneComponent.K2_SetRelativeLocation` (`self.EnemyHitbox`) (`KismetMathLibrary.VLerp` _relativelocation (0.0 0.0 -70.0) _returnvalue) false false))))

(event `SoundAggroReset_Event`
  ;[0.08 0.3951 1] TransitionAggroed
  (goto _label :!via `Reset`))

(event `RotateToPlayer_Event`
  (bind (_returnvalue_roll _returnvalue_pitch _returnvalue_yaw) (`KismetMathLibrary.BreakRotator` (`KismetMathLibrary.FindLookAtRotation` (`SceneComponent.K2_GetComponentLocation` (`self.Enemy`)) (`SceneComponent.K2_GetComponentLocation` (`Character.CapsuleComponent` (`self.BP_CharacterReference`))))))
  ;[0.92 0 0.1701] RotateToPlayer
  (set `self.DesiredRotation` (`KismetMathLibrary.MakeRotator` 0.0 0.0 (- _returnvalue_yaw 90.0)))
  (`SceneComponent.K2_SetWorldRotation` (`self.Enemy`) (`KismetMathLibrary.RInterpTo_Constant` (`SceneComponent.K2_GetComponentRotation` (`self.Enemy`)) (`self.DesiredRotation`) (`GameplayStatics.GetWorldDeltaSeconds`) (`self.RotationSpeed`)) false false))

(event `CompareRotations_Event`
  ;[0.3395 0 0.42] CheckIfPlayerInAttackRange
  (set `self.AttackPossible` true))

(event `AttackPlayer_Event`
  (bind (_vectororiginscale_x _vectororiginscale_y _vectororiginscale_z) (`KismetMathLibrary.BreakVector` (`self.VectorOriginScale`)))
  ;[0 0.1048 0.9] Blow Wind
  (`/Engine/EditorBlueprintResources/StandardMacros.DoOnce` false :!label _label_2
    (:`Completed`
      (set `self.Blowing` true)
      (bind (_direction _blowvalue) (`Timeline|BlowOn` :!via `PlayFromStart` :!label _label_3)
        (:`Update`
          (`SceneComponent.SetRelativeScale3D` (`self.WindSpace`) (`KismetMathLibrary.MakeVector` _vectororiginscale_x (* _blowvalue 3.36) _vectororiginscale_z)))))))

(event `ResetAttackParameter_Event`
  ;[0 0.1048 0.9] Blow Wind
  (goto _label_2 :!via `Reset`))

(event `StopBlowing_Event`
  ;[0 0.1048 0.9] Blow Wind
  (`|ExecutionSequence`
    (:`then_0`
      (goto _label_3 :!via `Stop`))
    (:`then_1`
      (bind (_direction _sizewind) (`Timeline|BlowOff` :!via `PlayFromStart`)
        (:`Update`
          (`SceneComponent.SetRelativeScale3D` (`self.EndWindSpace`) (`KismetMathLibrary.MakeVector` 1.0 _sizewind 1.0))
          (set `self.Blowing` false))
        (:`Finished`
          (`KismetSystemLibrary.Delay` (`self.FallOffDuration`))
          (set `self.AttackPossible` false)
          (`SceneComponent.SetRelativeScale3D` (`self.WindSpace`) (0.0 0.0 0.0))
          (`SceneComponent.SetRelativeScale3D` (`self.EndWindSpace`) (1.0 1.0 1.0))
          (`self.ResetAttackParameter_Event`))))))

(event `PushPlayer_Event`
  (bind _bp_characterreference (`self.BP_CharacterReference`))
  (bind _charactermovement (`Character.CharacterMovement` (`self.BP_CharacterReference`)))
  (bind _returnvalue (* (`SceneComponent.GetRightVector` (`self.Enemy`)) (/ (/ (`self.WindPower`) (`GameplayStatics.GetWorldDeltaSeconds`)) (* (`KismetMathLibrary.Vector_Distance` (`SceneComponent.K2_GetComponentLocation` (`self.Base`)) (`SceneComponent.K2_GetComponentLocation` (`Character.CapsuleComponent` (`self.BP_CharacterReference`)))) 0.01))))
  ;[0 0.8539 0.91] WindPhysics
  (if (and (`/Game/BluePrints/Control/BP_ThirdPersonCharacter.Moving` _bp_characterreference) (`/Game/BluePrints/Control/BP_ThirdPersonCharacter.Running` _bp_characterreference))
    (set `self.WindPower` (`self.MinWind`))
    (else
      (set `self.WindPower` (`self.MaxWind`))))
  (if (`NavMovementComponent.IsMovingOnGround` (`Character.CharacterMovement` (`self.BP_CharacterReference`)))
    (`CharacterMovementComponent.AddForce` _charactermovement _returnvalue)
    (else
      (`CharacterMovementComponent.AddForce` _charactermovement (* _returnvalue 0.05)))))

(fn `UserConstructionScript`)