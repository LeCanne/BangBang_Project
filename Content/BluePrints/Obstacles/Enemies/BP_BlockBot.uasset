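; BP_BlockBot is an enemy that chases the player on sight and kills them on touching its attack radius.
; PawnSensing starts a Tick-driven AIMoveTo with a one-shot alert; separate overlaps enable slow turning or end the chase.
; Player explosions destroy it, awarding score and adjusting the player's jump count, but hits on its Cube shield grant brief invincibility.
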(event `self.PawnSensing.OnSeePawn`
  (params (Pawn :type "Pawn Object Reference"))
  ;[1 0.399 0.399] Détecter le joueur
  (bind _asbp_third_person_character (cast `/Game/BluePrints/Control/BP_ThirdPersonCharacter` Pawn))
  (set `self.IsSeeingPlayer` true))

(event `Follow Player`
  ;[1 0.399 0.399] Détecter le joueur
  (if (`self.IsSeeingPlayer`)
    ;;[1 1 1] Phase Agro sur le joueur
    (`|AIMoveTo` self (0.0 0.0 0.0) (stale `self.PawnSensing.OnSeePawn` _asbp_third_person_character) 10.0
      (:`then`
        (`CharacterMovementComponent.SetMovementMode` (`self.CharacterMovement`) "MOVE_Walking" 0)
        (`SceneComponent.SetVisibility` (`self.TextRender`) true false)
        (`/Engine/EditorBlueprintResources/StandardMacros.DoOnce` false :!label _label
          (:`Completed`
            (`GameplayStatics.SpawnSoundAtLocation` "/Game/0_Dossiers_perso/Charles/Audio/SFX/Blocking/SFX_RobotVoice_Detection.SFX_RobotVoice_Detection" (`self.K2_GetActorLocation` self) (struct) 1.0 1.0 0.0 null null)))))))

(event `self.ReceiveTick`
  (params (DeltaSeconds :type "Float (single-precision)"))
  (bind _capsulecomponent (`self.CapsuleComponent`))
  (bind (_returnvalue_roll _returnvalue_pitch _returnvalue_yaw) (`KismetMathLibrary.BreakRotator` (`KismetMathLibrary.RInterpTo` (`SceneComponent.K2_GetComponentRotation` _capsulecomponent) (`KismetMathLibrary.FindLookAtRotation` (`SceneComponent.K2_GetComponentLocation` _capsulecomponent) (`SceneComponent.K2_GetComponentLocation` (`Actor.RootComponent` (`self.BP_ThirdPersonCharacter`)))) DeltaSeconds 0.5)))
  ;[1 0.399 0.399] Détecter le joueur
  (`self.Follow Player`)
  (if (`self.TurnToPlayer`)
    (`SceneComponent.K2_SetWorldRotation` (`self.CapsuleComponent`) (`KismetMathLibrary.MakeRotator` 0.0 0.0 _returnvalue_yaw) false false)))

(event `Death`
  (bind _bp_thirdpersoncharacter (`self.BP_ThirdPersonCharacter`))
  ;[0 1 0.5204] Mort (en teste)
  (`self.K2_DestroyActor`)
  (`|SpawnActorFromClass` "/Game/BluePrints/Interactable/BP_Explosion_Enemy.BP_Explosion_Enemy_C" (`self.GetTransform`) "Undefined" "MultiplyWithRoot" null null)
  (set `/Game/BluePrints/Control/BP_ThirdPersonCharacter.ScorePoint` (+ (`/Game/BluePrints/Control/BP_ThirdPersonCharacter.ScorePoint` _bp_thirdpersoncharacter) 200) _bp_thirdpersoncharacter))

(event `self.ReceiveActorEndOverlap`
  (params (OtherActor :type "Actor Object Reference"))
  ;[0 0.6955 1] Détection via la collision
  ;;[1 1 1] Sortie de la collision
  (cast `/Game/BluePrints/Control/BP_ThirdPersonCharacter` OtherActor)
  (`|AIMoveTo` self (0.0 0.0 0.0) self
    (:`then`
      (set `self.IsSeeingPlayer` false)
      (`SceneComponent.SetVisibility` (`self.TextRender`) false false)
      (goto _label :!via `Reset`))))

(event `self.AttackRadius.OnComponentBeginOverlap`
  (params (OverlappedComponent :type "PrimitiveComponent Object Reference") (OtherActor :type "Actor Object Reference") (OtherComp :type "PrimitiveComponent Object Reference") (OtherBodyIndex :type Integer) (bFromSweep :type Boolean) (SweepResult :type "HitResult Structure (by ref)"))
  ;[0 1 0.5204] Attaque
  (bind _asbp_third_person_character (cast `/Game/BluePrints/Control/BP_ThirdPersonCharacter` OtherActor))
  (`/Game/BluePrints/Control/BP_ThirdPersonCharacter.Die_Event` _asbp_third_person_character))

(event `self.IgnoreRadius.OnComponentEndOverlap`
  (params (OverlappedComponent :type "PrimitiveComponent Object Reference") (OtherActor :type "Actor Object Reference") (OtherComp :type "PrimitiveComponent Object Reference") (OtherBodyIndex :type Integer))
  ;[0 0.6955 1] Détection via la collision
  ;;[1 1 1] Entre de la collision
  (cast `/Game/BluePrints/Control/BP_ThirdPersonCharacter` OtherActor)
  (set `self.TurnToPlayer` false))

(event `self.CapsuleComponent.OnComponentBeginOverlap`
  (params (OverlappedComponent :type "PrimitiveComponent Object Reference") (OtherActor :type "Actor Object Reference") (OtherComp :type "PrimitiveComponent Object Reference") (OtherBodyIndex :type Integer) (bFromSweep :type Boolean) (SweepResult :type "HitResult Structure (by ref)"))
  (bind _bp_thirdpersoncharacter (`self.BP_ThirdPersonCharacter`))
  ;[0 0.6955 1] Détection via la collision
  ;;[1 1 1] Entre de la collision
  (cast `/Game/BluePrints/Interactable/BP_Explosion_Enemy` OtherActor)
  (if (not (`self.Invincible`))
    (`|ExecutionSequence`
      (:`then_0`
        (`self.Death`))
      (:`then_1`
        ;[1 1 1] Donne 1 d'explosion
        (if (`/Game/BluePrints/Control/BP_ThirdPersonCharacter.IsExplode` _bp_thirdpersoncharacter)
          (set `/Game/BluePrints/Control/BP_ThirdPersonCharacter.IsExplode` false _bp_thirdpersoncharacter)
          (bind _result (`/Engine/EditorBlueprintResources/StandardMacros.DecrementInt` (`/Game/BluePrints/Control/BP_ThirdPersonCharacter.JumpCount` _bp_thirdpersoncharacter))
            (:`  `
              (set `/Game/BluePrints/Control/BP_ThirdPersonCharacter.JumpCount` _result _bp_thirdpersoncharacter))))))))

(event `self.Cube.OnComponentBeginOverlap`
  (params (OverlappedComponent :type "PrimitiveComponent Object Reference") (OtherActor :type "Actor Object Reference") (OtherComp :type "PrimitiveComponent Object Reference") (OtherBodyIndex :type Integer) (bFromSweep :type Boolean) (SweepResult :type "HitResult Structure (by ref)"))
  ;[1 0.03125 0.03125] Defense
  (cast `/Game/BluePrints/Interactable/BP_Explosion_Enemy` OtherActor)
  (`KismetSystemLibrary.PrintString` "NANOMACHINES SON")
  (set `self.Invincible` true)
  (`KismetSystemLibrary.Delay` 0.5)
  (set `self.Invincible` false))

(event `self.AcceptanceRadius.OnComponentBeginOverlap`
  (params (OverlappedComponent :type "PrimitiveComponent Object Reference") (OtherActor :type "Actor Object Reference") (OtherComp :type "PrimitiveComponent Object Reference") (OtherBodyIndex :type Integer) (bFromSweep :type Boolean) (SweepResult :type "HitResult Structure (by ref)"))
  ;[0 0.6955 1] Détection via la collision
  ;;[1 1 1] Entre de la collision
  (bind _asbp_third_person_character (cast `/Game/BluePrints/Control/BP_ThirdPersonCharacter` OtherActor))
  (set `self.BP_ThirdPersonCharacter` _asbp_third_person_character)
  (set `self.TurnToPlayer` true))

(fn `UserConstructionScript`)