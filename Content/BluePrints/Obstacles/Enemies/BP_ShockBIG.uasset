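; BP_ShockBIG is an expanding electric shockwave hazard that stuns and throws the player.
; Every tick its static mesh grows horizontally at SpeedExpand, keeping its height.
; On overlap, the player character is stunned and thrown outward and upward from the shock's origin, respecting invincibility.
; A one-shot sequence plays the electric sound, activates the NSLighting effect after Lifetime, then destroys the actor after a further delay.
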(event `self.ReceiveTick`
  (params (DeltaSeconds :type "Float (single-precision)"))
  (bind _staticmesh (`self.StaticMesh`))
  (bind (_returnvalue_x _returnvalue_y _returnvalue_z) (`KismetMathLibrary.BreakVector` (`SceneComponent.K2_GetComponentScale` _staticmesh)))
  (bind (_returnvalue_x_2 _returnvalue_y_2) (`KismetMathLibrary.BreakVector` (`SceneComponent.K2_GetComponentScale` (`self.StaticMesh`))))
  (bind _returnvalue (* (`GameplayStatics.GetWorldDeltaSeconds`) (`self.SpeedExpand`)))
  (`SceneComponent.SetWorldScale3D` _staticmesh (`KismetMathLibrary.MakeVector` (+ _returnvalue _returnvalue_x_2) (+ _returnvalue_y_2 _returnvalue) _returnvalue_z))
  (`/Engine/EditorBlueprintResources/StandardMacros.DoOnce` false
    (:`Completed`
      (`GameplayStatics.PlaySoundAtLocation` "/Game/0_Dossiers_perso/Charles/Audio/Sound_Cue/SFX/A_Electric_Cue.A_Electric_Cue" (`self.K2_GetActorLocation`) (struct) 1.0 1.0 0.0 null null null null)
      (`KismetSystemLibrary.Delay` (`self.Lifetime`))
      (`ActorComponent.Activate` (`self.NS_lighting`) false)
      (`KismetSystemLibrary.Delay` 5.0)
      (`self.K2_DestroyActor`))))

(event `self.StaticMesh.OnComponentBeginOverlap`
  (params (OverlappedComponent :type "PrimitiveComponent Object Reference") (OtherActor :type "Actor Object Reference") (OtherComp :type "PrimitiveComponent Object Reference") (OtherBodyIndex :type Integer) (bFromSweep :type Boolean) (SweepResult :type "HitResult Structure (by ref)"))
  (bind _defaultsceneroot (`self.DefaultSceneRoot`))
  (bind _asbp_third_person_character (cast `/Game/BluePrints/Control/BP_ThirdPersonCharacter` OtherActor))
  (`/Game/BluePrints/Control/BP_ThirdPersonCharacter.StunPlayerFor_Event` _asbp_third_person_character 1.0)
  (bind (_returnvalue_x _returnvalue_y) (`KismetMathLibrary.BreakVector` (`KismetMathLibrary.Normal` (- (`SceneComponent.K2_GetComponentLocation` (`Character.CapsuleComponent` _asbp_third_person_character)) (`SceneComponent.K2_GetComponentLocation` _defaultsceneroot)))))
  (`/Game/BluePrints/Control/BP_ThirdPersonCharacter.ThrowPlayer_Event` _asbp_third_person_character (+ (* (`KismetMathLibrary.MakeVector` _returnvalue_x _returnvalue_y) (`self.StrenghtForward`)) (* (`SceneComponent.GetUpVector` _defaultsceneroot) (`self.StrenghtUp`))) true true true))

(fn `UserConstructionScript`)