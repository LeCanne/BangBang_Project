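; Sprayer ("Arroseur") enemy obstacle whose cone ping-pongs along a spline via the Pattern timeline.
; Each tick, a line trace along the actor's up axis drives PointScale's Z scale, while Cylinder overlaps change the player's state.
; An explosion touching the cone destroys the enemy, spawns another explosion, awards score and can decrement the player's JumpCount.
; The water-drop spawning loop is left unconnected.
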(event `self.ReceiveTick`
  (params (DeltaSeconds :type "Float (single-precision)"))
  (bind _returnvalue (`self.K2_GetActorLocation` (`ActorComponent.GetOwner` (`self.Cone`))))
  ;[1 1 1] Teste de raycast
  (bind _outhit (`KismetSystemLibrary.LineTraceSingleForObjects` _returnvalue (+ _returnvalue (* (`KismetMathLibrary.GetUpVector` (`self.K2_GetActorRotation` (`ActorComponent.GetOwner` (`self.Cone`)))) (`self.Vector_Raycast`))) (`self.Object Types`)))
  (`SceneComponent.SetRelativeScale3D` (`self.PointScale`) (`KismetMathLibrary.MakeVector` 1.0 1.0 (`KismetMathLibrary.Abs` (- (`KismetMathLibrary.NormalizeToRange` (`KismetMathLibrary.VSize` (- (`self.GetActorScale3D` (`ActorComponent.GetOwner` (`self.PointScale`))) (`.ImpactPoint` (`GameplayStatics.BreakHitResult` _outhit)))) 0.0 1000.0) 1.0)))))

(event `Death`
  (bind _bp_third_person (`self.BP Third Person`))
  ;[0 1 0.5204] Mort (en teste)
  (`/Engine/EditorBlueprintResources/StandardMacros.DoOnce` false
    (:`Completed`
      (`|SpawnActorFromClass` "/Game/BluePrints/Interactable/BP_Explosion_Enemy.BP_Explosion_Enemy_C" (`SceneComponent.K2_GetComponentToWorld` (`self.Cone`)) "Undefined" "MultiplyWithRoot" null null)
      (`self.K2_DestroyActor`)
      (set `/Game/BluePrints/Control/BP_ThirdPersonCharacter.ScorePoint` (+ (`/Game/BluePrints/Control/BP_ThirdPersonCharacter.ScorePoint` _bp_third_person) 20) _bp_third_person))))

(event `self.ReceiveBeginPlay`
  (bind _backtrack (`self.Backtrack`))
  (`|ExecutionSequence`
    (:`then_1`
      ;[0 1 0.322] Patterne de l'ennemie
      (bind (_direction _newtrack_0) (`Timeline|Pattern` :!label _label)
        (:`Update`
          (`SceneComponent.K2_SetWorldLocation` (`self.Cone`) (`SplineComponent.GetLocationAtDistanceAlongSpline` (`self.Spline`) (* (`SplineComponent.GetSplineLength` (`self.Spline`)) _newtrack_0) "World") false false))
        (:`Finished`
          (set `self.Backtrack` (not _backtrack))
          (if _backtrack
            (goto _label :!via `Reverse`)
            (else
              (goto _label :!via `PlayFromStart`))))))
    (:`then_2`
      (bind _returnvalue (`GameplayStatics.GetActorOfClass` "/Game/BluePrints/Control/BP_ThirdPersonCharacter.BP_ThirdPersonCharacter_C"))
      (set `self.BP Third Person` _returnvalue))))

(event `self.ReceiveActorEndOverlap`
  (params (OtherActor :type "Actor Object Reference"))
  ;[0 0.6939 1] Détection via la collision
  ;;[1 1 1] Sortie de la collision
)

(event `self.Cone.OnComponentBeginOverlap`
  (params (OverlappedComponent :type "PrimitiveComponent Object Reference") (OtherActor :type "Actor Object Reference") (OtherComp :type "PrimitiveComponent Object Reference") (OtherBodyIndex :type Integer) (bFromSweep :type Boolean) (SweepResult :type "HitResult Structure (by ref)"))
  (bind _bp_third_person (`self.BP Third Person`))
  ;[0 0.6939 1] Détection via la collision
  ;;[1 1 1] Entre de la collision
  (cast `/Game/BluePrints/Interactable/BP_Explosion_Enemy` OtherActor)
  (`|ExecutionSequence`
    (:`then_0`
      (`self.Death`))
    (:`then_1`
      ;[1 1 1] Donne 1 d'explosion
      (if (`/Game/BluePrints/Control/BP_ThirdPersonCharacter.IsExplode` _bp_third_person)
        (set `/Game/BluePrints/Control/BP_ThirdPersonCharacter.IsExplode` false _bp_third_person)
        (bind _result (`/Engine/EditorBlueprintResources/StandardMacros.DecrementInt` (`/Game/BluePrints/Control/BP_ThirdPersonCharacter.JumpCount` _bp_third_person))
          (:`  `
            (set `/Game/BluePrints/Control/BP_ThirdPersonCharacter.JumpCount` _result _bp_third_person)))))))

(event `self.Cylinder.OnComponentBeginOverlap`
  (params (OverlappedComponent :type "PrimitiveComponent Object Reference") (OtherActor :type "Actor Object Reference") (OtherComp :type "PrimitiveComponent Object Reference") (OtherBodyIndex :type Integer) (bFromSweep :type Boolean) (SweepResult :type "HitResult Structure (by ref)"))
  ;[0 0.6939 1] Détection via la collision
  ;;[1 1 1] Entre de la collision
  (bind _asbp_third_person_character (cast `/Game/BluePrints/Control/BP_ThirdPersonCharacter` OtherActor))
  (set `/Game/BluePrints/Control/BP_ThirdPersonCharacter.PlayerCurrentState` "NewEnumerator1" _asbp_third_person_character)
  (`/Game/BluePrints/Control/BP_ThirdPersonCharacter.TriggerState_Event` _asbp_third_person_character))

(fn `UserConstructionScript`)