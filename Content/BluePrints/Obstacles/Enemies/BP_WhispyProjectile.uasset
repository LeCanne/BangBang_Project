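; Wind projectile of the Whispy enemy that throws the player on contact.
; Each tick it grows with its age under random per-axis jitter, then destroys itself after its lifetime, which is also fed to the Niagara wind effect.
; The first player overlap launches the character forward and upward and disables collision.
; A separate event plays the shot sound, and a stun call is left unconnected.
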(event `self.ReceiveBeginPlay`)

(event `PlaySound`
  (`AudioComponent.Play` (`self.Audio_WindShoot`) 0.0))

(event `self.ReceiveTick`
  (params (DeltaSeconds :type "Float (single-precision)"))
  (bind _returnvalue (* (`KismetMathLibrary.RandomFloatInRange` 0.8 1.3) (`self.currentlife`)))
  (bind _output_get (set `self.currentlife` (+ DeltaSeconds (`self.currentlife`))))
  (`SceneComponent.SetRelativeScale3D` (`self.Scene`) (`KismetMathLibrary.MakeVector` _returnvalue _returnvalue _returnvalue))
  (if (> _output_get (`self.lifetime`))
    (`self.K2_DestroyActor`)))

(event `self.WindCollision.OnComponentBeginOverlap`
  (params (OverlappedComponent :type "PrimitiveComponent Object Reference") (OtherActor :type "Actor Object Reference") (OtherComp :type "PrimitiveComponent Object Reference") (OtherBodyIndex :type Integer) (bFromSweep :type Boolean) (SweepResult :type "HitResult Structure (by ref)"))
  (bind _scene (`self.Scene`))
  (bind _asbp_third_person_character (cast `/Game/BluePrints/Control/BP_ThirdPersonCharacter` OtherActor))
  (`/Game/BluePrints/Control/BP_ThirdPersonCharacter.ThrowPlayer_Event` _asbp_third_person_character (+ (* (`SceneComponent.GetForwardVector` _scene) (`self.WindStrength`)) (* (`SceneComponent.GetUpVector` _scene) (0.0 0.0 500.0))) false true)
  (`PrimitiveComponent.SetCollisionEnabled` (`self.WindCollision`) "NoCollision"))

(fn `UserConstructionScript`
  (`NiagaraComponent.SetVariableFloat` (`self.NS_wind`) "Lifetime" (`self.lifetime`)))