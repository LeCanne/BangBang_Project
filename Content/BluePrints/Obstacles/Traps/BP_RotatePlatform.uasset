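; Trap platform obstacle that swings back and forth on its roll axis, starting at BeginPlay.
; The RotatePlatform timeline drives the world roll of RotatePoint with its negated track value.
; When the timeline finishes, a DurationDelay pause loops back to the IsRotate toggle, which alternates between playing and reversing it.
; A DoOnce guards the start, which also prints a debug string.
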(event `self.ReceiveBeginPlay`
  (`/Engine/EditorBlueprintResources/StandardMacros.DoOnce` false
    (:`Completed`
      (`KismetSystemLibrary.PrintString` "Hello")
      (if (`self.IsRotate`) :!label _label
        (set `self.IsRotate` false)
        (bind (_direction _newtrack_0) (`Timeline|RotatePlatform` :!label _label_2)
          (:`Update`
            (`SceneComponent.K2_SetWorldRotation` (`self.RotatePoint`) (`KismetMathLibrary.MakeRotator` (* _newtrack_0 -1.0)) false false))
          (:`Finished`
            (`KismetSystemLibrary.Delay` (`self.Duration_Delay`))
            (goto _label)))
        (else
          (set `self.IsRotate` true)
          (goto _label_2 :!via `Reverse`))))))

(fn `UserConstructionScript`)