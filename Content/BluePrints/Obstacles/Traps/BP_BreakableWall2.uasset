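; Breakable wall obstacle that shatters when its mesh is overlapped by a BP_Explosion_Enemy.
; On break it hides the mesh, disables collision, fires the shatter and pouf effects, then destroys itself after a short delay.
; It also spawns a new BP_Explosion_Enemy at its own transform, which can chain into nearby breakables.
; The construction script feeds sprite size, color, scale, velocity and spawn count variables into the NSShatter effect.
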(event `self.Mesh.OnComponentBeginOverlap`
  (params (OverlappedComponent :type "PrimitiveComponent Object Reference") (OtherActor :type "Actor Object Reference") (OtherComp :type "PrimitiveComponent Object Reference") (OtherBodyIndex :type Integer) (bFromSweep :type Boolean) (SweepResult :type "HitResult Structure (by ref)"))
  (cast `/Game/BluePrints/Interactable/BP_Explosion_Enemy` OtherActor)
  (`SceneComponent.SetVisibility` (`self.Mesh`) false false)
  (`self.SetActorEnableCollision` false)
  (`ActorComponent.Activate` (`|MakeArray` (`self.NS_shatter`) (`self.NS_pouf`) :!type "ActorComponent Object Reference") false)
  (`|SpawnActorFromClass` "/Game/BluePrints/Interactable/BP_Explosion_Enemy.BP_Explosion_Enemy_C" (`self.GetTransform`) "Undefined" "MultiplyWithRoot" null null)
  (`KismetSystemLibrary.Delay` 3.0)
  (`self.K2_DestroyActor`))

(fn `UserConstructionScript`
  ;[1 0.9411 0] Vector2
  (`NiagaraComponent.SetVariableVec2` (`self.NS_shatter`) "SpriteMax" (`self.Size Max`))
  (`NiagaraComponent.SetVariableVec2` (`self.NS_shatter`) "SpriteMin" (`self.Size Min`))
  ;[0 0.08976 1] Color
  (`NiagaraComponent.SetVariableLinearColor` (`self.NS_shatter`) "ColorMax" (`self.Color Max`))
  (`NiagaraComponent.SetVariableLinearColor` (`self.NS_shatter`) "ColorMin" (`self.Color Min`))
  ;[0.08409 1 0] Float
  (`NiagaraComponent.SetVariableFloat` (`self.NS_shatter`) "Scale" (`self.Scale`))
  (`NiagaraComponent.SetVariableFloat` (`self.NS_shatter`) "VelocityMax" (`self.Velocity Max`))
  (`NiagaraComponent.SetVariableFloat` (`self.NS_shatter`) "VelocityMin" (`self.VelocityMin`))
  ;[0.1029 1 0.8094] Int
  (`NiagaraComponent.SetVariableInt` (`self.NS_shatter`) "SpawnCount" (`self.Spawn Count`)))