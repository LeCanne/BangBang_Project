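; Crane platform obstacle whose beam swings back and forth in yaw around the rotation it has at BeginPlay.
; Each tick advances a target offset by Speed, with StartReversed setting the direction and flipping whenever the offset's magnitude exceeds EndRotation.
; The beam's world yaw eases toward base plus offset with FInterpTo, smoothing the turnarounds, while pitch and roll are held at zero.
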(event `self.ReceiveBeginPlay`
  (bind (_returnvalue_roll _returnvalue_pitch _returnvalue_yaw) (`KismetMathLibrary.BreakRotator` (`SceneComponent.K2_GetComponentRotation` (`self.SM_beam`))))
  (set `self.BaseRotation` _returnvalue_yaw))

(event `self.ReceiveTick`
  (params (DeltaSeconds :type "Float (single-precision)"))
  (bind (_returnvalue_roll _returnvalue_pitch _returnvalue_yaw) (`KismetMathLibrary.BreakRotator` (`SceneComponent.K2_GetComponentRotation` (`self.SM_beam`))))
  (bind _returnvalue (* DeltaSeconds (`self.Speed`)))
  (`|ExecutionSequence`
    (:`then_0`
      (if (> (`KismetMathLibrary.Abs` (`self.CurrentRotationZ`)) (`KismetMathLibrary.Abs` (`self.EndRotation`)))
        (set `self.StartReversed` (not (`self.StartReversed`)))))
    (:`then_1`
      (if (`self.StartReversed`)
        (set `self.CurrentRotationZ` (+ (* _returnvalue -1.0) (`self.CurrentRotationZ`)))
        (else
          (set `self.CurrentRotationZ` (+ _returnvalue (`self.CurrentRotationZ`))))))
    (:`then_2`
      (`SceneComponent.K2_SetWorldRotation` (`self.SM_beam`) (`KismetMathLibrary.MakeRotator` 0.0 0.0 (`KismetMathLibrary.FInterpTo` _returnvalue_yaw (+ (`self.CurrentRotationZ`) (`self.BaseRotation`)) (`GameplayStatics.GetWorldDeltaSeconds`) 1.0)) false false))))

(fn `UserConstructionScript`)