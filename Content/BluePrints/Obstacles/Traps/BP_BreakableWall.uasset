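; BP_BreakableWall is a trap obstacle wall that disappears when an explosion touches it.
; When a component tagged EXPLOSION overlaps the Cube, the wall hides the mesh and disables actor collision rather than destroying itself.
; If Reactivates is set, it restores visibility and collision after a short delay.
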(event `self.Cube.OnComponentBeginOverlap`
  (params (OverlappedComponent :type "PrimitiveComponent Object Reference") (OtherActor :type "Actor Object Reference") (OtherComp :type "PrimitiveComponent Object Reference") (OtherBodyIndex :type Integer) (bFromSweep :type Boolean) (SweepResult :type "HitResult Structure (by ref)"))
  (bind _cube (`self.Cube`))
  (if (`ActorComponent.ComponentHasTag` OtherComp "EXPLOSION")
    (`SceneComponent.SetVisibility` _cube false false)
    (`self.SetActorEnableCollision` false)
    (if (`self.Reactivates`)
      (`KismetSystemLibrary.Delay` 2.0)
      (`SceneComponent.SetVisibility` _cube true false)
      (`self.SetActorEnableCollision` true))))

(fn `UserConstructionScript`)