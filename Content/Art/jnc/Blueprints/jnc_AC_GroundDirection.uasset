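; Actor component that estimates the ground's slope direction along its owner's forward or right axis.
; Each tick it sphere-traces downward at samples spread along that axis and normalizes the summed deltas between hit points.
; A fixed-alpha, frame-rate-dependent lerp smooths the result, easing toward the actor's axis when hits don't exceed a validity threshold.
; Optional debug drawing shows the hit points plus raw and smoothed directions.
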(event `self.ReceiveTick`
  (params (DeltaSeconds :type "Float (single-precision)"))
  (bind (_grounddirection _groundpoints) (`self.SampleGround`))
  (set `self.groundDirection` _grounddirection)
  (set `self.groundPoints` _groundpoints)
  (`self.ComputeSmoothGroundDirection`)
  (if (`self.debugDraw`)
    (`self.DrawDebug`)))

(fn `ComputeSmoothGroundDirection`
  (set `self.smoothGroundDirection` (`KismetMathLibrary.VLerp` (`self.smoothGroundDirection`) (`KismetMathLibrary.SelectVector` (`self.groundDirection`) (`self.GetActorDirection`) (> (`KismetArrayLibrary.Array_Length` (`self.groundPoints`)) (`self.sampleValidityThreshold`))) 0.15)))

(fn `DrawDebug`
  (bind _returnvalue (`Actor.K2_GetActorLocation` (`self.GetOwner`)))
  (for _array_element (`self.groundPoints`)
    (`KismetSystemLibrary.DrawDebugPoint` _array_element 10.0 (`self.debugColor`)))
  (`KismetSystemLibrary.DrawDebugArrow` _returnvalue (+ _returnvalue (* (`self.groundDirection`) 30.0)) 10.0 (`self.debugColor`))
  (`KismetSystemLibrary.DrawDebugArrow` _returnvalue (+ _returnvalue (* (`self.smoothGroundDirection`) 60.0)) 10.0 (`self.debugColor`)))

(fn `GetActorDirection`
  (returns (ReturnValue :type "Vector Structure"))
  (return (`KismetMathLibrary.SelectVector` (`Actor.GetActorForwardVector` (`self.GetOwner`)) (`Actor.GetActorRightVector` (`self.GetOwner`)) (`self.useForward`))))

(fn `SampleGround`
  (returns (groundDirection :type "Vector Structure") (groundPoints :type "Array of Vector Structure"))
  (locals (max :type Integer) (dir :type "Vector Structure" :default (0.0 0.0 0.0)) (loc :type "Vector Structure" :default (0.0 0.0 0.0)) (up :type "Vector Structure" :default (0.0 0.0 0.0)) (points :type "Array of Vector Structure") (cumulGroundDir :type "Vector Structure"))
  (bind _returnvalue (- (`self.sampleCount`) 1))
  (set `local.dir` (`self.GetActorDirection`))
  (set `local.loc` (`Actor.K2_GetActorLocation` (`self.GetOwner`)))
  (set `local.up` (`KismetMathLibrary.MakeVector` 0.0 0.0 1.0))
  (set `local.max` _returnvalue)
  (for _index (range (+ _returnvalue 1))
    (bind _returnvalue_2 (+ (`local.loc`) (* (`local.dir`) (* (- (/ (`KismetMathLibrary.Conv_IntToDouble` _index) (`local.max`)) 0.5) (`self.sampleRange`)))))
    (bind (_outhit _returnvalue_3) (`KismetSystemLibrary.SphereTraceSingle` (+ _returnvalue_2 (* (`local.up`) (`self.sampleZStartOffset`))) (+ _returnvalue_2 (* (`local.up`) (`self.sampleZEndOffset`))) 10.0 "TraceTypeQuery1" false (`|MakeArray` (`self.GetOwner`))))
    (if _returnvalue_3
      (`KismetArrayLibrary.Array_Add` (`local.points`) (`.ImpactPoint` (`GameplayStatics.BreakHitResult` _outhit)))))
  (for _index_2 (range (+ (- (`KismetArrayLibrary.Array_Length` (`local.points`)) 2) 1))
    (set `local.cumulGroundDir` (+ (`local.cumulGroundDir`) (- (`|GetArrayItem` (`local.points`) (+ _index_2 1)) (`|GetArrayItem` (`local.points`) _index_2)))))
  (return (`KismetMathLibrary.Normal` (`local.cumulGroundDir`)) (`local.points`)))