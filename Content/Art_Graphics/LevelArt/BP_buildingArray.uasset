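; BP_buildingArray is a level-art actor that builds a building from repeated wall meshes in its construction script.
; It assigns the Base mesh to the Top component, then loops over Count to add Wall mesh components offset vertically using Spacing.
; Each wall ignores the Camera collision channel and gets a dynamic material instance for wall color and a Windows-driven V offset parameter.
; The event graph holds no active logic.
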(fn `UserConstructionScript`
  (bind _wallmeshes (`self.WallMeshes`))
  (`StaticMeshComponent.SetStaticMesh` (`self.Top`) (`self.Base`))
  (for _index (range (+ (`self.Count`) 1))
    (bind _returnvalue (`AddComponent|NODE_AddStaticMeshComponent-2` :`RelativeTransform` (`KismetMathLibrary.MakeTransform` (`KismetMathLibrary.MakeVector` 0.0 0.0 (* (/ _index (`self.Count`)) (* (`self.Count`) (`self.Spacing`)))))))
    (bind _output_get (set `self.WallMeshes` _returnvalue))
    (`StaticMeshComponent.SetStaticMesh` _output_get (`self.Wall`))
    (`PrimitiveComponent.SetCollisionResponseToChannel` _wallmeshes "ECC_Camera" "ECR_Ignore")
    (bind _returnvalue_2 (`PrimitiveComponent.CreateDynamicMaterialInstance` _wallmeshes 0 null "None"))
    (`MaterialInstanceDynamic.SetVectorParameterValue` _returnvalue_2 "Color_wall" (`self.WallColor`))
    (`MaterialInstanceDynamic.SetScalarParameterValue` _returnvalue_2 "GREEN_offsetV" (* (`self.Windows`) 0.25))))