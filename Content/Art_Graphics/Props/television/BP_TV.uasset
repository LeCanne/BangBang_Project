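; BP_TV is a television prop that floats and wobbles, with a spinning fan and a configurable screen image.
; The construction script puts the Image texture on a dynamic screen material and makes its components ignore the Camera channel.
; A restarting timeline adds sine-based X/Y and curve-driven Z offsets to the root.
; Tick yaws the fan by DeltaSeconds plus a constant, so spin speed depends on frame rate.
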(event `self.ReceiveBeginPlay`
  (`|ExecutionSequence`
    (:`then_0`
      (bind (_direction _tvfly) (`Timeline|Timeline_tvFly` :!label _label)
        (:`Update`
          (bind _returnvalue (* _tvfly 50.0))
          (`SceneComponent.K2_AddLocalOffset` (`self.DefaultSceneRoot`) (`KismetMathLibrary.MakeVector` (`KismetMathLibrary.Sin` _returnvalue) (`KismetMathLibrary.Sin` _returnvalue) _tvfly) false false))
        (:`Finished`
          (goto _label :!via `PlayFromStart`))))))

(event `self.ReceiveTick`
  (params (DeltaSeconds :type "Float (single-precision)"))
  (`SceneComponent.K2_AddLocalRotation` (`self.fan`) (`KismetMathLibrary.MakeRotator` 0.0 0.0 (+ DeltaSeconds 20.0)) false false))

(fn `UserConstructionScript`
  (bind _screen (`self.screen`))
  (bind _returnvalue (`PrimitiveComponent.CreateDynamicMaterialInstance` _screen 0 null "None"))
  (`PrimitiveComponent.SetMaterial` _screen 0 _returnvalue)
  (`MaterialInstanceDynamic.SetTextureParameterValue` _returnvalue "Image" (`self.Image`))
  (`PrimitiveComponent.SetCollisionResponseToChannel` (`|MakeArray` (`self.SM_tv43`) (`self.fan`) (`self.screen`) null :!type "PrimitiveComponent Object Reference") "ECC_Camera" "ECR_Ignore")
  (`PrimitiveComponent.SetCollisionResponseToChannel` (`self.Box`) "ECC_Camera" "ECR_Ignore"))