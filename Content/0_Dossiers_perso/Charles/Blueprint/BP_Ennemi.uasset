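; BP_Ennemi is an enemy Blueprint that starts an AI move when its PawnSensing component sees a pawn.
; OnSeePawn sets IsSeeingPlayer and calls FollowPlayer, which runs AIMoveTo while that flag is true; nothing clears the flag.
; Overlap events fetch the third-person character, but only end overlap does more, printing a debug message.
; A debug sphere draw and a "Player In" print are left unconnected.
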(event `self.ReceiveActorBeginOverlap`
  (params (OtherActor :type "Actor Object Reference"))
  (`GameplayStatics.GetActorOfClass` "/Game/ThirdPerson/Blueprints/BP_ThirdPersonCharacter.BP_ThirdPersonCharacter_C"))

(event `self.ReceiveActorEndOverlap`
  (params (OtherActor :type "Actor Object Reference"))
  (`GameplayStatics.GetActorOfClass` "/Game/ThirdPerson/Blueprints/BP_ThirdPersonCharacter.BP_ThirdPersonCharacter_C")
  (`KismetSystemLibrary.PrintString` "Player Out" true true (struct :`R` 1.0 :`B` 0.105878 :`A` 1.0)))

(event `self.ReceiveTick`
  (params (DeltaSeconds :type "Float (single-precision)")))

(event `self.PawnSensing.OnSeePawn`
  (params (Pawn :type "Pawn Object Reference"))
  (set `self.IsSeeingPlayer` true)
  (`self.Follow Player`))

(event `Follow Player`
  (if (`self.IsSeeingPlayer`)
    (`|AIMoveTo` null (0.0 0.0 0.0) null)))

(fn `UserConstructionScript`)