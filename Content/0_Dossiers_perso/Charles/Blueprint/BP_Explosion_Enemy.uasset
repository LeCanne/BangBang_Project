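; BP_Explosion_Enemy is a short-lived explosion actor with sound, which by its name is tied to enemies.
; On BeginPlay it plays SC_explosion at the world origin rather than at the actor, and starts a Timeline.
; The Timeline's Scale track drives the world scale of both the Sphere and SphereCollisionExplosion.
; A Delay reached from the first update destroys the actor shortly afterwards, independent of the Timeline finishing.
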(event `self.ReceiveBeginPlay`
  ;[1 1 1] Explosion avec une Timeline + Son
  (`GameplayStatics.PlaySoundAtLocation` "/Game/0_Dossiers_perso/Charles/Audio/SFX/Sound_Cue/SC_explosion.SC_explosion" (0.0 0.0 0.0) (struct) 1.0 1.0 0.0 null null null null)
  (bind (_direction _scale) (`Timeline|Timeline`)
    (:`Update`
      (`|ExecutionSequence`
        (:`then_0`
          (`SceneComponent.SetWorldScale3D` (`self.Sphere`) (`KismetMathLibrary.Conv_DoubleToVector` _scale)))
        (:`then_1`
          (`SceneComponent.SetWorldScale3D` (`self.SphereCollision_Explosion`) (`KismetMathLibrary.Conv_DoubleToVector` _scale))))
      (`KismetSystemLibrary.Delay` 0.4)
      (`self.K2_DestroyActor`))))

(fn `UserConstructionScript`)