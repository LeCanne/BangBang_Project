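; BP_Enemy is an enemy pawn that chases the player once its PawnSensing component sees a pawn.
; Sighting sets IsSeeingPlayer and starts FollowPlayer, a loop that issues AIMoveTo toward player 0, stops movement after a delay, waits, then repeats while the flag holds.
; Any actor overlap ending redirects the move to the enemy itself and clears the flag, which ends the loop at its next check.
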(event `self.PawnSensing.OnSeePawn`
  (params (Pawn :type "Pawn Object Reference"))
  ;[1 0.399 0.399] Détecter le joueur
  (set `self.IsSeeingPlayer` true)
  (`self.Follow Player`))

(event `Follow Player`
  ;[1 0.399 0.399] Détecter le joueur
  (if (`self.IsSeeingPlayer`) :!label _label
    ;;[1 1 1] Phase Agro sur le joueur
    (`|AIMoveTo` self (0.0 0.0 0.0) (`GameplayStatics.GetPlayerCharacter` 0)
      (:`then`
        (`KismetSystemLibrary.Delay` 5.0)
        (`NavMovementComponent.StopActiveMovement` (`self.CharacterMovement`))
        (`KismetSystemLibrary.Delay` 5.0)
        (goto _label)))))

(event `self.ReceiveActorEndOverlap`
  (params (OtherActor :type "Actor Object Reference"))
  ;[1 1 1] Détection via la collision
  ;;[1 1 1] Sortie de la collision
  (`GameplayStatics.GetActorOfClass` "/Game/ThirdPerson/Blueprints/BP_ThirdPersonCharacter.BP_ThirdPersonCharacter_C")
  (`|AIMoveTo` self (0.0 0.0 0.0) self
    (:`then`
      (set `self.IsSeeingPlayer` false))))

(fn `UserConstructionScript`)