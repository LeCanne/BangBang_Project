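; Decal handler that finds the nearest surface around itself and, through SpawnDecal, places a short-lived decal on it.
; BeginPlay builds a Fibonacci sphere of directions, which SampleWorld line-traces to find the closest hit.
; Decal rotation follows a distance-weighted average direction, accumulated only from hits that beat the closest so far.
; With DebugDraw on, Tick resamples every frame and draws traces, hit point and both direction arrows.
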(event `self.ReceiveBeginPlay`
  (bind _points (`self.MakeFibonacciSphere` (`self.Sample Count`)))
  (set `self.Points` _points))

(event `self.ReceiveTick`
  (params (DeltaSeconds :type "Float (single-precision)"))
  (if (`self.debugDraw`)
    (bind (_hashit _hit _hitdirection _averagehitdirection) (`self.SampleWorld` (`self.K2_GetActorLocation`) "TraceTypeQuery1" (`self.Sample Radius`)))
    (set `self.Has Hit` _hashit)
    (set `self.Hit` _hit)
    (set `self.Hit Direction` _hitdirection)
    (set `self.Average Hit Direction` _averagehitdirection)
    (`self.DrawDebug`)))

(fn `DrawDebug`
  (bind (_bblockinghit _binitialoverlap _time _distance _location _impactpoint) (`GameplayStatics.BreakHitResult` (`self.Hit`)))
  (if (`self.Has Hit`)
    (`KismetSystemLibrary.DrawDebugPoint` _impactpoint 20.0 (struct :`G` 0.285352 :`B` 1.0 :`A` 1.0))
    (`KismetSystemLibrary.DrawDebugArrow` _impactpoint (+ _impactpoint (* (`self.Hit Direction`) -200.0)) 0.0 (struct :`G` 0.574882 :`B` 2.0 :`A` 1.0))
    (`KismetSystemLibrary.DrawDebugArrow` _impactpoint (+ _impactpoint (* (`self.Average Hit Direction`) -100.0)) 0.0 (struct :`G` 0.574882 :`B` 2.0 :`A` 1.0))))

(fn `MakeFibonacciSphere`
  (params (count :type Integer :default 32))
  (returns (points :type "Array of Vector Structure"))
  (locals (_points :type "Array of Vector Structure") (phi :type "Float (double-precision)") (theta :type "Float (double-precision)") (inv_phi :type "Float (double-precision)") (z :type "Float (double-precision)") (radius :type "Float (double-precision)" :default 0.0))
  (`KismetArrayLibrary.Array_Resize` (`local._points`) count)
  (bind _output_get (set `local.phi` (/ (+ 1.0 (`KismetMathLibrary.Sqrt` 5.0)) 2.0)))
  (set `local.inv_phi` (/ 1.0 _output_get))
  (for _index (range (`local.count`))
    (set `local.theta` (* 2.0 3.141593 (`local.inv_phi`) _index))
    (set `local.z` (- 1.0 (/ (+ (* 2.0 _index) 1.0) (`local.count`))))
    (set `local.radius` (`KismetMathLibrary.Sqrt` (- 1.0 (* (`local.z`) (`local.z`)))))
    (`KismetArrayLibrary.Array_Set` (`local._points`) _index (`KismetMathLibrary.MakeVector` (* (`local.radius`) (`KismetMathLibrary.Cos` (`local.theta`))) (* (`local.radius`) (`KismetMathLibrary.Sin` (`local.theta`))) (`local.z`))))
  (return (`local._points`)))

(fn `SampleWorld`
  (params (origin :type "Vector Structure") (traceChannel :type "ETraceTypeQuery Enum" :default "TraceTypeQuery1") (radius :type "Float (double-precision)" :default 100.0))
  (returns (hasHit :type Boolean) (hit :type "HitResult Structure") (hitDirection :type "Vector Structure") (averageHitDirection :type "Vector Structure"))
  (locals (tr :type "Transform Structure") (minD :type "Float (double-precision)") (_hasHit :type Boolean) (_hit :type "HitResult Structure") (_hitDirection :type "Vector Structure" :default (0.0 0.0 0.0)) (_cumulativeHitDirection :type "Vector Structure"))
  (bind _origin (`local.origin`))
  (set `local.minD` 100000000.0)
  (set `local.tr` (`self.GetTransform`))
  (for _array_element (`self.Points`)
    (bind _returnvalue (`KismetMathLibrary.TransformDirection` (`local.tr`) _array_element))
    (bind (_outhit _returnvalue_2) (`KismetSystemLibrary.LineTraceSingle` _origin (+ _origin (* _returnvalue (`local.radius`))) (`local.traceChannel`) false (`|MakeArray` (`self.GetOwner`)) (select `bool` (`self.debugDraw`) :`true` "ForOneFrame" :!type "EDrawDebugTrace Enum") true (struct :`G` 0.267153 :`B` 1.0 :`A` 0.2) (struct :`G` 0.266356 :`B` 1.0 :`A` 1.0) 0.0))
    (if _returnvalue_2
      (bind (_bblockinghit _binitialoverlap _time _distance) (`GameplayStatics.BreakHitResult` _outhit))
      (if (< _distance (`local.minD`))
        (set `local.minD` _distance)
        (set `local._hasHit` true)
        (set `local._hit` _outhit)
        (set `local._hitDirection` _returnvalue)
        (set `local._cumulativeHitDirection` (+ (/ _returnvalue (+ _distance 50.0)) (`local._cumulativeHitDirection`))))))
  (return (`local._hasHit`) (`local._hit`) (`local._hitDirection`) (`KismetMathLibrary.Normal` (`local._cumulativeHitDirection`))))

(fn `SpawnDecal`
  (bind (_hashit _hit _hitdirection _averagehitdirection) (`self.SampleWorld` (`self.K2_GetActorLocation`) "TraceTypeQuery1" (`self.Sample Radius`)))
  (if _hashit
    (`GameplayStatics.SpawnDecalAtLocation` (`self.Decal Material`) (150.0 300.0 300.0) (`.ImpactPoint` (`GameplayStatics.BreakHitResult` _hit)) (`KismetMathLibrary.ComposeRotators` (`KismetMathLibrary.MakeRotator` 0.0 -90.0) (`KismetMathLibrary.FindLookAtRotation` (`KismetMathLibrary.Vector_Down`) _averagehitdirection)) 10.0)))

(fn `UserConstructionScript`)