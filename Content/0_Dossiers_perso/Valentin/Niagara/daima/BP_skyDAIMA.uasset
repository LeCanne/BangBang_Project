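; BP_skyDAIMA is a sky sphere actor that sets up a stylable sky material from exposed variables.
; The construction script creates a dynamic instance of M_skyDAIMA on SkySphere and pushes sky, cloud, star brightness and tint values into it.
; ZenithColor and SkyColor both write "Sky Color", so SkyColor overrides the zenith value.
; The event graph is empty, so the Blueprint adds no runtime logic.
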(fn `UserConstructionScript`
  (bind _returnvalue (`PrimitiveComponent.CreateDynamicMaterialInstance` (`self.SkySphere`) 0 "/Game/0_Dossiers_perso/Valentin/Niagara/daima/M_skyDAIMA.M_skyDAIMA" "None"))
  (set `self.MaterialInstance` _returnvalue)
  (`MaterialInstanceDynamic.SetVectorParameterValue` (`self.MaterialInstance`) "Sky Color" (`self.Zenith Color`))
  (`MaterialInstanceDynamic.SetVectorParameterValue` (`self.MaterialInstance`) "Sky Color" (`self.Sky Color`))
  (`MaterialInstanceDynamic.SetVectorParameterValue` (`self.MaterialInstance`) "Cloud Color" (`self.Cloud Color`))
  (`MaterialInstanceDynamic.SetScalarParameterValue` (`self.MaterialInstance`) "Cloud Speed" (`self.Cloud Speed`))
  (`MaterialInstanceDynamic.SetScalarParameterValue` (`self.MaterialInstance`) "Stars brightness" (`self.Stars brightness`))
  (`MaterialInstanceDynamic.SetScalarParameterValue` (`self.MaterialInstance`) "CloudBackground_power" (`self.CloudBackground_power`))
  (`MaterialInstanceDynamic.SetVectorParameterValue` (`self.MaterialInstance`) "Overall Color" (`self.Tint Color`)))