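; BP_Array is a construction-script tool that lays out rows of repeated static meshes from its AssetList map.
; Each entry gets its own Hierarchical Instanced Static Mesh component, placed at the entry's transform with the entry's mesh.
; Instances line up along local X, spaced by the mesh's bounding-box width, with only the X count used.
; The event graph holds no active logic.
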(fn `UserConstructionScript`
  (bind (_currentdata_transform _currentdata_mesh _currentdata_offset _currentdata_count) (break `/Game/0_Dossiers_perso/Valentin/Blueprints/BP_building/F_assetData` (`self.CurrentData`)))
  (bind (_returnvalue_min _returnvalue_max) (break `Box` (`StaticMesh.GetBoundingBox` _currentdata_mesh)))
  (bind _returnvalue_x (`KismetMathLibrary.BreakVector` (- _returnvalue_max _returnvalue_min)))
  (bind _values (`BlueprintMapLibrary.Map_Values` (`self.AssetList`)))
  (for _array_element _values
    (bind _output_get (set `self.CurrentData` _array_element))
    (bind _returnvalue (`AddComponent|NODE_AddHierarchicalInstancedStaticMeshComponent-0` :`RelativeTransform` (break `/Game/0_Dossiers_perso/Valentin/Blueprints/BP_building/F_assetData` _output_get)))
    (bind _output_get_2 (set `self.CurrentHISM` _returnvalue))
    (`StaticMeshComponent.SetStaticMesh` _output_get_2 _currentdata_mesh)
    (for _index (range (`.X` (break `IntVector` _currentdata_count)))
      (`InstancedStaticMeshComponent.AddInstance` (`self.CurrentHISM`) (`KismetMathLibrary.MakeTransform` (`KismetMathLibrary.MakeVector` (* _index _returnvalue_x))) false))))