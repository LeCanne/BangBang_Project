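; Test actor that procedurally builds a rectangular outline of modular static meshes in its Construction Script.
; It divides a size vector by a piece distance to get per-axis counts, then calls CreateLine for four sides at 90-degree yaw steps.
; CreateLine places Mesh01 first, then repeats Mesh02 along the direction at TailleMorceau spacing.
; A looped version offset in Z is left unconnected, and the event graph is empty.
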(fn `CreateLine`
  (params (nbMorceau :type Integer) (yaw :type "Float (single-precision)") (PosDepart :type "Vector Structure") (direction :type "Vector Structure"))
  (locals (nbMorceauDroit :type Integer))
  (set `local.nbMorceauDroit` (- nbMorceau 1))
  (bind _returnvalue (`AddComponent|NODE_AddStaticMeshComponent-2` :`RelativeTransform` (`KismetMathLibrary.MakeTransform` PosDepart (`KismetMathLibrary.MakeRotator` 0.0 0.0 yaw))))
  (`StaticMeshComponent.SetStaticMesh` _returnvalue (`self.mesh01`))
  (for _index (range 1 (+ (`local.nbMorceauDroit`) 1))
    (bind _returnvalue_2 (`AddComponent|NODE_AddStaticMeshComponent-0` :`RelativeTransform` (`KismetMathLibrary.MakeTransform` (+ PosDepart (* (* _index (`self.taille morceau`)) direction)) (`KismetMathLibrary.MakeRotator` 0.0 0.0 yaw))))
    (`StaticMeshComponent.SetStaticMesh` _returnvalue_2 (`self.mesh02`))))

(fn `UserConstructionScript`
  (locals (nbMorceauX :type Integer :default 0) (nbMorceauY :type Integer :default 0) (nbMorceauZ :type Integer :default 0))
  (bind (_vector_x _vector_y _vector_z) (`KismetMathLibrary.BreakVector` (`self.vector`)))
  (bind _distance (`self.distance`))
  (`|ExecutionSequence`
    (:`then_0`
      (set `local.nbMorceauX` (`KismetMathLibrary.FFloor` (/ _vector_x _distance)))
      (set `local.nbMorceauY` (`KismetMathLibrary.FFloor` (/ _vector_y _distance)))
      (set `local.nbMorceauZ` (`KismetMathLibrary.FFloor` (/ _vector_z _distance))))
    (:`then_1`
      (`self.CreateLine` (`local.nbMorceauX`) 0.0 (0.0 0.0 0.0) (1.0 0.0 0.0))
      (`self.CreateLine` (`local.nbMorceauY`) 90.0 (`KismetMathLibrary.MakeVector` (* (`local.nbMorceauX`) (`self.taille morceau`))) (0.0 1.0 0.0))
      (`self.CreateLine` (`local.nbMorceauX`) 180.0 (`KismetMathLibrary.MakeVector` 150.0 (* (`local.nbMorceauY`) (`self.taille morceau`))) (1.0 0.0 0.0))
      (`self.CreateLine` (`local.nbMorceauY`) 270.0 (0.0 150.0 0.0) (0.0 1.0 0.0)))))