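; BP_test is a test Blueprint that procedurally builds a row of static mesh pieces along its local X axis.
; The Construction Script derives the piece count (NbMorceauX) by dividing the X of a Vector variable by a hardcoded length and flooring it.
; It adds one base mesh component, then loops to add the remaining pieces, offset by multiples of TailleMorceau.
; The Event Graph holds only disabled default events.
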(fn `UserConstructionScript`
  (locals (nbMorceauX :type Integer :default 0) (nbMorceauY :type Integer :default 0))
  (bind _vector_x (`KismetMathLibrary.BreakVector` (`self.vector`)))
  (`|ExecutionSequence`
    (:`then_0`
      (set `local.nbMorceauX` (`KismetMathLibrary.FFloor` (/ _vector_x 300.0))))
    (:`then_1`
      (bind _returnvalue (`AddComponent|NODE_AddStaticMeshComponent-2`))
      (`StaticMeshComponent.SetStaticMesh` _returnvalue null)
      (for _index (range 1 (`local.nbMorceauX`))
        (bind _returnvalue_2 (`AddComponent|NODE_AddStaticMeshComponent-0` :`RelativeTransform` (`KismetMathLibrary.MakeTransform` (`KismetMathLibrary.MakeVector` (* _index (`self.taille morceau`))))))
        (`StaticMeshComponent.SetStaticMesh` _returnvalue_2 null)))))